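; Base AI controller that runs the possessed character's behavior tree and seeds its blackboard with that character's tuning and team.
; Sight, damage and hearing perception drive an AI state enum mirrored to the blackboard.
; Hostile sight targets the nearest targetable actor and attacks, while hostile damage or any heard noise triggers investigation from lower-priority states.
; Stun overrides the state, and recovery restores attack, patrol or idle.
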(event `self.ReceivePossess`
  (params (PossessedPawn :type "Pawn Object Reference"))
  (`self.OnPossess` PossessedPawn)
  (add `/Game/Blueprints/Game/Characters/BP_BaseCharacter.OnToggleStunComplete` (`self._character`) (delegate `OnToggleStunComplete_Event`)) ; Listen for being stunned
)

(event `OnToggleStunComplete_Event`
  (params (IsStunned :type Boolean))
  (if IsStunned
    (set `self.AIState` "NewEnumerator1")
    (else
      (`self.OnStunRecoveryRestoreAIState`))))

(event `self.AIPerception.OnPerceptionUpdated`
  (params (UpdatedActors :type "Array of Actor Object Reference (by ref)"))
  (for _array_element UpdatedActors
    (`|ExecutionSequence`
      (:`then_0`
        (bind (_issensed _is_hostile) (`self.Can Sense Actor` "/Script/AIModule.AISense_Sight" _array_element))
        (`self.IsHostileSensed` _issensed _is_hostile
          (:`true`
            (`self.OnSightSenseUpdated`))))
      (:`then_1`
        (bind (_issensed_2 _is_hostile_2 _stimulus) (`self.Can Sense Actor` "/Script/AIModule.AISense_Damage" _array_element))
        (`self.IsHostileSensed` _issensed_2 _is_hostile_2
          (:`true`
            (`self.OnDamagedSenseUpdated` (`.StimulusLocation` (break `AIStimulus` _stimulus))))))
      (:`then_2`
        (bind (_issensed_3 _is_hostile_3 _stimulus_2) (`self.Can Sense Actor` "/Script/AIModule.AISense_Hearing" _array_element))
        (if _issensed_3
          (`self.OnHearingSenseUpdated` (`.StimulusLocation` (break `AIStimulus` _stimulus_2))))))))

(fn `Can Sense Actor`
  (params (Sense :type "AISense Class Reference") (Actor :type "Actor Object Reference"))
  (returns (IsSensed :type Boolean) (`Is Hostile` :type Boolean) (Stimulus :type "AIStimulus Structure"))
  (bind _info (`AIPerceptionComponent.GetActorsPerception` (`self.AIPerception`) Actor))
  (bind (_target _lastsensedstimuli _bishostile) (break `ActorPerceptionBlueprintInfo` _info))
  (for _array_element _lastsensedstimuli
    (bind _returnvalue (`AIPerceptionSystem.GetSenseClassForStimulus` _array_element))
    (if (== Sense _returnvalue)
      (return (`.bSuccessfullySensed` (break `AIStimulus` _array_element)) _bishostile _array_element))))

(fn `GetAIState`
  (returns (AIState :type "/Game/Blueprints/Game/AI/States/EN_AIStates Enum"))
  (return (`self.AIState`)))

(fn `GetInvestigateLocation`
  (returns (_investigateLocation :type "Vector Structure"))
  (return (`self._investigateLocation`)))

(fn `GetNearestTargetInLineOfSight`
  (returns (NeartestTarget :type "Actor Object Reference"))
  (locals (_nearestDistance :type "Float (double-precision)" :default 99999999.0) (_nearestTarget :type "Actor Object Reference"))
  (for _array_element (`AIPerceptionComponent.GetPerceivedHostileActorsBySense` (`self.AIPerception`) "/Script/AIModule.AISense_Sight")
    (bind _asbpi_targetable (cast `/Game/Blueprints/Core/Targetable/BPI_Targetable` _array_element))
    (bind _istargetable (`/Game/Blueprints/Core/Targetable/BPI_Targetable.IsTargetable` _asbpi_targetable))
    (if _istargetable
      (bind _returnvalue (`KismetMathLibrary.Vector_Distance` (`self.K2_GetActorLocation` _array_element) (`self.K2_GetActorLocation` (`self._character`))))
      (if (< _returnvalue (`local._nearestDistance`))
        (set `local._nearestTarget` _array_element)
        (set `local._nearestDistance` _returnvalue))))
  (return (`local._nearestTarget`)))

(fn `GetTarget`
  (returns (_target :type "Actor Object Reference"))
  (return (`self._target`)))

(fn `GetWorldSpawnedLocation`
  (returns (_worldSpawnedLocation :type "Vector Structure"))
  (return (`self._worldSpawnedLocation`)))

(fn `OnDamagedSenseUpdated`
  (params (investigateLocation :type "Vector Structure"))
  (switch `/Game/Blueprints/Game/AI/States/EN_AIStates` (`self.GetAIState`)
    (:`NewEnumerator0`
      _)
    (:`NewEnumerator2`
      _)
    (:`NewEnumerator3`
      _))
  (set `self._investigateLocation` investigateLocation)
  (`self.SetAIState` "NewEnumerator3"))

(fn `OnHearingSenseUpdated`
  (params (Location :type "Vector Structure"))
  (switch `/Game/Blueprints/Game/AI/States/EN_AIStates` (`self.GetAIState`)
    (:`NewEnumerator0`
      _)
    (:`NewEnumerator2`
      _))
  (set `self._investigateLocation` Location)
  (`self.SetAIState` "NewEnumerator3"))

(fn `OnPossess`
  (params (possessedPawn :type "Pawn Object Reference"))
  (locals (_attackRadiusKey :type Name :default "AttackRadius") (_strafeRadiusKey :type Name :default "StrafeRadius") (_strafeMovementSpeedKey :type Name :default "StrafeMovementSpeed") (_maxMovementSpeedKey :type Name :default "MaxMovementSpeed") (_investigateMovementSpeedKey :type Name :default "InvestigateMovementSpeed") (_patrolMovementSpeedKey :type Name :default "PatrolMovementSpeed") (_teamIDKey :type Name :default "ThisCharacterTeamID"))
  (bind _returnvalue (`AIBlueprintHelperLibrary.GetBlackboard` null))
  (set `self._worldSpawnedLocation` (`self.K2_GetActorLocation` possessedPawn))
  (bind _asbp_base_aicharacter (cast `/Game/Blueprints/Game/Characters/AI/BP_BaseAICharacter` possessedPawn))
  (bind _output_get (set `self._character` _asbp_base_aicharacter))
  (`self.OnPossesComplete`)
  (bind _behaviourtree (`/Game/Blueprints/Game/Characters/AI/BP_BaseAICharacter.GetAIBehaviourTree` _output_get))
  (`/Engine/EditorBlueprintResources/StandardMacros.IsValid` _behaviourtree
    (:`Is Valid`
      (`self.RunBehaviorTree` _behaviourtree)
      (`BlackboardComponent.SetValueAsFloat` _returnvalue (`local._attackRadiusKey`) (`/Game/Blueprints/Game/Characters/AI/BP_BaseAICharacter.GetAttackRadius` _output_get))
      (`BlackboardComponent.SetValueAsFloat` _returnvalue (`local._strafeRadiusKey`) (`/Game/Blueprints/Game/Characters/AI/BP_BaseAICharacter.GetStrafeRadius` _output_get))
      (`BlackboardComponent.SetValueAsFloat` _returnvalue (`local._strafeMovementSpeedKey`) (`/Game/Blueprints/Game/Characters/AI/BP_BaseAICharacter.GetStrafeMovementSpeed` _output_get))
      (`BlackboardComponent.SetValueAsFloat` _returnvalue (`local._maxMovementSpeedKey`) (`/Game/Blueprints/Game/Characters/AI/BP_BaseAICharacter.GetMaxMovementSpeed` _output_get))
      (`BlackboardComponent.SetValueAsFloat` _returnvalue (`local._investigateMovementSpeedKey`) (`/Game/Blueprints/Game/Characters/AI/BP_BaseAICharacter.GetInvestigateMovementSpeed` _output_get))
      (`BlackboardComponent.SetValueAsFloat` _returnvalue (`local._patrolMovementSpeedKey`) (`/Game/Blueprints/Game/Characters/AI/BP_BaseAICharacter.GetPatrolMovementSpeed` _output_get))
      (`BlackboardComponent.SetValueAsInt` _returnvalue (`local._teamIDKey`) (`BaseCharacter.TeamID` _output_get))
      (`self.SetAIState` (`/Game/Blueprints/Game/Characters/AI/BP_BaseAICharacter.GetStartingAIState` _output_get)))))

(fn `OnSightSenseUpdated`
  (locals (_nearestTarget :type "Actor Object Reference") (_nearestDistance :type "Float (double-precision)" :default 999999.0))
  (bind _neartesttarget (`self.GetNearestTargetInLineOfSight`))
  (switch `/Game/Blueprints/Game/AI/States/EN_AIStates` (`self.GetAIState`)
    (:`NewEnumerator0`
      _)
    (:`NewEnumerator2`
      _)
    (:`NewEnumerator3`
      _)
    (:`NewEnumerator4`
      _)
    (:`NewEnumerator8`
      _))
  (if (`KismetSystemLibrary.IsValid` _neartesttarget)
    (`self.SetTarget` _neartesttarget)
    (`self.SetAIState` "NewEnumerator4")
    (else
      (`self.SetTarget` null) ; Set Null
      (`self.RestoreState`))))

(fn `OnStunRecoveryRestoreAIState`
  (`/Engine/EditorBlueprintResources/StandardMacros.IsValid` (`self._target`)
    (:`Is Valid`
      (`self.SetAIState` "NewEnumerator4"))
    (:`Is Not Valid`
      (`/Engine/EditorBlueprintResources/StandardMacros.IsValid` (`/Game/Blueprints/Game/AI/Pathing/BPC_PatrolController.GetActivePatrolPath` (`/Game/Blueprints/Game/Characters/AI/BP_BaseAICharacter.PatrolController` (`self._character`)))
        (:`Is Valid`
          (`self.SetAIState` "NewEnumerator2"))
        (:`Is Not Valid`
          (`self.SetAIState` "NewEnumerator0"))))))

(fn `RestoreState`
  (bind _asbpi_patrol_character (cast `/Game/Blueprints/Game/AI/Pathing/BPI_PatrolCharacter` (`self._character`))
    (:`then`
      (bind _patrol (`/Game/Blueprints/Game/AI/Pathing/BPI_PatrolCharacter.GetCurrentPatrolPath` _asbpi_patrol_character))
      (`/Engine/EditorBlueprintResources/StandardMacros.IsValid` _patrol
        (:`Is Valid`
          (`self.SetAIState` "NewEnumerator2"))
        (:`Is Not Valid`
          (`self.SetAIState` "NewEnumerator0" :!label _label))))
    (:`CastFailed`
      (goto _label))))

(fn `SetAIState`
  (params (AIState :type "/Game/Blueprints/Game/AI/States/EN_AIStates Enum" :default "NewEnumerator0"))
  (locals (_stateKeyName :type Name :default "State"))
  (bind _output_get (set `self.AIState` AIState))
  (`BlackboardComponent.SetValueAsEnum` (`AIBlueprintHelperLibrary.GetBlackboard` null) (`local._stateKeyName`) _output_get)
  (`self.OnAIStateChangedEvent` _output_get))

(fn `SetTarget`
  (params (EnemyTarget :type "Actor Object Reference"))
  (locals (_targetBBKey :type Name :default "Target"))
  (bind _output_get (set `self._target` EnemyTarget))
  (`BlackboardComponent.SetValueAsObject` (`AIBlueprintHelperLibrary.GetBlackboard` null) (`local._targetBBKey`) _output_get))

(fn `StopRunningLogics`
  (`self.K2_ClearFocus`)
  (`BrainComponent.StopLogic` (`self.BrainComponent`) "Dead"))

(fn `UserConstructionScript`)