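; Base controller for player characters that feeds sight-based enemy detection into a targeting system.
; On possess it caches the player character and initializes TargetingSystem with it.
; AIPerception updates add sensed enemy characters to the targeting array and remove lost ones.
; SetFacingRotation interpolates control rotation toward a given look-at position, using a fixed delta time rather than frame time.
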(event `self.ReceivePossess`
  (params (PossessedPawn :type "Pawn Object Reference"))
  ;[1 1 1] Setup Targetting System
  (bind _asbp_base_player_character (cast `/Game/Blueprints/Game/Characters/Player/BP_BasePlayerCharacter` PossessedPawn))
  (set `self._character` _asbp_base_player_character)
  (`/Game/Blueprints/Game/TargetSystem/BPC_TargetSystem.Initialize Variables` (`self.TargetingSystem`) _asbp_base_player_character))

(event `self.AIPerception.OnTargetPerceptionUpdated`
  (params (Actor :type "Actor Object Reference") (Stimulus :type "AIStimulus Structure"))
  (bind _outactors (`AIPerceptionComponent.GetCurrentlyPerceivedActors` (`self.AIPerception`) "/Script/AIModule.AISense_Sight"))
  (bind _asbp_base_enemy_character (cast `/Game/Blueprints/Game/Characters/AI/Enemies/BP_BaseEnemyCharacter` Actor))
  (if Stimulus_bSuccessfullySensed
    (`/Game/Blueprints/Game/TargetSystem/BPC_TargetSystem.AddTargetToArray` (`self.TargetingSystem`) _asbp_base_enemy_character)
    (else
      (`/Game/Blueprints/Game/TargetSystem/BPC_TargetSystem.RemoveTargetFromArray` (`self.TargetingSystem`) _asbp_base_enemy_character)
      (if (`KismetArrayLibrary.Array_Contains` _outactors _asbp_base_enemy_character)
        (`KismetArrayLibrary.Array_RemoveItem` _outactors _asbp_base_enemy_character)))))

(fn `SetFacingRotation`
  (params (LookAtPosition :type "Vector Structure (by ref)") (InterpolateSpeed :type "Float (single-precision)"))
  (`/Engine/EditorBlueprintResources/StandardMacros.IsValid` (`self._character`)
    (:`Is Valid`
      (`self.SetControlRotation` (`KismetMathLibrary.RInterpTo` (`self.GetControlRotation`) (`KismetMathLibrary.FindLookAtRotation` (`self.K2_GetActorLocation` (`self._character`)) LookAtPosition) 0.001 InterpolateSpeed)))))

(fn `UserConstructionScript`)