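; Patrol controller component that tracks an AI's active spline patrol path and current point index.
; Setting a path resets the index and broadcasts a dispatcher, while a getter supplies the current point's world location as the move target.
; Reaching a point steps the index by travel direction, with spline type deciding end behavior: Loop wraps, Linear flips direction, and Linear Loop and Ping Pong share logic that resets the index and flips.
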(fn `GetActivePatrolPath`
  (returns (_activePatrolPath :type "/Game/Blueprints/Game/AI/Pathing/BP_PatrolPath Object Reference"))
  (return (`self._activePatrolPath`)))

(fn `GetMoveToPatrolPathPointLocation`
  (returns (Position :type "Vector Structure") (IsValid :type Boolean))
  (`/Engine/EditorBlueprintResources/StandardMacros.IsValid` (`self._activePatrolPath`)
    (:`Is Valid`
      (return (`/Game/Blueprints/Core/Utility/Spline/BP_Spline.GetSplinePointPositionData` (`self._activePatrolPath`) (`self._patrolPathCurrentIndex`) "World") true))
    (:`Is Not Valid`
      (`KismetSystemLibrary.PrintString` "ERROR: Your patrol point is not valid!")
      (return (0.0 0.0 0.0) false))))

(fn `On Patrol Point Reached`
  (`self.SetNextPatrolPathIndex` (`self._isPatrollingForward`)))

(fn `SetNextPatrolPathIndex`
  (params (isForwardDirection :type Boolean))
  (bind __patrolpathcurrentindex (`self._patrolPathCurrentIndex`))
  (if (`KismetSystemLibrary.IsValid` (`self._activePatrolPath`))
    (if isForwardDirection
      (if (>= __patrolpathcurrentindex (- (`SplineComponent.GetNumberOfSplinePoints` (`/Game/Blueprints/Core/Utility/Spline/BP_Spline.Spline` (`self._activePatrolPath`))) 1))
        (switch `/Game/Blueprints/Core/Utility/Spline/EN_SplineMovementType` (`/Game/Blueprints/Core/Utility/Spline/BP_Spline.GetSplineType` (`self._activePatrolPath`))
          (:`NewEnumerator0`
            (set `self._patrolPathCurrentIndex` 0))
          (:`NewEnumerator1`
            (`self.ToggleIsPatrollingForward`))
          (:`NewEnumerator3`
            (set `self._patrolPathCurrentIndex` (- (`SplineComponent.GetNumberOfSplinePoints` (`/Game/Blueprints/Core/Utility/Spline/BP_Spline.Spline` (`self._activePatrolPath`))) 2) :!label _label)
            (`self.ToggleIsPatrollingForward`))
          (:`NewEnumerator2`
            (goto _label)))
        (else
          (`/Engine/EditorBlueprintResources/StandardMacros.IncrementInt` __patrolpathcurrentindex)))
      (elif (< __patrolpathcurrentindex 0)
        (switch `/Game/Blueprints/Core/Utility/Spline/EN_SplineMovementType` (`/Game/Blueprints/Core/Utility/Spline/BP_Spline.GetSplineType` (`self._activePatrolPath`))
          (:`NewEnumerator0`
            (set `self._patrolPathCurrentIndex` (- (`SplineComponent.GetNumberOfSplinePoints` (`/Game/Blueprints/Core/Utility/Spline/BP_Spline.Spline` (`self._activePatrolPath`))) 2)))
          (:`NewEnumerator1`
            (`self.ToggleIsPatrollingForward`))
          (:`NewEnumerator3`
            (set `self._patrolPathCurrentIndex` 0 :!label _label_2)
            (`self.ToggleIsPatrollingForward`))
          (:`NewEnumerator2`
            (goto _label_2)))
        (else
          (`/Engine/EditorBlueprintResources/StandardMacros.DecrementInt` __patrolpathcurrentindex))))))

(fn `SetPatrolPath`
  (params (_activePatrolPath :type "/Game/Blueprints/Game/AI/Pathing/BP_PatrolPath Object Reference"))
  (set `self._activePatrolPath` _activePatrolPath)
  (set `self._patrolPathCurrentIndex` 0) ; ResetPath
  (`self.OnPatrolPathStartedComplete`))

(fn `ToggleIsPatrollingForward`
  (set `self._isPatrollingForward` (not (`self._isPatrollingForward`))))