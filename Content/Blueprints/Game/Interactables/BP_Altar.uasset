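; BP_Altar is an interactable altar that toggles between activated and deactivated each time it is interacted with.
; A FlipFlop on OnInteract calls the OnAlterActivated or OnAlterDeactivated dispatcher and plays or reverses a timeline.
; The timeline drives the m1 material parameter and the point light intensity, fading both in and out.
; The construction script creates the dynamic material instance from M_Altar on the altar mesh.
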(event `/Game/Blueprints/Game/Interactables/BPI_Interactable.OnInteract`
  (params (playerCharacter :type "/Game/Blueprints/Game/Characters/Player/BP_BasePlayerCharacter Object Reference"))
  (`/Engine/EditorBlueprintResources/StandardMacros.FlipFlop`
    (:`A`
      (`self.OnAlterActivated`)
      (bind (_direction _m1 _light) (`Timeline|Timeline_0` :!label _label)
        (:`Update`
          (`MaterialInstanceDynamic.SetScalarParameterValue` (`self.Altar`) "m1" _m1)
          (`LightComponent.SetIntensity` (`self.PointLight`) _light))))
    (:`B`
      (`self.OnAlterDeactivated`)
      (goto _label :!via `Reverse`))))

(fn `UserConstructionScript`
  (bind _returnvalue (`PrimitiveComponent.CreateDynamicMaterialInstance` (`self.SM_Altar`) 0 "/Game/Blueprints/Game/Portal/Materials/M_Altar.M_Altar" "None"))
  (set `self.Altar` _returnvalue))