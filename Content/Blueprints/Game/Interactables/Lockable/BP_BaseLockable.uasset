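; BP_BaseLockable is a base Blueprint for lockable interactables that remember being unlocked.
; OnUnlocked clears IsLocked and writes UnlockKeyValue to save key data under the actor's GUID string.
; On BeginPlay it reads that value back and, if non-zero, unlocks without calling the unlock event, restoring state after a respawn.
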(event `self.ReceiveBeginPlay`
  (`self.WasUnlockedCheck`))

(event `/Game/Blueprints/Game/Interactables/Lockable/BPI_Lockable.SetIsLocked`
  (params (isLocked :type Boolean))
  (set `self._isLocked` isLocked))

(event `/Game/Blueprints/Core/Save/BPI_Saveable.SetSavedValue`
  (params (Value :type Integer))
  (bind _key (`self.GetSavedKey`))
  (`/Game/Blueprints/Game/Utility/BP_FunctionLibrary.SetSaveKeyData` _key Value))

(fn `GetIsLocked`
  (returns (isLocked :type Boolean))
  (return (`self._isLocked`)))

(fn `GetSavedKey`
  (returns (Key :type String))
  (return (`KismetGuidLibrary.Conv_GuidToString` (`self.ActorGuid`))))

(fn `GetSavedValue`
  (returns (Value :type Integer))
  (return (`/Game/Blueprints/Game/Utility/BP_FunctionLibrary.GetSaveKeyData` (`KismetGuidLibrary.Conv_GuidToString` (`self.ActorGuid`)))))

(fn `OnUnlocked`
  (locals (_unlockKeyValue :type Integer :default 1))
  (set `self._isLocked` false)
  (`self.SetSavedValue` (`local._unlockKeyValue`)))

(fn `UnlockWithoutNotify`
  (`/Game/Blueprints/Game/Interactables/Lockable/BPI_Lockable.SetIsLocked` false))

(fn `UserConstructionScript`)

(fn `WasUnlockedCheck`
  (bind _value (`self.GetSavedValue`))
  (switch `int` _value ; 0 is false -- Do nothing\nAny other value is true.\nUsed to check if this was already unlocked\nbefore respawning
    (:`Default`
      (`self.UnlockWithoutNotify`))))