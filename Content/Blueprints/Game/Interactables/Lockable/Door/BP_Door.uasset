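; BP_Door is a lockable, interactable single or double door that swings open and closed.
; The construction script sets meshes and lock placement from DoorType, and shows the lock while locked.
; Interaction tries the player's key, then either toggles a forward/reverse swing timeline or plays a locked-rattle timeline.
; Collision is off during swings to avoid pushing the player, and doors starting open jump the timeline to its end.
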(event `self.ReceiveBeginPlay`
  (if (`self._isOpened`)
    ;[1 1 1] If we want the door to start opened, we need to set the timeline at the end of it so it doesn't snap in it's animation when trying to close it for the first time
    (`self.StartOpened`))
  (`parent.ReceiveBeginPlay`))

(event `/Game/Blueprints/Game/Interactables/BPI_Interactable.OnInteract`
  (params (playerCharacter :type "/Game/Blueprints/Game/Characters/Player/BP_BasePlayerCharacter Object Reference"))
  (`/Game/Blueprints/Game/Utility/BP_MacroLibrary.TryUseKey` self (`/Game/Blueprints/Game/Characters/Player/BP_BasePlayerCharacter.KeyController` playerCharacter)
    (:`KeyUsed`
      (`self.OnUnlocked`)
      (`self.SetDoorColliders` true :!label _label) ; Disable collider so the door doesnt push us
      (`self.ToggleOpenClose`))
    (:`NoKeys`
      ;[1 1 1] Play Locked
      (bind (_direction _rawrotationz) (`Timeline|TryOpenLockedTimeline`) ; Door is locked, wont open.
        (:`Update`
          (`self.RotateDoors` _rawrotationz))
        (:`Finished`
          (`self.ResetLockedTimeline`) ; Resets the timeline so when we \ndo "play" again, it starts at position 0
          (`self.OnDoorTryOpenLockedDoorComplete`))))
    (:`WasntLocked`
      (goto _label))))

(event `Open`
  (`self.ToggleIsDoorOpen`)
  (bind (_direction _rotationz) (`Timeline|MoveTimeline` :!label _label_2)
    (:`Update`
      (`self.RotateDoors` (`KismetMathLibrary.Lerp` 0.0 90.0 _rotationz)))
    (:`Finished`
      (`self.SetDoorColliders` false) ; Reenable collider so we can walk through
      (`self.OnDoorOpenClosedComplete`))))

(event `Close`
  (`self.ToggleIsDoorOpen`)
  (goto _label_2 :!via `Reverse`))

(fn `OnDoorOpenClosedComplete`
  (if (`self._isOpened`)
    (`self.OnDoorOpenedComplete`)
    (else
      (`self.OnDoorClosedComplete`))))

(fn `OnUnlocked`
  (`self.ToggleLockVisibilities` false)
  (`parent.OnUnlocked`))

(fn `ResetLockedTimeline`
  (`TimelineComponent.SetPlaybackPosition` (`self.TryOpenLockedTimeline`) 0.0 false true))

(fn `RotateDoors`
  (params (rotZ :type "Float (double-precision)"))
  (`SceneComponent.K2_SetRelativeRotation` (`self.DoorStaticMesh`) (`KismetMathLibrary.MakeRotator` 0.0 0.0 rotZ) false true)
  (`SceneComponent.K2_SetRelativeRotation` (`self.DoubleDoorStaticMesh`) (`KismetMathLibrary.MakeRotator` 0.0 0.0 (+ (* rotZ -1.0) 180.0)) false true))

(fn `SetDoorColliders`
  (params (isDisableCollider :type Boolean))
  (bind _doorstaticmesh (`self.DoorStaticMesh`))
  (if isDisableCollider
    (`PrimitiveComponent.SetCollisionEnabled` _doorstaticmesh "NoCollision")
    (`PrimitiveComponent.SetCollisionEnabled` (`self.DoubleDoorStaticMesh`) "NoCollision")
    (else
      (`PrimitiveComponent.SetCollisionEnabled` _doorstaticmesh "QueryAndPhysics")
      (`PrimitiveComponent.SetCollisionEnabled` (`self.DoubleDoorStaticMesh`) "QueryAndPhysics"))))

(fn `SetDoorType`
  (params (Door :type "/Game/Blueprints/Game/Interactables/Lockable/Door/EN_Door Enum" :default "NewEnumerator0"))
  (bind _doorstaticmesh (`self.DoorStaticMesh`))
  (bind _doubledoorstaticmesh (`self.DoubleDoorStaticMesh`))
  ;[1 1 1] Assign the mesh depending on the door type
  (switch `/Game/Blueprints/Game/Interactables/Lockable/Door/EN_Door` Door
    (:`NewEnumerator0`
      (`StaticMeshComponent.SetStaticMesh` _doorstaticmesh "/Game/Assets/Environments/Medieval_Village/meshes/building/SM_door_03.SM_door_03")
      ;[1 1 1] Set double door settings
      (`StaticMeshComponent.SetStaticMesh` _doubledoorstaticmesh "/Game/Assets/Environments/Medieval_Village/meshes/building/SM_door_03.SM_door_03")
      (`SceneComponent.K2_SetRelativeLocation` _doubledoorstaticmesh (280.0 0.0 0.0) false false))
    (:`NewEnumerator6`
      (`StaticMeshComponent.SetStaticMesh` _doorstaticmesh "/Game/Assets/Environments/Medieval_Village/meshes/building/SM_window_door_01.SM_window_door_01")
      (`StaticMeshComponent.SetStaticMesh` _doubledoorstaticmesh "/Game/Assets/Environments/Medieval_Village/meshes/building/SM_window_door_01.SM_window_door_01")
      (`SceneComponent.K2_SetRelativeLocation` _doubledoorstaticmesh (130.0 0.0 0.0) false false))
    (:`NewEnumerator1`
      (`StaticMeshComponent.SetStaticMesh` _doorstaticmesh "/Game/Assets/Environments/Viking_Village/meshes/building/SM_door_01.SM_door_01")
      (`SceneComponent.SetVisibility` _doubledoorstaticmesh false false :!label _label))
    (:`NewEnumerator2`
      (`StaticMeshComponent.SetStaticMesh` _doorstaticmesh "/Game/Assets/Environments/Stylized_Egypt/Meshes/building/SM_door_01.SM_door_01")
      (goto _label))
    (:`NewEnumerator3`
      (`StaticMeshComponent.SetStaticMesh` _doorstaticmesh "/Game/Assets/Environments/Medieval_Village/meshes/building/SM_door_01.SM_door_01")
      (goto _label))
    (:`NewEnumerator4`
      (`StaticMeshComponent.SetStaticMesh` _doorstaticmesh "/Game/Assets/Environments/Medieval_Village/meshes/building/SM_door_02.SM_door_02")
      (goto _label))
    (:`NewEnumerator7`
      (`StaticMeshComponent.SetStaticMesh` _doorstaticmesh "/Game/Assets/Environments/DreamscapeSeries/DreamscapeTower/Meshes/Tower/SM_Door_Base.SM_Door_Base")
      (goto _label))))

(fn `SetLocksRootOffset`
  (params (Selection :type "/Game/Blueprints/Game/Interactables/Lockable/Door/EN_Door Enum" :default "NewEnumerator0"))
  (locals (_offset :type "Vector Structure" :default (0.0 0.0 0.0)))
  (switch `/Game/Blueprints/Game/Interactables/Lockable/Door/EN_Door` Selection
    (:`NewEnumerator0`
      (set `local._offset` (140.0 -10.0 100.0)))
    (:`NewEnumerator6`
      (set `local._offset` (65.0 -10.0 60.0)))
    (:`NewEnumerator1`
      (set `local._offset` (91.0 -10.0 108.0)))
    (:`NewEnumerator2`
      (set `local._offset` (128.0 -10.0 97.0)))
    (:`NewEnumerator3`
      (set `local._offset` (119.0 -10.0 103.0)))
    (:`NewEnumerator4`
      (set `local._offset` (119.0 -10.0 103.0)))
    (:`NewEnumerator7`
      (set `local._offset` (218.0 -10.0 98.0))))
  (`SceneComponent.K2_SetRelativeLocation` (`self.LockRoot`) (`local._offset`) false false))

(fn `StartOpened`
  (bind _movetimeline (`self.MoveTimeline`))
  ;[1 1 1] If we want the door to start opened, we need to set the timeline at the end of it so it doesn't snap in it's animation when trying to close it for the first time
  (`TimelineComponent.SetNewTime` _movetimeline (`TimelineComponent.GetTimelineLength` _movetimeline))
  (`self.RotateDoors` 90.0))

(fn `ToggleIsDoorOpen`
  (set `self._isOpened` (not (`self._isOpened`))))

(fn `ToggleLockVisibilities`
  (params (isLocked :type Boolean))
  (`SceneComponent.SetVisibility` (`self.LockRoot`) isLocked true))

(fn `ToggleOpenClose`
  (if (`self._isOpened`)
    (`self.Close`)
    (else
      (`self.Open`))))

(fn `UnlockWithoutNotify`
  (`parent.UnlockWithoutNotify`)
  (`self.RotateDoors` 90.0))

(fn `UserConstructionScript`
  (bind __doortype (`self._doorType`))
  (bind _islocked (`self.GetIsLocked`))
  (`self.ToggleLockVisibilities` _islocked)
  (`self.SetLocksRootOffset` __doortype)
  (`self.SetDoorType` __doortype))