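; BP_TreasureChest is a lockable interactable chest that spawns a key, health potion or mana potion pickup when opened.
; Interacting tries the player's key controller, playing a locked montage without keys, or unlocking once and playing the opening montage.
; On blend out, a zero-rate montage holds the open pose and OnOpen spawns the reward, then reports it.
; UnlockWithoutNotify jumps straight to the open pose without spawning a reward.
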(event `self.ReceiveBeginPlay`
  (`parent.ReceiveBeginPlay`))

(event `ForceOpenAnim`
  (set `self._isOpened` true)
  (`|PlayMontage` (`self.SkeletalMesh`) "/Game/Assets/Environments/DreamscapeSeries/DreamscapeMountains/Meshes/Props/Animated/SK_Chest_Animated_01_Opened_Opened_Montage.SK_Chest_Animated_01_Opened_Opened_Montage" 0.0))

(event `/Game/Blueprints/Game/Interactables/BPI_Interactable.OnInteract`
  (params (playerCharacter :type "/Game/Blueprints/Game/Characters/Player/BP_BasePlayerCharacter Object Reference"))
  (bind _skeletalmesh (`self.SkeletalMesh`))
  (if (not (`self._isOpened`))
    (`/Game/Blueprints/Game/Utility/BP_MacroLibrary.TryUseKey` self (`/Game/Blueprints/Game/Characters/Player/BP_BasePlayerCharacter.KeyController` playerCharacter)
      (:`KeyUsed`
        (`/Engine/EditorBlueprintResources/StandardMacros.DoOnce` false :!label _label
          (:`Completed`
            (set `self._isOpened` true)
            (`self.OnUnlocked`)
            (`|PlayMontage` _skeletalmesh "/Game/Assets/Environments/DreamscapeSeries/DreamscapeMountains/Meshes/Props/Animated/SK_Chest_Animated_01_Open_Sequence_Montage1.SK_Chest_Animated_01_Open_Sequence_Montage1"
              (:`OnBlendOut`
                (`|PlayMontage` _skeletalmesh "/Game/Assets/Environments/DreamscapeSeries/DreamscapeMountains/Meshes/Props/Animated/SK_Chest_Animated_01_Opened_Opened_Montage.SK_Chest_Animated_01_Opened_Opened_Montage" 0.0
                  (:`then`
                    (`self.OnOpen`))))))))
      (:`NoKeys`
        (`|PlayMontage` (`self.SkeletalMesh`) "/Game/Assets/Environments/DreamscapeSeries/DreamscapeMountains/Meshes/Props/Animated/SK_Chest_Animated_01_Locked_Locked_Montage.SK_Chest_Animated_01_Locked_Locked_Montage"))
      (:`WasntLocked`
        (goto _label)))))

(fn `OnOpen`
  (bind _reward (`self.SpawnReward`))
  (`self.OnOpenComplete` _reward))

(fn `SpawnReward`
  (returns (Reward :type "/Game/Blueprints/Game/Pickups/BP_BasePickup Object Reference"))
  (bind (_returnvalue_location _returnvalue_rotation) (`KismetMathLibrary.BreakTransform` (`self.GetTransform` self)))
  (switch `/Game/Blueprints/Game/Pickups/EN_Pickups` (`self._rewardSpawned`)
    (:`NewEnumerator0`
      (bind _returnvalue (`|SpawnActorFromClass` "/Game/Blueprints/Game/Pickups/BP_KeyPickup.BP_KeyPickup_C" (`KismetMathLibrary.MakeTransform` _returnvalue_location _returnvalue_rotation) "Undefined" "OverrideRootScale" null true null))
      (return _returnvalue))
    (:`NewEnumerator1`
      (bind _returnvalue_2 (`|SpawnActorFromClass` "/Game/Blueprints/Game/Pickups/BP_HealthPotionPickup.BP_HealthPotionPickup_C" (`KismetMathLibrary.MakeTransform` _returnvalue_location _returnvalue_rotation) "Undefined" "OverrideRootScale" null true null))
      (return _returnvalue_2))
    (:`NewEnumerator2`
      (bind _returnvalue_3 (`|SpawnActorFromClass` "/Game/Blueprints/Game/Pickups/BP_ManaPotionPickup.BP_ManaPotionPickup_C" (`KismetMathLibrary.MakeTransform` _returnvalue_location _returnvalue_rotation) "Undefined" "OverrideRootScale" null true null))
      (return _returnvalue_3))))

(fn `UnlockWithoutNotify`
  (`parent.UnlockWithoutNotify`)
  (`self.ForceOpenAnim`))

(fn `UserConstructionScript`)