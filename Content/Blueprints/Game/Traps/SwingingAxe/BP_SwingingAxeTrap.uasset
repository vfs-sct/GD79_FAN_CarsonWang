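; Swinging axe trap actor that damages anything its capsule overlaps and reports itself as unblockable.
; A looping timeline at configurable play rate rocks the rotation root in an arc, starting via ActivateTrap or automatically on BeginPlay, after a delay.
; Deactivation breaks it permanently: damage and swinging stop, and rod and blade switch to physics simulation.
; The construction script scales the rod and positions the blade from a minimum-clamped length in meters.
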(event `self.ReceiveBeginPlay`
  (`TimelineComponent.SetPlayRate` (`self.SwingTimeline`) (`self._playrate`))
  (if (`self._isAutoStart`)
    (`/Game/Blueprints/Game/Traps/BPI_Trap.ActivateTrap`)))

(event `/Game/Blueprints/Game/Traps/BPI_Trap.ActivateTrap`
  (if (not (`self._isBroken`))
    (`KismetSystemLibrary.Delay` (`self._startDelay`))
    (`self.OnActivateStart` self)
    (set `self._canDealDamage` true)
    (`TimelineComponent.SetLooping` (`self.SwingTimeline`) true)
    (bind (_direction _alpha) (`Timeline|SwingTimeline`)
      (:`Update`
        (`self.Swing` _alpha)))))

(event `/Game/Blueprints/Game/Traps/BPI_Trap.DeactivateTrap`
  (`self.Break`))

(event `self.Capsule.OnComponentBeginOverlap`
  (params (OverlappedComponent :type "PrimitiveComponent Object Reference") (OtherActor :type "Actor Object Reference") (OtherComp :type "PrimitiveComponent Object Reference") (OtherBodyIndex :type Integer) (bFromSweep :type Boolean) (SweepResult :type "HitResult Structure (by ref)"))
  (if (`self._canDealDamage`)
    (`GameplayStatics.ApplyDamage` OtherActor (`self._damage`) null self)))

(fn `Break`
  (bind _swingtimeline (`self.SwingTimeline`))
  (set `self._canDealDamage` false)
  (`TimelineComponent.SetLooping` _swingtimeline false)
  (`TimelineComponent.Stop` _swingtimeline)
  (`PrimitiveComponent.SetSimulatePhysics` (`self.rod`) true)
  (`PrimitiveComponent.SetSimulatePhysics` (`self.Blade`) true)
  (set `self._isBroken` true)
  (`self.OnDeactivateStart` self))

(fn `GetIsUnblockable`
  (returns (IsUnblockable :type Boolean))
  (return true))

(fn `SetRodLength`
  (params (Meters :type "Float (double-precision)"))
  (bind _rod (`self.rod`))
  (bind (_relativescale3d_x _relativescale3d_y) (`KismetMathLibrary.BreakVector` (`SceneComponent.RelativeScale3D` _rod)))
  (`SceneComponent.SetRelativeScale3D` _rod (`KismetMathLibrary.MakeVector` _relativescale3d_x _relativescale3d_y (/ Meters 2.0)))
  (`SceneComponent.K2_SetWorldLocation` (`self.Blade`) (+ (`SceneComponent.K2_GetComponentLocation` _rod) (* (* (`SceneComponent.GetUpVector` _rod) -1.0) (* Meters 100.0))) false true))

(fn `Swing`
  (params (Alpha :type "Float (double-precision)"))
  (`SceneComponent.K2_SetRelativeRotation` (`self.rotRoot`) (`KismetMathLibrary.RLerp` (struct :`Roll` 65.0) (struct :`Roll` -65.0) Alpha true) true true))

(fn `UserConstructionScript`
  (locals (_minLength :type "Float (double-precision)" :default 2.0))
  (bind __minlength (`local._minLength`))
  (if (< (`self._rodLengthInMeters`) __minlength)
    (bind _output_get (set `self._rodLengthInMeters` __minlength)))
  (`self.SetRodLength` _output_get))