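; Saw blade trap that runs along a length-adjustable track and deals unblockable damage to overlapping actors while active.
; Activation, automatic or triggered, waits a start delay, raises the blade by timeline, then a second timeline moves it between two endpoints as Tick spins it.
; Deactivation stops movement and damage and lowers the blade by reversing the first timeline.
; The construction script scales the base and repositions the end caps.
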(event `self.ReceiveBeginPlay`
  ;[1 1 1] Init
  (`TimelineComponent.SetPlayRate` (`self.MoveTimeline`) (`self._playrate`))
  (if (`self._isAutoPlay`)
    (`/Game/Blueprints/Game/Traps/BPI_Trap.ActivateTrap`)))

(event `/Game/Blueprints/Game/Traps/BPI_Trap.ActivateTrap`
  (`KismetSystemLibrary.Delay` (`self._startDelay`))
  (`self.OnActivateStart`)
  (bind (_direction _alpha) (`Timeline|PrepareBladeTimeline` :!label _label)
    (:`Update`
      (`self.PrepareBlade` _alpha))
    (:`Finished`
      (switch `ETimelineDirection` _direction
        (:`Forward`
          (bind (_direction_2 _alpha_2) (`Timeline|MoveTimeline`)
            (:`Update`
              (`self.Move` _alpha_2))))))))

(event `/Game/Blueprints/Game/Traps/BPI_Trap.DeactivateTrap`
  (`self.OnDeactivateStart`)
  (goto _label :!via `Reverse`))

(event `self.ReceiveTick`
  (params (DeltaSeconds :type "Float (single-precision)"))
  ;[1 1 1] Spin blade if active
  (if (`self.IsBladeMoving`)
    (`self.SpinBlade`)))

(event `self.Box.OnComponentBeginOverlap`
  (params (OverlappedComponent :type "PrimitiveComponent Object Reference") (OtherActor :type "Actor Object Reference") (OtherComp :type "PrimitiveComponent Object Reference") (OtherBodyIndex :type Integer) (bFromSweep :type Boolean) (SweepResult :type "HitResult Structure (by ref)"))
  ;[1 1 1] Deal damage
  (if (`self._canDealDamage`)
    (`GameplayStatics.ApplyDamage` OtherActor (`self._damage`) null self)))

(fn `GetIsUnblockable`
  (returns (IsUnblockable :type Boolean))
  (return true))

(fn `IsBladeMoving`
  (returns (isBladeMoving :type Boolean))
  (return (`TimelineComponent.IsPlaying` (`self.MoveTimeline`))))

(fn `Move`
  (params (Alpha :type "Float (double-precision)"))
  (bind _blade (`self.Blade`))
  (bind (_returnvalue_x _returnvalue_y _returnvalue_z) (`KismetMathLibrary.BreakVector` (`SceneComponent.K2_GetComponentLocation` _blade)))
  (bind (_returnvalue_x_2 _returnvalue_y_2) (`KismetMathLibrary.BreakVector` (`KismetMathLibrary.VLerp` (`SceneComponent.K2_GetComponentLocation` (`self.EndPointA`)) (`SceneComponent.K2_GetComponentLocation` (`self.EndPointB`)) Alpha)))
  (`SceneComponent.K2_SetWorldLocation` _blade (`KismetMathLibrary.MakeVector` _returnvalue_x_2 _returnvalue_y_2 _returnvalue_z) true true))

(fn `OnActivateStart`
  (set `self._canDealDamage` true))

(fn `OnDeactivateComplete`)

(fn `OnDeactivateStart`
  (`TimelineComponent.Stop` (`self.MoveTimeline`))
  (set `self._canDealDamage` false))

(fn `PrepareBlade`
  (params (Alpha :type "Float (single-precision)"))
  (bind _blade (`self.Blade`))
  (bind (_relativelocation_x _relativelocation_y) (`KismetMathLibrary.BreakVector` (`SceneComponent.RelativeLocation` _blade)))
  (`SceneComponent.K2_SetRelativeLocation` _blade (`KismetMathLibrary.VLerp` (`KismetMathLibrary.MakeVector` _relativelocation_x _relativelocation_y -20.0) (`KismetMathLibrary.MakeVector` _relativelocation_x _relativelocation_y 20.0) Alpha) true true))

(fn `ScaleTrackLength`
  (params (Meters :type "Float (double-precision)"))
  (locals (_unitsPerMeter :type "Float (double-precision)" :default 25.0))
  (bind _centerbase (`self.CenterBase`))
  (bind (_returnvalue_x _returnvalue_y _returnvalue_z) (`KismetMathLibrary.BreakVector` (`SceneComponent.K2_GetComponentScale` _centerbase)))
  (bind _returnvalue (- (* Meters 2.0) 1.0))
  (bind _returnvalue_2 (* (`local._unitsPerMeter`) _returnvalue))
  (`SceneComponent.SetWorldScale3D` _centerbase (`KismetMathLibrary.MakeVector` _returnvalue_x _returnvalue _returnvalue_z))
  (`SceneComponent.K2_SetRelativeLocation` (`self.EndCap1`) (`KismetMathLibrary.MakeVector` 0.0 _returnvalue_2) false false)
  (`SceneComponent.K2_SetRelativeLocation` (`self.EndCap`) (`KismetMathLibrary.MakeVector` 0.0 (* _returnvalue_2 -1.0)) false false))

(fn `SpinBlade`
  (`SceneComponent.K2_AddRelativeRotation` (`self.Blade`) (struct :`Roll` -5.0) true true))

(fn `UserConstructionScript`
  (if (< (`self._trackLengthInMeters`) 1.0)
    (set `self._trackLengthInMeters` 1.0))
  (`self.ScaleTrackLength` (`self._trackLengthInMeters`)))