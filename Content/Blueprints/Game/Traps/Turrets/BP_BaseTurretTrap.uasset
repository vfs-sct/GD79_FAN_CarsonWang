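; Base turret trap that raises a turret, fires volleys from four spawn points and lowers it again.
; MoveTimeline drives the rise and fall; once raised, shots spread across ShootTime while an optional SpinTimeline rotates the turret, then OnSwitch's FlipFlop retracts it.
; Auto-play repeats this on a looping timer, while ActivateTrap and DeactivateTrap drive the timelines directly.
; SpawnBullet is an empty hook that child turrets override to define their projectile.
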(event `self.ReceiveBeginPlay`
  (`self.SetBulletSpawnPoints`)
  (`TimelineComponent.SetPlayRate` (`self.SpinTimeline`) (/ 1.0 (`self._shootTime`)))
  (if (`self._isAutoPlay`)
    (`KismetSystemLibrary.Delay` (`self.GetMoveTimelineTime`))
    (bind _returnvalue (`KismetSystemLibrary.K2_SetTimerDelegate` (delegate `OnSwitch`) (+ (`self._shootCooldown`) (`self._shootTime`)) true))
    (set `self._shootHandler` _returnvalue)))

(event `OnSwitch`
  (`/Engine/EditorBlueprintResources/StandardMacros.FlipFlop`
    (:`A`
      (bind (_direction _alpha) (`Timeline|MoveTimeline` :!label _label)
        (:`Update`
          (`self.MoveTurret` _alpha))
        (:`Finished`
          (if (`|EnumEquality` _direction "Forward")
            (`|ExecutionSequence`
              (:`then_0`
                (if (`self.IsSpinTrap`)
                  (bind (_direction_2 _alpha_2) (`Timeline|SpinTimeline` :!via `PlayFromStart`)
                    (:`Update`
                      (`self.SpinTurret` _alpha_2))
                    (:`Finished`
                      (`self.OnSwitch` :!label _label_2)))
                  (else
                    (`KismetSystemLibrary.Delay` (+ (`self.GetSpinTimelineTime`) 1.0))
                    (goto _label_2))))
              (:`then_1`
                (`/Game/Blueprints/Game/Utility/BP_MacroLibrary.ForLoopWithDelay` 0 (`self._timesShotPerCycle`) (`self.GetDelayShootTime`)
                  (:`LoopBody`
                    (`self.Shoot`)))))))))
    (:`B`
      (goto _label :!via `Reverse`))))

(event `/Game/Blueprints/Game/Traps/BPI_Trap.ActivateTrap`
  (`self.OnActivateStarted` self)
  (goto _label))

(event `/Game/Blueprints/Game/Traps/BPI_Trap.DeactivateTrap`
  (`KismetSystemLibrary.K2_ClearAndInvalidateTimerHandle` (`self._shootHandler`))
  (`self.OnDeactivateStarted` self)
  (`TimelineComponent.Stop` (`self.SpinTimeline`))
  (goto _label :!via `Reverse`))

(fn `EndAttack`)

(fn `GetDelayShootTime`
  (returns (Delay :type "Float (double-precision)"))
  (return (/ (`self._shootTime`) (`self._timesShotPerCycle`))))

(fn `GetIsUnblockable`
  (returns (IsUnblockable :type Boolean))
  (return false))

(fn `GetMoveTimelineTime`
  (returns (ReturnValue :type "Float (double-precision)"))
  (bind _movetimeline (`self.MoveTimeline`))
  (return (/ (`TimelineComponent.GetTimelineLength` _movetimeline) (`TimelineComponent.GetPlayRate` _movetimeline))))

(fn `GetSpinTimelineTime`
  (returns (ReturnValue :type "Float (double-precision)"))
  (bind _spintimeline (`self.SpinTimeline`))
  (return (/ (`TimelineComponent.GetTimelineLength` _spintimeline) (`TimelineComponent.GetPlayRate` _spintimeline))))

(fn `MoveTurret`
  (params (Alpha :type "Float (double-precision)"))
  (`SceneComponent.K2_SetRelativeLocation` (`self.Turret`) (`KismetMathLibrary.VLerp` (0.0 0.0 0.0) (0.0 0.0 65.0) Alpha) false false))

(fn `SetAutoShoot`)

(fn `SetBulletSpawnPoints`
  (set `self._bulletSpawnPoints` (`|MakeArray` (`self.SpawnPoint2`) (`self.SpawnPoint3`) (`self.SpawnPoint4`) (`self.SpawnPoint1`))))

(fn `Shoot`
  (for _array_element (`self._bulletSpawnPoints`)
    (`/Engine/EditorBlueprintResources/StandardMacros.IsValid` _array_element
      (:`Is Valid`
        (bind (_returnvalue_location _returnvalue_rotation) (`KismetMathLibrary.BreakTransform` (`SceneComponent.K2_GetComponentToWorld` _array_element)))
        (`self.SpawnBullet` _returnvalue_location _returnvalue_rotation (`self._damage`) self (`self._arrowSpeed`))))))

(fn `SpawnBullet`
  (params (`Spawn Transform Location` :type "Vector Structure") (`Spawn Transform Rotation` :type "Rotator Structure") (Damage :type "Float (double-precision)") (_caster :type "Actor Object Reference") (_speed :type "Float (single-precision)"))
  ;[1 1 1] YOU NEED TO CODE WHAT YOUR CHILD TURRET SHOOTS! (OVERRIDE)
)

(fn `SpinTurret`
  (params (Alpha :type "Float (double-precision)"))
  (`SceneComponent.K2_SetRelativeRotation` (`self.Turret`) (`KismetMathLibrary.RLerp` (struct) (struct :`Yaw` 360.0) Alpha) false false))

(fn `UserConstructionScript`)