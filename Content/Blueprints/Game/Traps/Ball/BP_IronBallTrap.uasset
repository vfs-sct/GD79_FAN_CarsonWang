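; BP_IronBallTrap is an iron ball trap that damages actors it hits while moving fast enough.
; Sphere hit events pass the other actor to OnCollision, which applies Damage when the ball's velocity exceeds SpeedRequiredToDamage.
; ActivateTrap and DeactivateTrap toggle CanDealDamage, though the hit logic shown here never checks that flag.
; GetIsUnblockable returns false, reporting the trap as blockable.
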(event `self.Sphere.OnComponentHit`
  (params (HitComponent :type "PrimitiveComponent Object Reference") (OtherActor :type "Actor Object Reference") (OtherComp :type "PrimitiveComponent Object Reference") (NormalImpulse :type "Vector Structure") (Hit :type "HitResult Structure (by ref)"))
  (if (`self.IsVelocityEnoughToDamageTargets`)
    (`self.OnCollision` OtherActor)))

(event `/Game/Blueprints/Game/Traps/BPI_Trap.DeactivateTrap`
  (set `self._canDealDamage` false))

(event `/Game/Blueprints/Game/Traps/BPI_Trap.ActivateTrap`
  (set `self._canDealDamage` true))

(fn `GetIsUnblockable`
  (returns (IsUnblockable :type Boolean))
  (return false))

(fn `IsVelocityEnoughToDamageTargets`
  (returns (ReturnValue :type Boolean))
  (return (> (`KismetMathLibrary.VSize` (`self.GetVelocity`)) (`self._speedRequiredToDamage`))))

(fn `OnCollision`
  (params (Actor :type "Actor Object Reference"))
  (`/Engine/EditorBlueprintResources/StandardMacros.IsValid` Actor
    (:`Is Valid`
      (`GameplayStatics.ApplyDamage` Actor (`self._damage`)))))

(fn `UserConstructionScript`)