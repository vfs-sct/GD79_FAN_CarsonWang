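; Spike trap that moves its spikes between inactive and fully extended spots and damages actors that begin overlapping its box.
; Activation, automatic on BeginPlay if IsAutoActive, loops MoveTimeline at a configurable play rate to drive a swept location lerp.
; Deactivation stops that timeline and plays a separate deactivation timeline through the same Move function.
; It fires activate/deactivate start callbacks and reports itself as unblockable.
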(event `self.ReceiveBeginPlay`
  (`self.SetTimelinePlayrate`)
  (if (`self._isAutoActive`)
    (`/Game/Blueprints/Game/Traps/BPI_Trap.ActivateTrap`)))

(event `/Game/Blueprints/Game/Traps/BPI_Trap.ActivateTrap`
  (`self.OnActivateStarted`)
  (`TimelineComponent.SetLooping` (`self.MoveTimeline`) true)
  (`|ExecutionSequence`
    (:`then_0`
      (bind (_direction _alpha) (`Timeline|MoveTimeline` :!via `PlayFromStart` :!label _label)
        (:`Update`
          (`self.Move` _alpha))))
    (:`then_1`
      (bind (_direction_2 _alpha_2) (`Timeline|DeactiveateTimeline` :`NewTime` (`KismetMathLibrary.NormalizeToRange` (`TimelineComponent.GetPlaybackPosition` (`self.MoveTimeline`)) 0.0 1.0) :!via `Stop` :!label _label_2)
        (:`Update`
          (`self.Move` _alpha_2))))))

(event `/Game/Blueprints/Game/Traps/BPI_Trap.DeactivateTrap`
  (`self.OnDeactivateStarted`)
  (`TimelineComponent.SetLooping` (`self.MoveTimeline`) false) ; Don't play/stop/reverse. Allow timeline to\ncontinue and end.
  (`|ExecutionSequence`
    (:`then_0`
      (goto _label :!via `Stop`))
    (:`then_1`
      (goto _label_2))))

(event `self.Box.OnComponentBeginOverlap`
  (params (OverlappedComponent :type "PrimitiveComponent Object Reference") (OtherActor :type "Actor Object Reference") (OtherComp :type "PrimitiveComponent Object Reference") (OtherBodyIndex :type Integer) (bFromSweep :type Boolean) (SweepResult :type "HitResult Structure (by ref)"))
  (`GameplayStatics.ApplyDamage` OtherActor (`self._damage`) null self))

(fn `GetIsUnblockable`
  (returns (IsUnblockable :type Boolean))
  (return true))

(fn `Move`
  (params (Alpha :type "Float (double-precision)"))
  (`SceneComponent.K2_SetWorldLocation` (`self.Spike`) (`KismetMathLibrary.VLerp` (`SceneComponent.K2_GetComponentLocation` (`self.InactiveSpot`)) (`SceneComponent.K2_GetComponentLocation` (`self.FullyExtendedSpot`)) Alpha) true true))

(fn `SetTimelinePlayrate`
  (`TimelineComponent.SetPlayRate` (`self.MoveTimeline`) (`self._timelinePlayRate`)))

(fn `UserConstructionScript`)