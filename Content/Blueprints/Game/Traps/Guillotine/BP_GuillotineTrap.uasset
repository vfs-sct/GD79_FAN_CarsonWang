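; Guillotine trap that repeatedly drops a blade and damages overlapping actors during the timeline's kill window.
; Activation, optionally automatic at BeginPlay, loops a rate-adjusted timeline after a delay, moving the blade between start and drop points; deactivation reverses it.
; Construction scales track and blade to a minimum-clamped length and sets ceiling height.
; Two overlap volumes toggle chain-segment visibility and collision, showing or hiding links as they enter.
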(event `self.ReceiveBeginPlay`
  (`self.SetTimelinePlayrate`)
  (if (`self._isStartActive`)
    (`/Game/Blueprints/Game/Traps/BPI_Trap.ActivateTrap`)))

(event `/Game/Blueprints/Game/Traps/BPI_Trap.ActivateTrap`
  (`KismetSystemLibrary.Delay` (`self._startDelay`))
  (`self.OnActivateStarted` self)
  (`TimelineComponent.SetLooping` (`self.DropTimeline`) true)
  (bind (_direction _alpha) (`Timeline|DropTimeline` :!label _label)
    (:`Update`
      (`self.MoveBlade` _alpha))
    (:`CanKill`
      (set `self._canKill` true))
    (:`CantKill`
      (set `self._canKill` false))))

(event `/Game/Blueprints/Game/Traps/BPI_Trap.DeactivateTrap`
  (`self.OnDeactivateStarted` self)
  (`TimelineComponent.SetLooping` (`self.DropTimeline`) false)
  (goto _label :!via `Reverse`))

(event `self.Box.OnComponentBeginOverlap`
  (params (OverlappedComponent :type "PrimitiveComponent Object Reference") (OtherActor :type "Actor Object Reference") (OtherComp :type "PrimitiveComponent Object Reference") (OtherBodyIndex :type Integer) (bFromSweep :type Boolean) (SweepResult :type "HitResult Structure (by ref)"))
  (if (`self._canKill`)
    (`/Engine/EditorBlueprintResources/StandardMacros.IsValid` OtherActor
      (:`Is Valid`
        (`GameplayStatics.ApplyDamage` OtherActor (`self._damage`) null self)))))

(event `self.ShowOverlap.OnComponentBeginOverlap`
  (params (OverlappedComponent :type "PrimitiveComponent Object Reference") (OtherActor :type "Actor Object Reference") (OtherComp :type "PrimitiveComponent Object Reference") (OtherBodyIndex :type Integer) (bFromSweep :type Boolean) (SweepResult :type "HitResult Structure (by ref)"))
  (if (`KismetArrayLibrary.Array_Contains` (`self._chains`) OtherComp)
    (`SceneComponent.SetVisibility` OtherComp true false)
    (`PrimitiveComponent.SetCollisionEnabled` OtherComp "QueryAndPhysics")))

(event `self.HideOverlap.OnComponentBeginOverlap`
  (params (OverlappedComponent :type "PrimitiveComponent Object Reference") (OtherActor :type "Actor Object Reference") (OtherComp :type "PrimitiveComponent Object Reference") (OtherBodyIndex :type Integer) (bFromSweep :type Boolean) (SweepResult :type "HitResult Structure (by ref)"))
  (if (`KismetArrayLibrary.Array_Contains` (`self._chains`) OtherComp)
    (`SceneComponent.SetVisibility` OtherComp false false)
    (`PrimitiveComponent.SetCollisionEnabled` OtherComp "QueryOnly")))

(fn `GetIsUnblockable`
  (returns (IsUnblockable :type Boolean))
  (return true))

(fn `MoveBlade`
  (params (Alpha :type "Float (single-precision)"))
  (`SceneComponent.K2_SetWorldLocation` (`self.BladeContainer`) (`KismetMathLibrary.VLerp` (`SceneComponent.K2_GetComponentLocation` (`self.BladeStart`)) (`SceneComponent.K2_GetComponentLocation` (`self.DropPoint`)) Alpha) true true))

(fn `ScaleTrackLength`
  (params (Meters :type "Float (double-precision)"))
  (locals (_unitsPerMeter :type "Float (double-precision)" :default 25.0))
  (bind _basecontainer (`self.BaseContainer`))
  (bind _topbasecontainer (`self.TopBaseContainer`))
  (bind _blade (`self.Blade`))
  (bind (_returnvalue_x _returnvalue_y _returnvalue_z) (`KismetMathLibrary.BreakVector` (`SceneComponent.K2_GetComponentScale` _blade)))
  (bind (_returnvalue_x_2 _returnvalue_y_2 _returnvalue_z_2) (`KismetMathLibrary.BreakVector` (`SceneComponent.K2_GetComponentScale` _basecontainer)))
  (bind (_returnvalue_x_3 _returnvalue_y_3 _returnvalue_z_3) (`KismetMathLibrary.BreakVector` (`SceneComponent.K2_GetComponentScale` _topbasecontainer)))
  (bind _returnvalue (- (* Meters 2.0) 1.0))
  (bind _returnvalue_2 (* _returnvalue (`local._unitsPerMeter`)))
  (bind _returnvalue_3 (- _returnvalue 1.0))
  (bind _returnvalue_4 (* _returnvalue_2 -1.0))
  (`SceneComponent.SetWorldScale3D` _topbasecontainer (`KismetMathLibrary.MakeVector` _returnvalue_x_3 _returnvalue_3 _returnvalue_z_3))
  (`SceneComponent.SetWorldScale3D` _blade (`KismetMathLibrary.MakeVector` _returnvalue_x (/ _returnvalue 2.0) _returnvalue_z))
  (`|ExecutionSequence`
    (:`then_0`
      (`SceneComponent.K2_SetRelativeLocation` (`self.TopCap`) (`KismetMathLibrary.MakeVector` 0.0 _returnvalue_2) false false)
      (`SceneComponent.K2_SetRelativeLocation` (`self.TopCap2`) (`KismetMathLibrary.MakeVector` 0.0 _returnvalue_4) false false)
      (`SceneComponent.K2_SetRelativeLocation` (`self.BaseCap`) (`KismetMathLibrary.MakeVector` 0.0 _returnvalue_4) false false)
      (`SceneComponent.K2_SetRelativeLocation` (`self.BaseCap1`) (`KismetMathLibrary.MakeVector` 0.0 _returnvalue_2) false false))
    (:`then_1`
      (`SceneComponent.SetWorldScale3D` _basecontainer (`KismetMathLibrary.MakeVector` _returnvalue_x_2 _returnvalue_3 _returnvalue_z_2)))))

(fn `SetHeight`
  (`SceneComponent.K2_SetRelativeLocation` (`self.Ceiling`) (`KismetMathLibrary.MakeVector` 0.0 0.0 (`self._dropHeight`)) false false))

(fn `SetTimelinePlayrate`
  (`TimelineComponent.SetPlayRate` (`self.DropTimeline`) (`self._timelinePlayrate`)))

(fn `UserConstructionScript`
  (locals (_minimumLength :type "Float (double-precision)" :default 1.5))
  (bind __minimumlength (`local._minimumLength`))
  (if (< (`self._trackLengthInMeters`) __minimumlength)
    (set `self._trackLengthInMeters` __minimumlength))
  (`self.ScaleTrackLength` (`self._trackLengthInMeters`))
  (`KismetArrayLibrary.Array_Clear` (`self._chains`))
  (set `self._chains` (`|MakeArray` (`self.ChainBase1`) (`self.Chain12`) (`self.Chain31`) (`self.Chain30`) (`self.Chain29`) (`self.Chain28`) (`self.Chain27`) (`self.Chain26`) (`self.Chain6`) (`self.Chain5`) (`self.Chain4`) (`self.Chain7`) (`self.Chain25`) (`self.Chain24`) (`self.Chain15`) (`self.Chain14`) (`self.Chain13`) (`self.Chain22`) (`self.ChainBase`) (`self.Chain10`) (`self.Chain9`) (`self.Chain3`) (`self.Chain`) (`self.Chain1`) (`self.Chain20`) (`self.Chain19`) (`self.Chain11`) (`self.Chain18`) (`self.Chain17`) (`self.Chain16`) (`self.Chain2`) (`self.Chain21`) (`self.Chain23`) (`self.Chain8`) (`self.Chain22`) :!type "PrimitiveComponent Object Reference"))
  (`self.SetHeight`))