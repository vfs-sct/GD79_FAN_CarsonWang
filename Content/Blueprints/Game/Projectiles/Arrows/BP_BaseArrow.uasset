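; Base arrow projectile that flies forward at its spawn-set speed, ignoring its caster, and expires after a set lifespan.
; On box hit it makes noise, stops moving and sphere-traces the hit component for the exact point and bone.
; A successful trace attaches it to that bone and pushes it in by a penetration depth.
; It then damages once, via TryOnHit for BP_BaseCharacter or ApplyDamage for other actors.
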(event `self.ReceiveBeginPlay`
  (bind _projectilemovement (`self.ProjectileMovement`))
  (`PrimitiveComponent.IgnoreActorWhenMoving` (`self.Box`) (`self._caster`) true)
  (bind _output_get (set `ProjectileMovementComponent.MaxSpeed` (`self._speed`) _projectilemovement))
  (bind _output_get_2 (set `ProjectileMovementComponent.InitialSpeed` _output_get _projectilemovement))
  (set `MovementComponent.Velocity` (* (`self.GetActorForwardVector` self) _output_get_2) _projectilemovement)
  (set `self._canDealDamage` true)
  (`self.SetLifeSpan` (`self._lifeSpanDuration`)))

(event `self.Box.OnComponentHit`
  (params (HitComponent :type "PrimitiveComponent Object Reference") (OtherActor :type "Actor Object Reference") (OtherComp :type "PrimitiveComponent Object Reference") (NormalImpulse :type "Vector Structure") (Hit :type "HitResult Structure (by ref)"))
  (bind _targetcomponent (`self.TargetComponent`))
  (bind _damage (`self.Damage`))
  (bind _targetactor (`self.TargetActor`))
  (bind _instigator (`self.Instigator`))
  (bind _projectilemovement (`self.ProjectileMovement`))
  (if (`self._canDealDamage`)
    (`self.MakeNoise` 1.0 null (`self.K2_GetActorLocation`) 400.0)
    (`ProjectileMovementComponent.StopSimulating` _projectilemovement Hit)
    (set `MovementComponent.Velocity` (0.0 0.0 0.0) _projectilemovement)
    (`PrimitiveComponent.SetCollisionEnabled` (`self.Box`) "NoCollision")
    (set `self.TargetActor` OtherActor)
    (bind _output_get (set `self.TargetComponent` OtherComp))
    (bind (_hitlocation _hitnormal _bonename _outhit _returnvalue) (`PrimitiveComponent.K2_SphereTraceComponent` _output_get (`SceneComponent.K2_GetComponentLocation` (`self.LineTraceStart`)) (`SceneComponent.K2_GetComponentLocation` (`self.LineTraceEnd`)) 15.0 true false false))
    (if _returnvalue
      (set `self.HitLocation` _hitlocation)
      (set `self.Hit Normal` _hitnormal)
      (set `self.Bone Name` _bonename)
      (`/Engine/EditorBlueprintResources/StandardMacros.IsValid` _targetcomponent
        (:`Is Valid`
          (`self.Attach` _targetcomponent (`self.Bone Name`)))
        (:`Is Not Valid`
          _))
      (`self.Penetrate` (`self.HitLocation`) (`self.PenetrateDepth`))
      (`/Engine/EditorBlueprintResources/StandardMacros.IsValid` _targetactor
        (:`Is Valid`
          (bind _asbp_base_character (cast `/Game/Blueprints/Game/Characters/BP_BaseCharacter` _targetactor)
            (:`then`
              (`/Game/Blueprints/Game/Characters/BP_BaseCharacter.TryOnHit` _asbp_base_character _instigator _damage))
            (:`CastFailed`
              (`GameplayStatics.ApplyDamage` _targetactor _damage null _instigator) ; Non-Characters
            )))
        (:`Is Not Valid`
          _))
      (set `self._canDealDamage` false))))

(fn `Attach`
  (params (Component :type "PrimitiveComponent Object Reference") (SocketName :type Name))
  (`self.SetActorEnableCollision` false)
  (`PrimitiveComponent.SetSimulatePhysics` (`self.SkeletalMesh`) false)
  (`self.K2_AttachToComponent` Component SocketName "KeepWorld" "KeepWorld" "KeepWorld"))

(fn `Penetrate`
  (params (hitLocation :type "Vector Structure") (depth :type "Float (single-precision)" :default 10.0))
  (`self.K2_SetActorLocation` (+ hitLocation (* (`self.GetActorForwardVector`) depth))))

(fn `UserConstructionScript`)