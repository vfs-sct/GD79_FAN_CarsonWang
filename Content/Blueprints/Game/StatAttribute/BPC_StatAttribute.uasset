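; Actor component for a numeric attribute such as health or mana, starting at max on BeginPlay.
; Adjust functions clamp the current value between zero and max and keep max positive, firing dispatchers for value changes and reaching zero.
; A looping timer applies regen per tick while below max and not paused.
; Changing the regen rate clears and restarts the timer to avoid stacked ticks.
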(event `self.ReceiveBeginPlay`
  (set `self._currentValue` (`self.maxValue`))
  (`self.OnValueChanged`)
  (`self.OnStartRegenCheck`) ; If your regen is at 0, this won't actually do anything.
)

(event `OnStartRegenCheck`
  ;[1 1 1] Regen on this attribute if applicable. Attributes like mana/health can benefit from regen. Mana is defaulted with regen
  (if (!= (`self.regenPerTick`) 0.0)
    (`self.EndRegen`) ; Kill any existing regen timer handler, then restart it\nin the next node. This will make\nSure there isn't multiple regen ticks happening.
    (bind _returnvalue (`KismetSystemLibrary.K2_SetTimerDelegate` (delegate `OnRegen`) (`self.regenTick`) true))
    (set `self._regenHandler` _returnvalue)))

(event `OnRegen`
  ;[1 1 1] Regen on this attribute if applicable. Attributes like mana/health can benefit from regen. Mana is defaulted with regen
  (`self.Regen` (`self.regenPerTick`)))

(event `OnEndRegen`
  ;[1 1 1] Regen on this attribute if applicable. Attributes like mana/health can benefit from regen. Mana is defaulted with regen
  (`self.EndRegen`))

(fn `AdjustCurrentValue`
  (params (value :type "Float (double-precision)"))
  (bind _returnvalue (+ value (`self._currentValue`)))
  (if (> _returnvalue (`self.maxValue`))
    ;[1 1 1] Don't allow current health to exceed max health
    (set `self._currentValue` (`self.maxValue`))
    (else
      ;[1 1 1] Zero Check
      (if (<= _returnvalue 0.0)
        (set `self._currentValue` 0.0)
        (`self.OnZeroReached`)
        (else
          (set `self._currentValue` _returnvalue)))))
  (`self.OnValueChanged`))

(fn `AdjustMaxValue`
  (params (valkue :type "Float (double-precision)"))
  (bind _returnvalue (+ valkue (`self.maxValue`)))
  (if (<= _returnvalue 0.0)
    (set `self.maxValue` (`self.maximumMinimumValue`)) ; Never drop max below the minimum value for the MAX
    (else
      (set `self.maxValue` _returnvalue)))
  (`self.OnValueChanged`))

(fn `AdjustRegenValue`
  (params (value :type "Float (double-precision)"))
  (bind _output_get (set `self.regenPerTick` (+ value (`self.regenPerTick`))))
  (`self.EndRegen`) ; Kill any existing regen, then restart it\nafter if the value isn't 0. This will make\nSure there isn't multiple regen ticks.
  (`self.OnRegenValueChangedComplete` _output_get)
  (if (!= _output_get 0.0)
    (`self.OnStartRegenCheck`)))

(fn `EndRegen`
  (if (`KismetSystemLibrary.K2_IsValidTimerHandle` (`self._regenHandler`))
    (`KismetSystemLibrary.K2_ClearAndInvalidateTimerHandle` (`self._regenHandler`))))

(fn `GetCurrentValue`
  (returns (_currentHealth :type "Float (double-precision)"))
  (return (`self._currentValue`)))

(fn `GetMaxValue`
  (returns (_maxHealth :type "Float (double-precision)"))
  (return (`self.maxValue`)))

(fn `GetNormalizedCurrentValue`
  (returns (ReturnValue :type "Float (double-precision)"))
  (return (/ (`self._currentValue`) (`self.maxValue`))))

(fn `GetRegenValue`
  (returns (_regenPerSecond :type "Float (double-precision)"))
  (return (`self.regenPerTick`)))

(fn `IsOverZero`
  (returns (ReturnValue :type Boolean))
  (return (> (`self._currentValue`) 0.0)))

(fn `OnValueChanged`
  (`self.OnValueChangedComplete` (`self._currentValue`) (`self.maxValue`) (`self.GetNormalizedCurrentValue`)))

(fn `OnZeroReached`
  (`self.OnZeroValueReachedComplete`))

(fn `Regen`
  (params (value :type "Float (double-precision)"))
  (if (and (!= value 0.0) (< (`self.GetCurrentValue`) (`self.GetMaxValue`)) (not (`self._isRegenPaused`)))
    (`self.AdjustCurrentValue` value)))

(fn `ToggleRegen`
  (params (isPaused :type Boolean))
  (set `self._isRegenPaused` isPaused))