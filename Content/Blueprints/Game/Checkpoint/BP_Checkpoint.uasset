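; BP_Checkpoint is a checkpoint actor that records player progress by ID when the player overlaps its box.
; The game instance's checkpoint-set event makes the matching checkpoint play triggered and looping feedback and the others deactivate theirs.
; Lower IDs are rejected unless backtracking is allowed, and BeginPlay restores the current checkpoint's loop.
; In the editor, the construction script auto-assigns a free ID on placement and flags duplicates through colored text.
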(event `self.ReceiveBeginPlay`
  (add `/Game/Blueprints/Game/GameInstance/BP_CustomGameInstance.OnCheckpointSet` (`/Game/Blueprints/Game/Utility/BP_FunctionLibrary.GetCustomGameInstance`) (delegate `OnCheckpointSet_Event`))
  (if (== (`/Game/Blueprints/Game/Utility/BP_FunctionLibrary.GetCurrentCheckpointID`) (`self._id`))
    (`self.PlayActivatedLoopFeedback`)))

(event `OnCheckpointSet_Event`
  (params (CheckpointId :type Integer))
  (if (== CheckpointId (`self._id`))
    (`self.OnCheckpointActivated`)
    (else
      (`self.OnCheckpointDeactivated`))))

(event `self.Box.OnComponentBeginOverlap`
  (params (OverlappedComponent :type "PrimitiveComponent Object Reference") (OtherActor :type "Actor Object Reference") (OtherComp :type "PrimitiveComponent Object Reference") (OtherBodyIndex :type Integer) (bFromSweep :type Boolean) (SweepResult :type "HitResult Structure (by ref)"))
  (`/Game/Blueprints/Game/Utility/BP_MacroLibrary.IsPlayer` OtherActor
    (:`true`
      (`/Game/Blueprints/Game/Utility/BP_FunctionLibrary.SetCurrentCheckpointID` (`self._id`) (`self._isAllowBacktracking`)))))

(fn `GetID`
  (returns (_id :type Integer))
  (return (`self._id`)))

(fn `JustSpawnedCheck`
  (locals (_allCheckpointIds :type "Array of Integer") (_checkIndex :type Integer))
  (bind __checkindex (`local._checkIndex`))
  (if (`self._justSpawned`)
    (set `self._justSpawned` false) ; Turn this off so the valid ID check\nis no longer called after dropping\nitem into scene
    (bind _outactors (`GameplayStatics.GetAllActorsOfClass` "BP_Checkpoint_C"))
    (for _array_element _outactors
      (bind __id (`self.GetID` _array_element))
      (if (and (!= _array_element self) (not (`KismetArrayLibrary.Array_Contains` (`local._allCheckpointIds`) __id)))
        (`KismetArrayLibrary.Array_AddUnique` (`local._allCheckpointIds`) __id)))
    ;[1 1 1] Auto assign a VALID id
    (if (`KismetArrayLibrary.Array_Contains` (`local._allCheckpointIds`) (`local._checkIndex`)) :!label _label
      (`/Engine/EditorBlueprintResources/StandardMacros.IncrementInt` __checkindex
        (:`  `
          (goto _label)))
      (else
        (`self.SetID` __checkindex)))))

(fn `OnCheckpointActivated`
  (`self.PlayActivatedLoopFeedback`)
  (`self.PlayTriggeredFeedback`))

(fn `OnCheckpointDeactivated`
  (`ActorComponent.Deactivate` (`self.ActivatedLoopFeedback`))
  (`ActorComponent.Deactivate` (`self.TriggeredFeedback`)))

(fn `PlayActivatedLoopFeedback`
  (`ActorComponent.Activate` (`self.ActivatedLoopFeedback`) true))

(fn `PlayTriggeredFeedback`
  (`ActorComponent.Activate` (`self.TriggeredFeedback`) true))

(fn `Set IDText for Editor`
  (params (InInt :type Integer))
  (locals (_text :type Text) (_duplicateIdColor :type "Color Structure" :default (struct :`B` 48 :`R` 255 :`A` 255)) (_validIdColor :type "Color Structure" :default (struct :`B` 65 :`G` 255)))
  (bind __id (`self._id`))
  (`TextRenderComponent.SetTextRenderColor` (`self.TextRender`) (`local._validIdColor`))
  (set `local._text` (`KismetTextLibrary.Conv_StringToText` (`KismetStringLibrary.Concat_StrStr` "ID: " (`KismetStringLibrary.Conv_IntToString` InInt))))
  (bind _outactors (`GameplayStatics.GetAllActorsOfClass` "BP_Checkpoint_C"))
  (for _array_element _outactors
    (if (!= self _array_element)
      (if (== (`self.GetID` _array_element) __id)
        (set `local._text` (`KismetTextLibrary.Conv_StringToText` (`KismetStringLibrary.Concat_StrStr` "DUPLICATE ID OF '" (`KismetStringLibrary.Conv_IntToString` __id) "' FOUND! \nREPLACE WITH A UNIQUE ID")))
        (`TextRenderComponent.SetTextRenderColor` (`self.TextRender`) (`local._duplicateIdColor`))
        (break))))
  (`TextRenderComponent.K2_SetText` (`self.TextRender`) (`local._text`)))

(fn `SetID`
  (params (_id :type Integer))
  (returns (ID :type Integer))
  (bind _output_get (set `self._id` _id))
  (return _output_get))

(fn `UserConstructionScript`
  (`self.JustSpawnedCheck`)
  (`self.Set IDText for Editor` (`self._id`)))