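; BP_CheckpointData is a data holder for the checkpoint system.
; It stores a spawn value, a current ID and a text order, each exposed through a plain getter and setter.
; It has no other logic, and only the spawn setter also returns the value it stores.
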(fn `GetCurrentID`
  (returns (_currentID :type Integer))
  (return (`self._currentID`)))

(fn `GetSpawn`
  (returns (_spawn :type "/Game/Blueprints/Game/Checkpoint/Tools/EN_Spawn Enum"))
  (return (`self._spawn`)))

(fn `GetTextOrder`
  (returns (_textOrder :type Text))
  (return (`self._textOrder`)))

(fn `SetCurrentID`
  (params (_currentID :type Integer))
  (set `self._currentID` _currentID))

(fn `SetSpawn`
  (params (_spawn :type "/Game/Blueprints/Game/Checkpoint/Tools/EN_Spawn Enum" :default "NewEnumerator0"))
  (returns (Spawn :type "/Game/Blueprints/Game/Checkpoint/Tools/EN_Spawn Enum"))
  (bind _output_get (set `self._spawn` _spawn))
  (return _output_get))

(fn `SetTextOrder`
  (params (_textOrder :type Text))
  (set `self._textOrder` _textOrder))