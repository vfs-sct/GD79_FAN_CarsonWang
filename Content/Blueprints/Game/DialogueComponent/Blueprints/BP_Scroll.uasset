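; BP_Scroll is an interactable pickup that adds an amount of a condition, noted as 'Scroll', to the player's conditions.
; It binds to its DialogueComponent's input event at BeginPlay and acts only while the player overlaps.
; A DoOnce, reset by input received outside overlap, gates the pickup sound and condition change.
; It then destroys the interaction ring and itself, both only if that ring is valid.
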(event `self.ReceiveBeginPlay`
  (add `/Game/Blueprints/Game/DialogueComponent/Blueprints/Dialogue_Component.ED Input Received` (`self.Dialogue_Component`) (delegate `Input Received`)) ; Ensures this actor will receive input when\nplayer presses 'interact' button
)

(event `Input Received`
  (bind _interaction_ring (`/Game/Blueprints/Game/DialogueComponent/Blueprints/Dialogue_Component.Interaction Ring` (`self.Dialogue_Component`)))
  ;[0.08731 0.4212 1] Add 'Scroll' to player conditions & delete this actor
  (if (`/Game/Blueprints/Game/DialogueComponent/Blueprints/Dialogue_Component.Overlaping Player?` (`self.Dialogue_Component`))
    (`/Engine/EditorBlueprintResources/StandardMacros.DoOnce` false :!label _label
      (:`Completed`
        (`GameplayStatics.PlaySound2D` (`self.🔊 Pickup Sound`) 1.0 1.0 0.0 null null)
        (`/Game/Blueprints/Game/DialogueComponent/Blueprints/Dialogue_Component.Change Player Condition Amount` (`self.Dialogue_Component`) (`self.Condition Key`) (`self.Amount (+)`))
        (`/Engine/EditorBlueprintResources/StandardMacros.IsValid` _interaction_ring
          (:`Is Valid`
            (`self.K2_DestroyActor` _interaction_ring)
            (`self.K2_DestroyActor` self)))))
    (else
      (goto _label :!via `Reset`))))

(fn `UserConstructionScript`)