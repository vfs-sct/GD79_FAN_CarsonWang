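; Dialogue-driven cinematic mover that carries a static mesh or target actor, plus an optional cine camera, along a spline.
; BeginPlay or dialogue events enable Tick when the start branch matches, advancing along the spline.
; The camera can track targets, fade and switch focus to a second target, while player conditions and another actor's dialogue branch are updated.
; Completion or a permitted skip stops Tick, optionally saving position or destroying the actors.
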(event `self.ReceiveBeginPlay`
  (bind ___start_on_branch (`self.↗ Start On Branch`))
  (bind _dialogue_component (`self.Dialogue_Component`))
  (bind _returnvalue_location (`KismetMathLibrary.BreakTransform` (`SplineComponent.GetTransformAtDistanceAlongSpline` (`self.Spline`) (* (`self.↗ Start Distance`) (/ (`SplineComponent.GetSplineLength` (`self.Spline`)) 1.0)) "World" false)))
  (`self.Set All Vars From Structs`)
  (add `/Game/Blueprints/Game/DialogueComponent/Blueprints/Dialogue_Component.ED Dialogue Started` _dialogue_component (delegate `Dialogue Started`))
  (add `/Game/Blueprints/Game/DialogueComponent/Blueprints/Dialogue_Component.ED Dialogue Ended / Continued` _dialogue_component (delegate `Dialogue Ended`))
  (if (`self.💾 Use Save System?`)
    (`KismetSystemLibrary.Delay` 0.01)
    (bind _bp_dc_save_ref (`/Game/Blueprints/Game/DialogueComponent/Blueprints/Essentials/BP_DC_Library.Get DC Player's Save REF`))
    (`/Engine/EditorBlueprintResources/StandardMacros.IsValid` _bp_dc_save_ref
      (:`Is Valid`
        (set `self.↗ Start Distance` (`/Game/Blueprints/Game/DialogueComponent/Blueprints/Dialogue_Component.Spline Location` (`self.Dialogue_Component`)))
        (`self.Actor Location` _returnvalue_location))
      (:`Is Not Valid`
        _)))
  (`|ExecutionSequence`
    (:`then_0`
      (bind _player_character_s_dialogue_component (`/Game/Blueprints/Game/DialogueComponent/Blueprints/Essentials/BP_DC_Library.Get Player Character's Dialogue Component`))
      (add `/Game/Blueprints/Game/DialogueComponent/Blueprints/Dialogue_Component.ED Interact Button Pressed` _player_character_s_dialogue_component (delegate `Player Pressing Input`)))
    (:`then_1`
      (if (`self.↗ Start On Begin Play?`)
        (if (`KismetStringLibrary.IsEmpty` ___start_on_branch) :!label _label
          (`self.SetActorTickEnabled` true :!label _label_2)
          (elif (`KismetStringLibrary.EqualEqual_StrStr` (`/Game/Blueprints/Game/DialogueComponent/Blueprints/Dialogue_Component.🏁 START 🏁` (`self.Dialogue_Component`)) ___start_on_branch)
            (goto _label_2)))))))

(event `Dialogue Started`
  (goto _label))

(event `Dialogue Ended`
  (goto _label))

(event `Skip / End Sequence`
  (`self.SetActorTickEnabled` false :!label _label_3)
  (set `self.↗ Start Distance` 0.0)
  (if (`self.💾 Save On End?`)
    (`self.Save Position  `
      (:`then`
        _)
      (:`OutputPin`
        (set `self.↗ Start Distance` 0.0 :!label _label_4)))
    (else
      (goto _label_4)))
  (if (`self.↗ Destroy On End?`)
    (`self.K2_DestroyActor` (`ActorComponent.GetOwner` (`self.Actor To Move`)))
    (`self.K2_DestroyActor`)))

(event `self.ReceiveTick`
  (params (DeltaSeconds :type "Float (single-precision)"))
  (bind _cinecamera (`self.CineCamera`))
  (bind ___condition_key (`self.🗣 Condition Key`))
  (bind ___condition_value____ (`self.🗣 Condition Value (+)`))
  (bind _output_get (set `self.Time` DeltaSeconds))
  (`|ExecutionSequence`
    (:`then_0`
      (bind _player_character_s_dialogue_component (`/Game/Blueprints/Game/DialogueComponent/Blueprints/Essentials/BP_DC_Library.Get Player Character's Dialogue Component`))
      (`/Engine/EditorBlueprintResources/StandardMacros.IsValid` _player_character_s_dialogue_component
        (:`Is Valid`
          (bind ((`Condition_5_1122152E46EF2FEEFF08CF9198C32887` _condition)) (break `/Game/Blueprints/Game/DialogueComponent/Data/Structs/Dialogue/Essentials/S_Player_Condition_Checks` (`/Game/Blueprints/Game/DialogueComponent/Blueprints/Dialogue_Component.⚖ Player Conditions ⚖` _player_character_s_dialogue_component)))
          (bind (_value _returnvalue) (`BlueprintMapLibrary.Map_Find` _condition ___condition_key))
          (if _returnvalue
            (`BlueprintMapLibrary.Map_Add` _condition ___condition_key (+ _value ___condition_value____))
            (else
              (`BlueprintMapLibrary.Map_Add` _condition ___condition_key ___condition_value____))))
        (:`Is Not Valid`
          _))
      (bind ___actor_to_effect (`self.🗣 Actor To Effect`)
        (:`then`
          (bind _returnvalue_2 (`self.GetComponentByClass` ___actor_to_effect "/Game/Blueprints/Game/DialogueComponent/Blueprints/Dialogue_Component.Dialogue_Component_C"))
          (`/Engine/EditorBlueprintResources/StandardMacros.IsValid` _returnvalue_2
            (:`Is Valid`
              (set `/Game/Blueprints/Game/DialogueComponent/Blueprints/Dialogue_Component.🏁 START 🏁` (`self.🗣 🏁 START 🏁`) _returnvalue_2) ; Changes NPC's dialogue
            )
            (:`Is Not Valid`
              _)))
        (:`else`
          _))
      (`/Engine/EditorBlueprintResources/StandardMacros.DoOnce` false
        (:`Completed`
          (if (`self.🎥 Use Camera Fade?`)
            (`PlayerCameraManager.StartCameraFade` (`GameplayStatics.GetPlayerCameraManager` 0) (`self.🎥 Fade Start`) (`self.🎥 Fade End`) (`self.🎥 Fade Duration`) (`self.🎥 Fade Color`) (`self.🎥 Should Fade Audio`) (`self.🎥 Hold when Done`))))))
    (:`then_1`
      (bind _output_get_2 (set `self.↗ Start Distance` (+ (* _output_get (`self.↗ Speed`)) (`self.↗ Start Distance`))))
      (bind _output_get_3 (set `self.Spine Distance` (/ (* _output_get_2 (/ (`SplineComponent.GetSplineLength` (`self.Spline`)) 1.0)) (`SplineComponent.Duration` (`self.Spline`)))))
      (if (`self.🎯 Use Spline Location?`)
        (bind (_returnvalue_location _returnvalue_rotation) (`KismetMathLibrary.BreakTransform` (`SplineComponent.GetTransformAtDistanceAlongSpline` (`self.Spline`) _output_get_3 "World" false)))
        (`self.Actor Location` _returnvalue_location))
      (if (`self.🎯 Use Spline Rotation?`)
        (`self.Actor Rotation` _returnvalue_rotation))
      (`|ExecutionSequence`
        (:`then_0`
          (if (`self.📷 Change To 2nd Target?`)
            (`/Engine/EditorBlueprintResources/StandardMacros.DoOnce` false
              (:`Completed`
                (`KismetSystemLibrary.Delay` (`self.📷 Delay Until Change`))
                (bind ___2nd_target (`self.📷 2nd Target`)
                  (:`then`
                    (set `self.🎥 1st Target` ___2nd_target)
                    (set `CineCameraComponent.FocusSettings` (make `CameraFocusSettings` :`ManualFocusDistance` (`self.Next Focus Distance`) :`bSmoothFocusChanges` true :`FocusSmoothingInterpSpeed` (`self.Next Focus Smoothing Interp Speed`) :`FocusOffset` (`self.Next Focus Offset`)) _cinecamera)
                    (set `CineCameraComponent.CurrentAperture` (`self.Next Aperture`) _cinecamera)
                    (set `CameraComponent.PostProcessSettings` (`self.Next Post Process Settings`) (`self.CineCamera`)))
                  (:`else`))))))
        (:`then_1`
          (if (not (`self.🎯 Use Spline Rotation?`))
            (bind ___1st_target (`self.🎥 1st Target`)
              (:`then`
                (`self.Actor Rotation` (`KismetMathLibrary.Conv_VectorToRotator` (+ (`self.K2_GetActorLocation` ___1st_target) (`self.🎥 Lookat Offset`)))))
              (:`else`
                _)))
          (if (>= (`self.↗ Start Distance`) (/ (`SplineComponent.Duration` (`self.Spline`)) 1.0))
            (goto _label_3)))))))

(event `Player Pressing Input`
  (if (and (`self.IsActorTickEnabled`) (`self.🎥 Can Skip Sequence?`))
    (set `self.↗ Start Distance` 1.0)
    (`self.Skip / End Sequence`)))

(fn `UserConstructionScript`
  (bind _staticmesh (`self.StaticMesh`))
  (bind ___hide_static_mesh_in_game_ (`self.↗ Hide Static Mesh In Game?`))
  (bind (_returnvalue_location _returnvalue_rotation) (`KismetMathLibrary.BreakTransform` (`SplineComponent.GetTransformAtDistanceAlongSpline` (`self.Spline`) (* (`self.↗ Start Distance`) (/ (`SplineComponent.GetSplineLength` (`self.Spline`)) 1.0)) "World" false)))
  (`self.Set All Vars From Structs`)
  (bind _cinecamera (`self.CineCamera`)
    (:`then`
      (set `CineCameraComponent.FocusSettings` (make `CameraFocusSettings` :`ManualFocusDistance` (`self.🎥 Focus Distance`) :`bSmoothFocusChanges` true :`FocusSmoothingInterpSpeed` (`self.🎥 Focus Interp`) :`FocusOffset` (`self.🎥 Focus Offset`)) _cinecamera)
      (set `CameraComponent.PostProcessSettings` (`self.🎥 Post Process Settings`) (`self.CineCamera`))
      (set `CineCameraComponent.CurrentAperture` (`self.🎥 Current Aperture`) _cinecamera))
    (:`else`
      _))
  (set `SplineComponent.Duration` (`self.↗ Duration`) (`self.Spline`))
  (set `self.↗ Start Distance` (`self.↗ Start Distance`))
  (`self.Actor Location` _returnvalue_location)
  (if (`self.🎯 Use Spline Rotation?`)
    (`self.Actor Rotation` _returnvalue_rotation))
  (`SceneComponent.SetHiddenInGame` _staticmesh ___hide_static_mesh_in_game_ false)
  (if ___hide_static_mesh_in_game_
    (`PrimitiveComponent.SetCollisionEnabled` _staticmesh "NoCollision")))