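; Blueprint function library of lookup helpers for the Dialogue Component system.
; It finds components on actors or player character 0, with validity-filtered variants, and exposes the player's save reference.
; Speaker helpers follow an owner component's REF actor to set or read CurrentlySpeakingActor on that actor's component.
; The all-actors search scans every Actor for the component, but its return node is unconnected.
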(fn `Get All Actors Using Dialogue Component`
  (returns (`Actor With Component` :type "Actor Object Reference") (`Dialogue Component (Validated)` :type "/Game/Blueprints/Game/DialogueComponent/Blueprints/Dialogue_Component Object Reference"))
  (locals (`Actor With Dialogue Component` :type "Array of Actor Object Reference"))
  (bind _outactors (`GameplayStatics.GetAllActorsOfClass` null "/Script/Engine.Actor"))
  (for _array_element _outactors
    (`/Engine/EditorBlueprintResources/StandardMacros.IsValid` (`Actor.GetComponentByClass` _array_element "/Game/Blueprints/Game/DialogueComponent/Blueprints/Dialogue_Component.Dialogue_Component_C")
      (:`Is Valid`
        (`KismetArrayLibrary.Array_Add` (`local.Actor With Dialogue Component`) _array_element)))))

(fn `Get Current DC Speaker`
  (params (`DC Owner` :type "Actor Object Reference"))
  (returns (`Currently Speaking Actor` :type "Actor Object Reference"))
  (bind _ref (`/Game/Blueprints/Game/DialogueComponent/Blueprints/Dialogue_Component.REF` (`self.Get Dialogue Component` `DC Owner`))
    (:`then`
      (bind (_actor_ _dialogue_component__validated_) (`self.Get Vaild Dialogue Component Of Actor` _ref))
      (return (`/Game/Blueprints/Game/DialogueComponent/Blueprints/Dialogue_Component.Currently Speaking Actor` _dialogue_component__validated_)))
    (:`else`)))

(fn `Get DC Player's Save REF`
  (returns (`BP DC Save REF` :type "/Game/Blueprints/Game/DialogueComponent/Blueprints/Essentials/BP_DC_Save Object Reference"))
  (bind _player_character_s_dialogue_component (`self.Get Player Character's Dialogue Component` null))
  (`/Engine/EditorBlueprintResources/StandardMacros.IsValid` _player_character_s_dialogue_component
    (:`Is Valid`
      (return (`/Game/Blueprints/Game/DialogueComponent/Blueprints/Dialogue_Component.BP DC Save REF` _player_character_s_dialogue_component)))
    (:`Is Not Valid`
      (return null))))

(fn `Get Dialogue Component`
  (params (`DC Owner` :type "Actor Object Reference"))
  (returns (`Dialogue Component` :type "/Game/Blueprints/Game/DialogueComponent/Blueprints/Dialogue_Component Object Reference"))
  (return (`Actor.GetComponentByClass` `DC Owner` "/Game/Blueprints/Game/DialogueComponent/Blueprints/Dialogue_Component.Dialogue_Component_C")))

(fn `Get Dialogue Component Of Actor`
  (params (Actor :type "Actor Object Reference"))
  (returns (`Actor ` :type "Actor Object Reference") (`Dialogue Component (Validated)` :type "/Game/Blueprints/Game/DialogueComponent/Blueprints/Dialogue_Component Object Reference"))
  (return Actor (`Actor.GetComponentByClass` Actor "/Game/Blueprints/Game/DialogueComponent/Blueprints/Dialogue_Component.Dialogue_Component_C")))

(fn `Get NOT Vaild Dialogue Component Of Actor`
  (params (Actor :type "Actor Object Reference"))
  (returns (`Actor ` :type "Actor Object Reference"))
  (`/Engine/EditorBlueprintResources/StandardMacros.IsValid` (`Actor.GetComponentByClass` Actor "/Game/Blueprints/Game/DialogueComponent/Blueprints/Dialogue_Component.Dialogue_Component_C")
    (:`Is Not Valid`
      (return Actor))))

(fn `Get Player Character's Dialogue Component`
  (returns (`Player Character's Dialogue Component` :type "/Game/Blueprints/Game/DialogueComponent/Blueprints/Dialogue_Component Object Reference"))
  (bind _returnvalue (`GameplayStatics.GetPlayerCharacter` null))
  (`/Engine/EditorBlueprintResources/StandardMacros.IsValid` _returnvalue
    (:`Is Valid`
      (bind (_actor_ _dialogue_component__validated_) (`self.Get Vaild Dialogue Component Of Actor` _returnvalue))
      (return _dialogue_component__validated_))))

(fn `Get Vaild Dialogue Component Of Actor`
  (params (Actor :type "Actor Object Reference"))
  (returns (`Actor ` :type "Actor Object Reference") (`Dialogue Component (Validated)` :type "/Game/Blueprints/Game/DialogueComponent/Blueprints/Dialogue_Component Object Reference"))
  (bind _returnvalue (`Actor.GetComponentByClass` Actor "/Game/Blueprints/Game/DialogueComponent/Blueprints/Dialogue_Component.Dialogue_Component_C"))
  (`/Engine/EditorBlueprintResources/StandardMacros.IsValid` _returnvalue
    (:`Is Valid`
      (return Actor _returnvalue))))

(fn `Set Current DC Speaker`
  (params (`DC Owner` :type "Actor Object Reference"))
  (bind _ref (`/Game/Blueprints/Game/DialogueComponent/Blueprints/Dialogue_Component.REF` (`self.Get Dialogue Component` `DC Owner`))
    (:`then`
      (bind (_actor_ _dialogue_component__validated_) (`self.Get Vaild Dialogue Component Of Actor` _ref))
      (set `/Game/Blueprints/Game/DialogueComponent/Blueprints/Dialogue_Component.Currently Speaking Actor` `DC Owner` _dialogue_component__validated_) ; Sets owner as REF's Speaking Actor
      (return))
    (:`else`)))