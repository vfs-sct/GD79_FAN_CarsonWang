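; Base character for player and AI, handling combat reactions, health, death and team identity.
; Incoming damage makes noise for AI hearing, then resolves as dodge, facing-checked block (bypassed by unblockable traps) or hit.
; Hits drive Health, floating text, non-overlapping voice SFX and stagger montages, with stun handled separately.
; Zero health stops AI and regen, loosens collision and broadcasts death; OnBlockHit lets the player override leftover block damage.
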(event `self.ReceiveBeginPlay`
  (add `self.OnTakeAnyDamage` (delegate `OnTakeAnyDamage_Event`))
  (add `self.OnDestroyed` (delegate `OnDestroyed_Event`)))

(event `OnTakeAnyDamage_Event` :!signature `self.OnTakeAnyDamage`
  (params (DamagedActor :type "Actor Object Reference") (Damage :type "Float (single-precision)") (DamageType :type "DamageType Object Reference") (InstigatedBy :type "Controller Object Reference") (DamageCauser :type "Actor Object Reference"))
  (`self.TryOnHit` DamageCauser Damage))

(event `OnDestroyed_Event` :!signature `self.OnDestroyed`
  (params (DestroyedActor :type "Actor Object Reference"))
  (`self.OnDeathComplete`))

(event `OnStun`
  (bind _stunanim (`self.StunAnim`))
  ;[1 1 1] Stun
  (`/Engine/EditorBlueprintResources/StandardMacros.IsValid` _stunanim
    (:`Is Valid`
      (`self.OnStunned`)
      (`|PlayMontage` (`self.Mesh`) _stunanim
        (:`OnCompleted`
          _)
        (:`OnInterrupted`
          _))
      (`self.SetIsStunned` false))))

(event `OnHitRecovery`
  (bind _hitrecoveryanim (`self.hitRecoveryAnim`))
  ;[1 1 1] HitRecovery
  (`/Engine/EditorBlueprintResources/StandardMacros.IsValid` _hitrecoveryanim
    (:`Is Valid`
      (`self.SetIsStaggered` true)
      (`self.StopAnimMontage` null) ; pass in null anim montage to stop\ncurrently playing montage, if any.
      (`|PlayMontage` (`self.Mesh`) _hitrecoveryanim
        (:`OnCompleted`
          _)
        (:`OnInterrupted`
          _))
      (`self.SetIsStaggered` false))))

(event `self.ReceivePossessed`
  (params (NewController :type "Controller Object Reference"))
  ;[1 1 1] Possessed
  (set `self._controller` NewController))

(event `self.Health.OnZeroValueReachedComplete`
  ;[1 1 1] On Death
  (`self.OnDeath`))

(event `OnAttackShoutCallout`
  ;[1 1 1] On Attack Shout Callout
  (if (not (`self.IsSpeakingSFXPlaying`))
    (bind _duration (`self.PlayRandomOnAttackSFX`))
    (`KismetSystemLibrary.Delay` _duration)
    (set `self.IsSpeakingSFXPlaying` false)))

(event `OnHitShoutCallout`
  ;[1 1 1] On Hit Shout Callout
  (if (not (`self.IsSpeakingSFXPlaying`))
    (bind _duration (`self.PlayRandomOnHitSFX`))
    (`KismetSystemLibrary.Delay` _duration)
    (set `self.IsSpeakingSFXPlaying` false)))

(fn `CheckBlockAngle`
  (params (Attackter :type "Actor Object Reference"))
  (returns (isAttackWithinBlockAngle :type Boolean))
  (locals (_canBlock :type Boolean :default false))
  (`/Engine/EditorBlueprintResources/StandardMacros.IsValid` Attackter
    (:`Is Valid`
      (`/Game/Blueprints/Game/Utility/BP_MacroLibrary.IsTargetInfrontOfActorFacing` self Attackter ; Dot product. Only block attacks infront\nof the actor's facing direction
        (:`TargetIsInfront`
          (set `local._canBlock` true :!label _label))
        (:`TargetIsBehind`
          (set `local._canBlock` false))))
    (:`Is Not Valid`
      (goto _label)))
  (return (`local._canBlock`)))

(fn `End Blocking`
  (`self.SetIsBlocking` false))

(fn `GetIsAlive`
  (returns (ReturnValue :type Boolean))
  (return (`/Game/Blueprints/Game/StatAttribute/BPC_StatAttribute.IsOverZero` (`self.Health`))))

(fn `GetIsBlocking`
  (returns (_isBlocking :type Boolean))
  (return (`self._isBlocking`)))

(fn `GetIsDodging`
  (returns (_isDodging :type Boolean))
  (return (`self._isDodging`)))

(fn `GetIsStaggered`
  (returns (isStaggered :type Boolean))
  (return (`self._isStaggered`)))

(fn `GetIsStunned`
  (returns (_isStunned :type Boolean))
  (return (`self._isStunned`)))

(fn `GetTeam`
  (returns (team :type Integer))
  (return (`self.TeamID`)))

(fn `IsTargetable`
  (returns (isTargetable :type Boolean))
  (return (`/Game/Blueprints/Game/StatAttribute/BPC_StatAttribute.IsOverZero` (`self.Health`))))

(fn `MakeNoiseDetection`
  (params (Loudness :type "Float (single-precision)" :default 1.0) (MaxRange :type "Float (single-precision)" :default 500.0))
  (`self.MakeNoise` Loudness self (`self.K2_GetActorLocation`) MaxRange))

(fn `OnBlockHit`
  (params (Damage :type Integer))
  (returns (UnblockedDamage :type Integer))
  (bind _returnvalue (`self.K2_GetActorLocation`))
  ;[1 1 1] Base always returns no unblocked damage for ai. Player overrides differently.
  (`GameplayStatics.SpawnEmitterAtLocation` "/Game/FlexibleCombatSystem/DemoRoom/VFX/P_BlockImpact.P_BlockImpact" _returnvalue)
  (`GameplayStatics.PlaySoundAtLocation` "/Game/Audio/SFX/Magic_Spells_Sound_Effects_V2_0/Medieval_Combat_Sounds_BONUS/Shield_Metal_1_1.Shield_Metal_1_1" _returnvalue (struct) 1.0 1.0 0.0 null null null null)
  (return 0))

(fn `OnDeath`
  (bind _capsulecomponent (`self.CapsuleComponent`))
  (bind _returnvalue (`AIBlueprintHelperLibrary.GetAIController` self))
  ;[1 1 1] Stop running AI Logics
  (bind _asbp_base_aicontroller (cast `/Game/Blueprints/Game/AI/Controllers/BP_BaseAIController` (`self.GetController`))
    (:`then`
      (`/Game/Blueprints/Game/AI/Controllers/BP_BaseAIController.StopRunningLogics` _asbp_base_aicontroller))
    (:`CastFailed`
      _))
  (`/Game/Blueprints/Game/StatAttribute/BPC_StatAttribute.OnEndRegen` (`self.Mana`))
  (`/Game/Blueprints/Game/StatAttribute/BPC_StatAttribute.OnEndRegen` (`self.Health`))
  ;[1 1 1] Remove collision on some channels on death so player and dynamic objects can pass through
  (`PrimitiveComponent.SetCollisionResponseToChannel` (`self.Mesh`) "ECC_Visibility" "ECR_Ignore")
  (`PrimitiveComponent.SetCollisionResponseToChannel` _capsulecomponent "ECC_Visibility" "ECR_Ignore")
  (`PrimitiveComponent.SetCollisionResponseToChannel` _capsulecomponent "ECC_PhysicsBody" "ECR_Ignore")
  (`PrimitiveComponent.SetCollisionResponseToChannel` (`self.Mesh`) "ECC_PhysicsBody" "ECR_Ignore")
  (`PrimitiveComponent.SetCollisionResponseToChannel` _capsulecomponent "ECC_Pawn" "ECR_Ignore")
  (`PrimitiveComponent.SetCollisionResponseToChannel` (`self.Mesh`) "ECC_Pawn" "ECR_Ignore")
  (`self.StopAnimMontage` null) ; pass in null anim montage to stop\ncurrently playing montage, if any.
  (`/Engine/EditorBlueprintResources/StandardMacros.IsValid` _returnvalue
    (:`Is Valid`
      (`Controller.StopMovement` _returnvalue))
    (:`Is Not Valid`
      _))
  (`self.OnDeathComplete`))

(fn `OnDodged`)

(fn `OnHeal`
  (params (amount :type Integer))
  (bind _health (`self.Health`))
  (if (`/Game/Blueprints/Game/StatAttribute/BPC_StatAttribute.IsOverZero` _health)
    (`/Game/Blueprints/Game/Utility/BP_FunctionLibrary.CreateFloatingText` (`KismetStringLibrary.Conv_IntToString` amount) (`self.K2_GetActorLocation`) "NewEnumerator1")
    (`/Game/Blueprints/Game/StatAttribute/BPC_StatAttribute.AdjustCurrentValue` _health (`KismetMathLibrary.Conv_IntToDouble` amount))))

(fn `OnHit`
  (params (damage :type Integer))
  (bind _health (`self.Health`))
  (if (`/Game/Blueprints/Game/StatAttribute/BPC_StatAttribute.IsOverZero` _health)
    (`self.OnHitShoutCallout`)
    (`/Game/Blueprints/Game/Utility/BP_FunctionLibrary.CreateFloatingText` (`KismetStringLibrary.Conv_IntToString` damage) (`self.K2_GetActorLocation`) (`self.damagedFloatingTextType`))
    (`/Game/Blueprints/Game/StatAttribute/BPC_StatAttribute.AdjustCurrentValue` _health (`KismetMathLibrary.Conv_IntToDouble` (* damage -1)))
    (`self.OnHitRecovery`)))

(fn `OnStunned`
  (`self.SetIsStunned` true)
  (`self.StopAnimMontage` null) ; pass in null anim montage to stop\ncurrently playing montage, if any.
)

(fn `PlayRandomOnAttackSFX`
  (returns (Duration :type "Float (single-precision)"))
  (bind _outitem (`KismetArrayLibrary.Array_Random` (`self.OnAttackSfxList`)))
  (`/Engine/EditorBlueprintResources/StandardMacros.IsValid` _outitem
    (:`Is Valid`
      (`GameplayStatics.PlaySoundAtLocation` _outitem (`self.K2_GetActorLocation`) (struct) 1.0 1.0 0.0 null null null null)
      (set `self.IsSpeakingSFXPlaying` true)
      (return (`SoundBase.Duration` _outitem)))
    (:`Is Not Valid`
      (return 0.0))))

(fn `PlayRandomOnHitSFX`
  (returns (Duration :type "Float (single-precision)"))
  (bind _outitem (`KismetArrayLibrary.Array_Random` (`self.OnHitSfxList`)))
  (`/Engine/EditorBlueprintResources/StandardMacros.IsValid` _outitem
    (:`Is Valid`
      (`GameplayStatics.PlaySoundAtLocation` _outitem (`self.K2_GetActorLocation`) (struct) 1.0 1.0 0.0 null null null null)
      (set `self.IsSpeakingSFXPlaying` true)
      (return (`SoundBase.Duration` _outitem)))
    (:`Is Not Valid`
      (return 0.0))))

(fn `SetIsBlocking`
  (params (_isBlocking :type Boolean))
  (set `self._isBlocking` _isBlocking))

(fn `SetIsDodging`
  (params (_isDodging :type Boolean))
  (set `self._isDodging` _isDodging))

(fn `SetIsStaggered`
  (params (_isStaggered :type Boolean))
  (bind _output_get (set `self._isStaggered` _isStaggered))
  (`self.OnToggleStaggeredComplete` self _output_get))

(fn `SetIsStunned`
  (params (_isStunned :type Boolean))
  (bind _output_get (set `self._isStunned` _isStunned))
  (`self.OnToggleStunComplete` _output_get))

(fn `StartBlocking`
  (`self.SetIsBlocking` true))

(fn `StopRunningAILogics`
  (`BrainComponent.StopLogic` (`AIController.BrainComponent` (`AIBlueprintHelperLibrary.GetAIController` null)) ""))

(fn `TryOnHit`
  (params (DamageCauser :type "Actor Object Reference") (Damage :type "Float (double-precision)"))
  (returns (AttackResult :type "/Game/Blueprints/Game/AttackResult/EAttackResult Enum"))
  (locals (_damage :type Integer :default 0) (_damageResult :type "/Game/Blueprints/Game/AttackResult/EAttackResult Enum" :default "NewEnumerator0"))
  (`self.MakeNoiseDetection` 1.0 1000.0) ; Causes other AI to trigger hearing to come to check out\nthis location if in radius of this target being hit.
  (set `local._damage` (`KismetMathLibrary.FTrunc` Damage))
  (`self.OnHitAttempt` DamageCauser
    (:`Hit`
      (`self.OnHit` (`local._damage`) :!label _label))
    (:`Blocked`
      (bind _unblockeddamage (`self.OnBlockHit` (`local._damage`)))
      (bind _output_get (set `local._damage` (`KismetMathLibrary.Abs_Int` _unblockeddamage))) ; If not able to block the entire\ndamage, pass over left over damage
      (if (> _output_get 0)
        (goto _label)
        (else
          (set `local._damageResult` "NewEnumerator2"))))
    (:`Dodged`
      (`self.OnDodged`)
      (set `local._damageResult` "NewEnumerator1")))
  (return (`local._damageResult`)))

(fn `UserConstructionScript`)