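; BP_SandGolemCharacter is the Sand Golem enemy character, whose attacks knock targets back.
; Overlaps on its two hand spheres and an explosion sphere report attack contact, with colliders toggled from APB_SandGolem attack montages.
; ToggleMeleeDamageCollision switches either or both hand colliders by index, leaving the explosion sphere untouched.
; OnAttackCallback launches damaged targets away from the golem, scaling down the force on blocked hits.
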(event `self.ReceiveTick`
  (params (DeltaSeconds :type "Float (single-precision)"))
  (`parent.ReceiveTick` DeltaSeconds))

(event `self.LeftHandSphereDamageDetection.OnComponentBeginOverlap`
  (params (OverlappedComponent :type "PrimitiveComponent Object Reference") (OtherActor :type "Actor Object Reference") (OtherComp :type "PrimitiveComponent Object Reference") (OtherBodyIndex :type Integer) (bFromSweep :type Boolean) (SweepResult :type "HitResult Structure (by ref)"))
  ;[1 1 1] The Anim BP is setting the colliders enabled/disabled during attack Anims. Look at APB_SandGolem and it's attack anim montages as example.
  (`self.OnAttackTargetContact` OtherActor))

(event `self.RightHandSphereDamageDetection.OnComponentBeginOverlap`
  (params (OverlappedComponent :type "PrimitiveComponent Object Reference") (OtherActor :type "Actor Object Reference") (OtherComp :type "PrimitiveComponent Object Reference") (OtherBodyIndex :type Integer) (bFromSweep :type Boolean) (SweepResult :type "HitResult Structure (by ref)"))
  ;[1 1 1] The Anim BP is setting the colliders enabled/disabled during attack Anims. Look at APB_SandGolem and it's attack anim montages as example.
  (`self.OnAttackTargetContact` OtherActor))

(event `self.ExplosionSphereDamageDetection.OnComponentBeginOverlap`
  (params (OverlappedComponent :type "PrimitiveComponent Object Reference") (OtherActor :type "Actor Object Reference") (OtherComp :type "PrimitiveComponent Object Reference") (OtherBodyIndex :type Integer) (bFromSweep :type Boolean) (SweepResult :type "HitResult Structure (by ref)"))
  ;[1 1 1] The Anim BP is setting the colliders enabled/disabled during attack Anims. Look at APB_SandGolem and it's attack anim montages as example.
  (`self.OnAttackTargetContact` OtherActor))

(fn `OnAttackCallback`
  (params (attackTarget :type "/Game/Blueprints/Game/Characters/BP_BaseCharacter Object Reference") (attackResult :type "/Game/Blueprints/Game/AttackResult/EAttackResult Enum" :default "NewEnumerator0") (attackIndex :type Integer))
  (locals (_knockbackForce :type "Float (double-precision)"))
  ;[1 1 1] Sand golem's attacks will add force/knockback to the target
  (`/Engine/EditorBlueprintResources/StandardMacros.IsValid` attackTarget
    (:`Is Valid`
      (switch `/Game/Blueprints/Game/AttackResult/EAttackResult` attackResult
        (:`NewEnumerator0`
          (set `local._knockbackForce` (`self._knockbackHitForce`)))
        (:`NewEnumerator2`
          (set `local._knockbackForce` (* (`self._knockbackHitForce`) (`self._knockbackHitForceBlockedMultiplier`))) ; Add less force if blocked
        ))
      (`self.LaunchCharacter` attackTarget (* (`KismetMathLibrary.GetDirectionUnitVector` (`self.K2_GetActorLocation`) (`self.K2_GetActorLocation` attackTarget)) (`local._knockbackForce`)) false false))))

(fn `ToggleMeleeDamageCollision`
  (params (IsEnabled :type Boolean) (CollisionIndex :type Integer))
  (switch `int` CollisionIndex
    (:`Default`
      ;[1 1 1] Both hand slam attack and default Default will toggle all damage collision. Used to turn off everything on stun, etc.
      (`self.SetCollisionDamageObject` IsEnabled (`self.RightHandSphereDamageDetection`) :!label _label)
      (`self.SetCollisionDamageObject` IsEnabled (`self.LeftHandSphereDamageDetection`)))
    (:`0`
      (`self.SetCollisionDamageObject` IsEnabled (`self.RightHandSphereDamageDetection`)))
    (:`1`
      (`self.SetCollisionDamageObject` IsEnabled (`self.LeftHandSphereDamageDetection`)))
    (:`2`
      (goto _label))))

(fn `UserConstructionScript`
  (`parent.UserConstructionScript`))