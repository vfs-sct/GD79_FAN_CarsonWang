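; BP_Blacksmith is a human melee enemy character built on a parent class that supplies death and attack handling.
; Construction makes skeletal mesh children follow the main Mesh as leader pose, forming one animated body.
; Weapon collision overlaps report attack contacts, with melee damage toggling that collision on or off.
; When the parent's death-complete event fires, a timeline lowers the mesh so the finished death pose does not appear to float.
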(event `self.ReceiveBeginPlay`
  ;[1 1 1] lowers mesh during animation to make finished death animation not look like it's floating
  (`parent.ReceiveBeginPlay`)
  (add `/Game/Blueprints/Game/Characters/BP_BaseCharacter.OnDeathComplete` (delegate `LowerMesh`)))

(event `LowerMesh`
  ;[1 1 1] lowers mesh during animation to make finished death animation not look like it's floating
  (bind (_direction _alpha) (`Timeline|LowerMeshTimeline`)
    (:`Update`
      (`SceneComponent.K2_SetRelativeLocation` (`self.Mesh`) (`KismetMathLibrary.VLerp` (0.0 0.0 -90.0) (0.0 0.0 -110.0) _alpha) false false))))

(event `self.WeaponCollision.OnComponentBeginOverlap`
  (params (OverlappedComponent :type "PrimitiveComponent Object Reference") (OtherActor :type "Actor Object Reference") (OtherComp :type "PrimitiveComponent Object Reference") (OtherBodyIndex :type Integer) (bFromSweep :type Boolean) (SweepResult :type "HitResult Structure (by ref)"))
  ;[1 1 1] attack target on collision
  (`self.OnAttackTargetContact` OtherActor))

(fn `SetLeaderPose`
  (for _array_element (`SceneComponent.GetChildrenComponents` (`self.Mesh`) false)
    (bind _asskeletal_mesh_component (cast `SkeletalMeshComponent` _array_element))
    (`SkinnedMeshComponent.SetLeaderPoseComponent` _asskeletal_mesh_component (`self.Mesh`) false false)))

(fn `ToggleMeleeDamageCollision`
  (params (IsEnabled :type Boolean) (CollisionIndex :type Integer))
  (`self.SetCollisionDamageObject` IsEnabled (`self.WeaponCollision`)))

(fn `UserConstructionScript`
  (`parent.UserConstructionScript`)
  (`self.SetLeaderPose`))