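; BP_ImpCharacter is the Imp enemy AI character, adding hand-based melee hit detection to inherited character logic.
; ToggleMeleeDamageCollision enables or disables damage collision on the right hand (index 0) or left hand (index 1).
; Hand overlaps pass the other actor to OnAttackTargetContact, with the left hand firing on overlap begin and the right on overlap end.
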(event `self.LeftHandCollision.OnComponentBeginOverlap`
  (params (OverlappedComponent :type "PrimitiveComponent Object Reference") (OtherActor :type "Actor Object Reference") (OtherComp :type "PrimitiveComponent Object Reference") (OtherBodyIndex :type Integer) (bFromSweep :type Boolean) (SweepResult :type "HitResult Structure (by ref)"))
  (`self.OnAttackTargetContact` OtherActor))

(event `self.RightHandCollision.OnComponentEndOverlap`
  (params (OverlappedComponent :type "PrimitiveComponent Object Reference") (OtherActor :type "Actor Object Reference") (OtherComp :type "PrimitiveComponent Object Reference") (OtherBodyIndex :type Integer))
  (`self.OnAttackTargetContact` OtherActor))

(fn `ToggleMeleeDamageCollision`
  (params (IsEnabled :type Boolean) (CollisionIndex :type Integer))
  (switch `int` CollisionIndex
    (:`0`
      (`self.SetCollisionDamageObject` IsEnabled (`self.RightHandCollision`)))
    (:`1`
      (`self.SetCollisionDamageObject` IsEnabled (`self.LeftHandCollision`)))))

(fn `UserConstructionScript`
  (`parent.UserConstructionScript`))