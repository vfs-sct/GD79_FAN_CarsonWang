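; Anubis enemy AI character that deals melee damage with a spear and a shield.
; Overlaps on either weapon collider are forwarded to OnAttackTargetContact.
; ToggleMeleeDamageCollision switches one collider by index, or both by default for cases like stun, with separate per-weapon toggle functions also defined.
; Per the author's note, the Anim BP enables and disables the colliders during attack montages.
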(event `self.ReceiveBeginPlay`
  (`parent.ReceiveBeginPlay`))

(event `self.Spear.OnComponentBeginOverlap`
  (params (OverlappedComponent :type "PrimitiveComponent Object Reference") (OtherActor :type "Actor Object Reference") (OtherComp :type "PrimitiveComponent Object Reference") (OtherBodyIndex :type Integer) (bFromSweep :type Boolean) (SweepResult :type "HitResult Structure (by ref)"))
  ;[1 1 1] The Anim BP is setting the colliders enabled/disabled during attack Anims. Look at APB_Anubis and it's attack anim montages as example.
  (`self.OnAttackTargetContact` OtherActor))

(event `self.Shield.OnComponentBeginOverlap`
  (params (OverlappedComponent :type "PrimitiveComponent Object Reference") (OtherActor :type "Actor Object Reference") (OtherComp :type "PrimitiveComponent Object Reference") (OtherBodyIndex :type Integer) (bFromSweep :type Boolean) (SweepResult :type "HitResult Structure (by ref)"))
  ;[1 1 1] The Anim BP is setting the colliders enabled/disabled during attack Anims. Look at APB_Anubis and it's attack anim montages as example.
  (`self.OnAttackTargetContact` OtherActor))

(fn `ToggleMeleeDamageCollision`
  (params (IsEnabled :type Boolean) (CollisionIndex :type Integer))
  (switch `int` CollisionIndex
    (:`Default`
      ;[1 1 1] Default will toggle all damage collision. Used to turn off everything on stun, etc.
      (`self.SetCollisionDamageObject` IsEnabled (`self.Spear`))
      (`self.SetCollisionDamageObject` IsEnabled (`self.Shield`)))
    (:`0`
      (`self.SetCollisionDamageObject` IsEnabled (`self.Spear`)))
    (:`1`
      (`self.SetCollisionDamageObject` IsEnabled (`self.Shield`)))))

(fn `ToggleShieldDamageCollision`
  (params (IsOn :type Boolean))
  (bind _shield (`self.Shield`))
  (if IsOn
    (`PrimitiveComponent.SetCollisionEnabled` _shield "QueryAndProbe")
    (`PrimitiveComponent.SetCollisionResponseToChannel` _shield "ECC_Pawn" "ECR_Overlap")
    (else
      (`PrimitiveComponent.SetCollisionEnabled` _shield "NoCollision"))))

(fn `ToggleSpearDamageCollision`
  (params (IsOn :type Boolean))
  (bind _spear (`self.Spear`))
  (if IsOn
    (`PrimitiveComponent.SetCollisionEnabled` _spear "QueryAndProbe")
    (`PrimitiveComponent.SetCollisionResponseToChannel` _spear "ECC_Pawn" "ECR_Overlap")
    (else
      (`PrimitiveComponent.SetCollisionEnabled` _spear "NoCollision"))))

(fn `UserConstructionScript`
  (`parent.UserConstructionScript`))