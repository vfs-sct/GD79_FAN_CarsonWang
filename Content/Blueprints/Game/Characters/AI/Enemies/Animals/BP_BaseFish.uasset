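; Base Blueprint for fish enemies that handles melee contact damage from jaw and tail collision components.
; Overlaps on either component pass the other actor to the attack contact handler.
; ToggleMeleeDamageCollision switches jaw or tail damage by index, with a second jaw index that clears hit targets first when double hits are allowed.
; The construction script calls SetCollisions, which is empty here.
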(event `self._jawsCollision.OnComponentBeginOverlap`
  (params (OverlappedComponent :type "PrimitiveComponent Object Reference") (OtherActor :type "Actor Object Reference") (OtherComp :type "PrimitiveComponent Object Reference") (OtherBodyIndex :type Integer) (bFromSweep :type Boolean) (SweepResult :type "HitResult Structure (by ref)"))
  (`self.OnAttackTargetContact` OtherActor))

(event `self._tailCollision.OnComponentBeginOverlap`
  (params (OverlappedComponent :type "PrimitiveComponent Object Reference") (OtherActor :type "Actor Object Reference") (OtherComp :type "PrimitiveComponent Object Reference") (OtherBodyIndex :type Integer) (bFromSweep :type Boolean) (SweepResult :type "HitResult Structure (by ref)"))
  (`self.OnAttackTargetContact` OtherActor))

(fn `SetCollisions`)

(fn `ToggleMeleeDamageCollision`
  (params (IsEnabled :type Boolean) (CollisionIndex :type Integer))
  ;[1 1 1] sets collisions from int. 0 and 1 = jaws, 2 = tail. Also determines if anglerfish can double hit from boolean
  (switch `int` CollisionIndex
    (:`0`
      (`self.SetCollisionDamageObject` IsEnabled (`self._jawsCollision`) :!label _label))
    (:`1`
      (if (`self._canDoubleHit`)
        (`self.ClearHitTargets`)
        (goto _label)
        (else
          (goto _label))))
    (:`2`
      (`self.SetCollisionDamageObject` IsEnabled (`self._tailCollision`)))))

(fn `UserConstructionScript`
  (`parent.UserConstructionScript`)
  (`self.SetCollisions`))