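; BP_Cow is a cow enemy character with two melee hit zones, horns and legs.
; An index selects which collision has its damage toggled, and overlaps on either are passed to OnAttackTargetContact.
; ReverseCow flips the mesh between two opposite facings through RotateCow, which uses a timeline to blend the mesh's relative rotation.
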(event `RotateCow`
  (params (OldRotation :type "Rotator Structure") (NewRotation :type "Rotator Structure"))
  (bind (_direction _rotate) (`Timeline|Timeline` :`NewTime` 1.0 :!via `PlayFromStart`)
    (:`Update`
      (`SceneComponent.K2_SetRelativeRotation` (`self.Mesh`) (`KismetMathLibrary.RLerp` OldRotation NewRotation _rotate) false false))))

(event `self.HornsCollision.OnComponentBeginOverlap`
  (params (OverlappedComponent :type "PrimitiveComponent Object Reference") (OtherActor :type "Actor Object Reference") (OtherComp :type "PrimitiveComponent Object Reference") (OtherBodyIndex :type Integer) (bFromSweep :type Boolean) (SweepResult :type "HitResult Structure (by ref)"))
  ;[1 1 1] attack on collision
  (`self.OnAttackTargetContact` OtherActor))

(event `self.LegsCollision.OnComponentBeginOverlap`
  (params (OverlappedComponent :type "PrimitiveComponent Object Reference") (OtherActor :type "Actor Object Reference") (OtherComp :type "PrimitiveComponent Object Reference") (OtherBodyIndex :type Integer) (bFromSweep :type Boolean) (SweepResult :type "HitResult Structure (by ref)"))
  ;[1 1 1] attack on collision
  (`self.OnAttackTargetContact` OtherActor))

(fn `ReverseCow`
  (params (isForwardFacing :type Boolean))
  (if isForwardFacing
    (`self.RotateCow` (struct :`Yaw` 270.0) (struct :`Yaw` 90.0))
    (else
      (`self.RotateCow` (struct :`Yaw` 90.0) (struct :`Yaw` 270.0)))))

(fn `ToggleMeleeDamageCollision`
  (params (IsEnabled :type Boolean) (CollisionIndex :type Integer))
  ;[1 1 1] collisions set from int. 0 = horns, 1 = legs
  (switch `int` CollisionIndex
    (:`0`
      (`self.SetCollisionDamageObject` IsEnabled (`self.HornsCollision`)))
    (:`1`
      (`self.SetCollisionDamageObject` IsEnabled (`self.LegsCollision`)))))

(fn `UserConstructionScript`
  (`parent.UserConstructionScript`))