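; BP_SkeletonArcher is a humanoid skeleton enemy that shoots arrows at targets chosen by its AI controller.
; Construction makes the main mesh the leader pose for its child skeletal meshes, and simple functions show or hide the arrow prop.
; Shoot spawns a BP_SkeletonArrow with the archer's damage and speed, then applies the skeleton arrow mesh.
; Aim leads the nearest line-of-sight target, predicting position from its velocity and arrow travel time.
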(fn `CalculatePredictedLocation`
  (params (Actor :type "Actor Object Reference"))
  (returns (`Predicted Location` :type "Vector Structure"))
  (return (+ (`self.K2_GetActorLocation` Actor) (* (`self.GetVelocity` Actor) (/ (`KismetMathLibrary.VSize` (- (`self.K2_GetActorLocation` Actor) (`SceneComponent.K2_GetComponentLocation` (`self.ArrowSpawn`)))) (`self._arrowSpeed`))))))

(fn `GetArrowTransform`
  (returns (Transform :type "Transform Structure"))
  (bind (_returnvalue_location _returnvalue_rotation _returnvalue_scale) (`KismetMathLibrary.BreakTransform` (`SceneComponent.K2_GetComponentToWorld` (`self.ArrowSpawn`))))
  (bind _returnvalue (`AIBlueprintHelperLibrary.GetAIController` self))
  ;[1 1 1] cast to AI controller
  (`/Engine/EditorBlueprintResources/StandardMacros.IsValid` _returnvalue
    (:`Is Valid`
      (bind _asbp_base_aicontroller (cast `/Game/Blueprints/Game/AI/Controllers/BP_BaseAIController` _returnvalue))
      ;[1 1 1] keep arrow spawn location/scale, rotate to look at target's predicted location
      (return (`KismetMathLibrary.MakeTransform` _returnvalue_location (`KismetMathLibrary.FindLookAtRotation` _returnvalue_location (`self.CalculatePredictedLocation` (`/Game/Blueprints/Game/AI/Controllers/BP_BaseAIController.GetNearestTargetInLineOfSight` _asbp_base_aicontroller))) _returnvalue_scale)))))

(fn `HideArrow`
  ;[1 1 1] hides arrow mesh component
  (`SceneComponent.SetVisibility` (`self.ArrowSet`) false false))

(fn `SetLeaderPose`
  ;[1 1 1] grab each component in the body
  (for _array_element (`SceneComponent.GetChildrenComponents` (`self.Mesh`) false)
    ;[1 1 1] put body mesh as leader pose component
    (bind _asskeletal_mesh_component (cast `SkeletalMeshComponent` _array_element))
    (`SkinnedMeshComponent.SetLeaderPoseComponent` _asskeletal_mesh_component (`self.Mesh`) false false)))

(fn `Shoot`
  ;[1 1 1] shoot arrow and make it look like skeleton arrow
  (bind _returnvalue (`|SpawnActorFromClass` "/Game/Blueprints/Game/Projectiles/Arrows/BP_SkeletonArrow.BP_SkeletonArrow_C" (`self.GetArrowTransform`) "Undefined" "MultiplyWithRoot" null (`KismetMathLibrary.Conv_IntToDouble` (`self.GetAttackDamage`)) self (`self._arrowSpeed`) null))
  (`SkeletalMeshComponent.SetSkeletalMeshAsset` (`/Game/Blueprints/Game/Projectiles/Arrows/BP_BaseArrow.SkeletalMesh` _returnvalue) "/Game/Assets/Characters/StylizedEnemyNPC/Meshes/SkeletonArcher/Weapons/SK_Arrow.SK_Arrow"))

(fn `ShowArrow`
  ;[1 1 1] shows arrow mesh component
  (`SceneComponent.SetVisibility` (`self.ArrowSet`) true false))

(fn `UserConstructionScript`
  (`parent.UserConstructionScript`)
  (`self.SetLeaderPose`))