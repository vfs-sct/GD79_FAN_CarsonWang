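; Skeleton wizard humanoid enemy that fires spell projectiles at targets.
; Construction script makes its child skeletal meshes follow the body mesh via Leader Pose.
; Small spell spawns BP_BaseSpell from SpellOrigin, aimed at the AI controller's nearest line-of-sight target with linear lead prediction from target velocity and spell speed.
; Big spell is only a placeholder debug print.
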(fn `CalculatePredictedLocation`
  (params (Actor :type "Actor Object Reference"))
  (returns (`Predicted Location` :type "Vector Structure"))
  (return (+ (`self.K2_GetActorLocation` Actor) (* (`self.GetVelocity` Actor) (/ (`KismetMathLibrary.VSize` (- (`self.K2_GetActorLocation` Actor) (`SceneComponent.K2_GetComponentLocation` (`self.SpellOrigin`)))) (`self._spellSpeed`))))))

(fn `FireBigSpell`
  (`KismetSystemLibrary.PrintString` "big thing"))

(fn `FireSmallSpell`
  (`|SpawnActorFromClass` "/Game/Blueprints/Game/Projectiles/Spells/BP_BaseSpell.BP_BaseSpell_C" (`self.GetSpellTransform`) "Undefined" "MultiplyWithRoot" null (`KismetMathLibrary.Conv_IntToDouble` (`self.GetAttackDamage`)) (`self._spellSpeed`) null))

(fn `GetSpellTransform`
  (returns (Transform :type "Transform Structure"))
  (bind _returnvalue (`AIBlueprintHelperLibrary.GetAIController` self))
  (bind (_returnvalue_location _returnvalue_rotation _returnvalue_scale) (`KismetMathLibrary.BreakTransform` (`SceneComponent.K2_GetComponentToWorld` (`self.SpellOrigin`))))
  (`/Engine/EditorBlueprintResources/StandardMacros.IsValid` _returnvalue
    (:`Is Valid`
      (bind _asbp_base_aicontroller (cast `/Game/Blueprints/Game/AI/Controllers/BP_BaseAIController` _returnvalue))
      (return (`KismetMathLibrary.MakeTransform` _returnvalue_location (`KismetMathLibrary.FindLookAtRotation` _returnvalue_location (`self.CalculatePredictedLocation` (`/Game/Blueprints/Game/AI/Controllers/BP_BaseAIController.GetNearestTargetInLineOfSight` _asbp_base_aicontroller))) _returnvalue_scale)))))

(fn `SetLeaderPose`
  ;[1 1 1] grab each skeletal mesh component
  (for _array_element (`SceneComponent.GetChildrenComponents` (`self.Mesh`) false)
    ;[1 1 1] set body as leader bone
    (bind _asskeletal_mesh_component (cast `SkeletalMeshComponent` _array_element))
    (`SkinnedMeshComponent.SetLeaderPoseComponent` _asskeletal_mesh_component (`self.Mesh`) false false)))

(fn `UserConstructionScript`
  (`parent.UserConstructionScript`)
  (`self.SetLeaderPose`))