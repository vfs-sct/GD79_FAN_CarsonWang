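; BP_SkeletonWarrior_2H is the two-handed Skeleton Warrior enemy, customizing how its melee attacks register hits.
; It overrides ToggleMeleeDamageCollision so both collision indices switch damage on the same left weapon capsule.
; With CanDoubleHit enabled, index 1 clears hit targets before each toggle, letting the second attack hit on both upward and downward swings.
; Its event graph holds only disabled stubs, and construction defers to the parent.
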(fn `ToggleMeleeDamageCollision`
  (params (IsEnabled :type Boolean) (CollisionIndex :type Integer))
  ;[1 1 1] If canDoubleHit is enabled, the second attack will be able to hit the player on both the upward and downward swings. Otherwise, both attacks only hit once
  (switch `int` CollisionIndex
    (:`0`
      _)
    (:`1`
      (if (`self._canDoubleHit`)
        (`self.ClearHitTargets`))))
  (`self.SetCollisionDamageObject` IsEnabled (`self.WepL_DamageCollisionCapsule`)))

(fn `UserConstructionScript`
  (`parent.UserConstructionScript`))