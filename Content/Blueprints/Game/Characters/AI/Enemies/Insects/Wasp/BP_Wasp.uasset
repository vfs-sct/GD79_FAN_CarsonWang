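; BP_Wasp is an insect enemy character that damages the player with stinger and hand melee attacks.
; Overlaps on the stinger, left hand and right hand collision components are all forwarded to OnAttackTargetContact.
; ToggleMeleeDamageCollision switches damage collision by attack index through SetCollisionDamageObject, with one index for the stinger and another for both hands together.
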(event `self.LeftHandCollision.OnComponentBeginOverlap`
  (params (OverlappedComponent :type "PrimitiveComponent Object Reference") (OtherActor :type "Actor Object Reference") (OtherComp :type "PrimitiveComponent Object Reference") (OtherBodyIndex :type Integer) (bFromSweep :type Boolean) (SweepResult :type "HitResult Structure (by ref)"))
  ;[1 1 1] damage player when attacking
  (`self.OnAttackTargetContact` OtherActor))

(event `self.StingerCollision.OnComponentBeginOverlap`
  (params (OverlappedComponent :type "PrimitiveComponent Object Reference") (OtherActor :type "Actor Object Reference") (OtherComp :type "PrimitiveComponent Object Reference") (OtherBodyIndex :type Integer) (bFromSweep :type Boolean) (SweepResult :type "HitResult Structure (by ref)"))
  ;[1 1 1] damage player when attacking
  (`self.OnAttackTargetContact` OtherActor))

(event `self.RightHandCollision.OnComponentBeginOverlap`
  (params (OverlappedComponent :type "PrimitiveComponent Object Reference") (OtherActor :type "Actor Object Reference") (OtherComp :type "PrimitiveComponent Object Reference") (OtherBodyIndex :type Integer) (bFromSweep :type Boolean) (SweepResult :type "HitResult Structure (by ref)"))
  ;[1 1 1] damage player when attacking
  (`self.OnAttackTargetContact` OtherActor))

(fn `ToggleMeleeDamageCollision`
  (params (IsEnabled :type Boolean) (CollisionIndex :type Integer))
  (switch `int` CollisionIndex
    (:`0`
      ;[1 1 1] set stinger active on index 0
      (`self.SetCollisionDamageObject` IsEnabled (`self.StingerCollision`)))
    (:`1`
      ;[1 1 1] set hands active on index 1
      (`self.SetCollisionDamageObject` IsEnabled (`self.LeftHandCollision`))
      (`self.SetCollisionDamageObject` IsEnabled (`self.RightHandCollision`)))))

(fn `UserConstructionScript`
  (`parent.UserConstructionScript`))