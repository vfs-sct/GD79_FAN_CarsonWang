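; BP_FireflyGrounded is a grounded firefly insect enemy with a bite attack and a configurable point light.
; The construction script calls SetLights, which sets the light's visibility and color from IsLightOn and LightColor.
; ToggleMeleeDamageCollision switches the BiteCollision damage object on or off, and overlaps on that collision are passed to OnAttackTargetContact.
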(event `self.BiteCollision.OnComponentBeginOverlap`
  (params (OverlappedComponent :type "PrimitiveComponent Object Reference") (OtherActor :type "Actor Object Reference") (OtherComp :type "PrimitiveComponent Object Reference") (OtherBodyIndex :type Integer) (bFromSweep :type Boolean) (SweepResult :type "HitResult Structure (by ref)"))
  (`self.OnAttackTargetContact` OtherActor))

(fn `SetLights`
  (bind _pointlight (`self.PointLight`))
  (`SceneComponent.SetVisibility` _pointlight (`self._isLightOn`) false)
  (`LightComponent.SetLightColor` _pointlight (`self._lightColor`) true))

(fn `ToggleMeleeDamageCollision`
  (params (IsEnabled :type Boolean) (CollisionIndex :type Integer))
  (`self.SetCollisionDamageObject` IsEnabled (`self.BiteCollision`)))

(fn `UserConstructionScript`
  (`parent.UserConstructionScript`)
  (`self.SetLights`))