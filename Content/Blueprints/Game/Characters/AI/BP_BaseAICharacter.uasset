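; Base character class for AI enemies, supplying attack, patrol, investigate and movement-speed data to its AI controller and behavior tree.
; Attacks play random or cycled montages with a cooldown, tracking hit targets so each is damaged once per swing.
; Attempted hits are reported as AI damage sense events, and stun or stagger switches off melee collisions.
; Subclasses override melee collision toggling and per-attack hit callbacks.
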(event `self.ReceivePossessed`
  (params (NewController :type "Controller Object Reference"))
  ;[1 1 1] Listen for AI state changed
  (bind _asbp_base_aicontroller (cast `/Game/Blueprints/Game/AI/Controllers/BP_BaseAIController` NewController))
  (add `/Game/Blueprints/Game/AI/Controllers/BP_BaseAIController.OnAIStateChangedEvent` _asbp_base_aicontroller (delegate `OnAIStateChangedEvent_Event`)))

(event `OnAIStateChangedEvent_Event`
  (params (State :type "/Game/Blueprints/Game/AI/States/EN_AIStates Enum" :default "NewEnumerator0"))
  ;[1 1 1] Listen for AI state changed
  (`self.OnAIStateChanged` State))

(event `self.ReceiveBeginPlay`
  (`parent.ReceiveBeginPlay`)
  ;[1 1 1] AI senses to detect someone hidden/out of view has attempted to attack this target. AI will chase/investigate where the attack came from
  (add `self.OnAttemptedToBeHitEvent` (delegate `OnAttemptedToBeHitEvent_Event`))
  ;[1 1 1] If stunned or staggered, disable all melee damage collisions by feeding in value -1 so 'ToggleMeleeDamageCollision' method can run through it's default state. See BP_Anubis 'ToggleMeleeDamageCollision' method for example.
  (add `self.OnToggleStunComplete` (delegate `OnToggleStunComplete_Event`))
  (add `self.OnToggleStaggeredComplete` (delegate `OnToggleStaggeredComplete_Event`)))

(event `OnToggleStaggeredComplete_Event` :!signature `self.OnToggleStaggeredComplete`
  (params (Character :type "/Game/Blueprints/Game/Characters/BP_BaseCharacter Object Reference") (IsStaggered :type Boolean))
  ;[1 1 1] If stunned or staggered, disable all melee damage collisions by feeding in value -1 so 'ToggleMeleeDamageCollision' method can run through it's default state. See BP_Anubis 'ToggleMeleeDamageCollision' method for example.
  (if IsStaggered
    (`self.ToggleMeleeDamageCollision` false -1 :!label _label)))

(event `OnAttemptedToBeHitEvent_Event` :!signature `self.OnAttemptedToBeHitEvent`
  (params (Instigator :type "Actor Object Reference"))
  ;[1 1 1] AI senses to detect someone hidden/out of view has attempted to attack this target. AI will chase/investigate where the attack came from
  (`self.OnTryReportDamageEventForAIStateChange` Instigator))

(event `OnToggleStunComplete_Event` :!signature `self.OnToggleStunComplete`
  (params (IsStunned :type Boolean))
  ;[1 1 1] If stunned or staggered, disable all melee damage collisions by feeding in value -1 so 'ToggleMeleeDamageCollision' method can run through it's default state. See BP_Anubis 'ToggleMeleeDamageCollision' method for example.
  (if IsStunned
    (goto _label)))

(event `self.ReceiveTick`
  (params (DeltaSeconds :type "Float (single-precision)"))
  (`self.IncrementAttackCooldownTimerCheck` DeltaSeconds))

(event `/Game/Blueprints/Game/AI/Pathing/BPI_PatrolCharacter.OnPatrolPointReached`
  ;[1 1 1] Patrol Path for AIs
  (`/Game/Blueprints/Game/AI/Pathing/BPC_PatrolController.On Patrol Point Reached` (`self.PatrolController`)))

(event `PlayLookAroundAnimMontage`
  (bind __lookaroundanimmontage (`self._lookAroundAnimMontage`))
  ;[1 1 1] Look Around. Called from the behaviour tree while investiagting areas. If no animation montage, nothing will play, and do a delay instead
  (if (and (`self.GetIsAlive`) (not (`self.GetIsStunned`)))
    (`/Engine/EditorBlueprintResources/StandardMacros.IsValid` __lookaroundanimmontage
      (:`Is Valid`
        (`|PlayMontage` (`self.Mesh`) __lookaroundanimmontage
          (:`OnCompleted`
            _)
          (:`OnInterrupted`
            _)))
      (:`Is Not Valid`
        (`KismetSystemLibrary.Delay` 1.5)))
    (`self.OnLookAroundCompleteEvent`)))

(event `/Game/Blueprints/Game/AI/Pathing/BPI_PatrolCharacter.SetPatrolPath`
  (params (patrolPath :type "/Game/Blueprints/Game/AI/Pathing/BP_PatrolPath Object Reference"))
  ;[1 1 1] Patrol Path for AIs
  (bind _output_get (set `self._startingPatrolPath` patrolPath)) ; Used for default starting point on AI Spawn
  (`/Game/Blueprints/Game/AI/Pathing/BPC_PatrolController.SetPatrolPath` (`self.PatrolController`) _output_get))

(event `Attack`
  (params (AttackTarget :type "Actor Object Reference"))
  ;[1 1 1] Attack
  (set `self._targetCurrentlyAttacking` AttackTarget)
  (set `self._isAttacking` true)
  (`self.ClearHitTargets`) ; Resets a list of targets hit from previous attack\nto prevent the same target to be hit multiple\ntimes during the same attack
  (`|PlayMontage` (`self.Mesh`) (`self.GetAttackMontage`)
    (:`OnCompleted`
      _)
    (:`OnInterrupted`
      _))
  (set `self._targetCurrentlyAttacking` null) ; Reset Attack Target To null\nonce attack is done
  (`self.OnSetAttackIndex`)
  (set `self._attackCooldownTimer` 0.0)
  (set `self._isAttacking` false)
  (`self.OnAttackCompleteEvent`))

(fn `AddTargetHitThisAttackToList`
  (params (Actor :type "Actor Object Reference (by ref)"))
  (`KismetArrayLibrary.Array_Add` (`self._targetsHitThisAttack`) Actor))

(fn `CanHitTargetThisAttack`
  (params (Actor :type "Actor Object Reference (by ref)"))
  (returns (TargetCanTryBeHitThisAttack :type Boolean))
  (if (or (`self.GetIsAlive`) (not (`self.GetIsStunned`)))
    (bind _asbpi_targetable (cast `/Game/Blueprints/Core/Targetable/BPI_Targetable` Actor)
      (:`then`
        (bind _istargetable (`/Game/Blueprints/Core/Targetable/BPI_Targetable.IsTargetable` _asbpi_targetable))
        (if _istargetable
          ;[1 1 1] Don't attack teammates/self
          (bind _team (`/Game/Blueprints/Core/Targetable/BPI_Targetable.GetTeam` _asbpi_targetable))
          (if (!= _team (`self.TeamID`))
            (return (not (`KismetArrayLibrary.Array_Contains` (`self.GetTargetsHitThisAttack`) Actor)))
            (else
              _))))
      (:`CastFailed`
        (return (not (`KismetArrayLibrary.Array_Contains` (`self.GetTargetsHitThisAttack`) Actor))))))
  (return false))

(fn `ClearHitTargets`
  (`KismetArrayLibrary.Array_Clear` (`self._targetsHitThisAttack`)))

(fn `GetAIBehaviourTree`
  (returns (behaviourTree :type "BehaviorTree Object Reference"))
  (return (`self._aiBehaviourTree`)))

(fn `GetAttackCooldown`
  (returns (_attackCooldown :type "Float (double-precision)"))
  (return (`self._attackCooldown`)))

(fn `GetAttackDamage`
  (returns (_attackDamage :type Integer))
  (return (`self._attackDamage`)))

(fn `GetAttackIndex`
  (returns (_attackCount :type Integer))
  (return (`self._attackIndex`)))

(fn `GetAttackMontage`
  (returns (attackMontage :type "AnimMontage Object Reference"))
  (return (`|GetArrayItem` (`self._attackMontage`) (`self.GetAttackIndex`))))

(fn `GetAttackRadius`
  (returns (radius :type "Float (double-precision)"))
  (return (`self._attackRadius`)))

(fn `GetCurrentPatrolPath`
  (returns (Patrol :type "/Game/Blueprints/Game/AI/Pathing/BP_PatrolPath Object Reference"))
  (return (`/Game/Blueprints/Game/AI/Pathing/BPC_PatrolController.GetActivePatrolPath` (`self.PatrolController`))))

(fn `GetInvestigateMovementSpeed`
  (returns (_startingMovementSpeed :type "Float (double-precision)"))
  (return (* (`self._startingMovementSpeed`) (`self._investigateMovementSpeedMultiplier`))))

(fn `GetMaxMovementSpeed`
  (returns (_startingMovementSpeed :type "Float (double-precision)"))
  (return (`self._startingMovementSpeed`)))

(fn `GetMoveToPatrolPathPointLocation`
  (returns (isValid :type Boolean) (location :type "Vector Structure"))
  (bind (_position _isvalid) (`/Game/Blueprints/Game/AI/Pathing/BPC_PatrolController.GetMoveToPatrolPathPointLocation` (`self.PatrolController`)))
  (return _isvalid _position))

(fn `GetPatrolMovementSpeed`
  (returns (ReturnValue :type "Float (double-precision)"))
  (return (* (`self._startingMovementSpeed`) (`self._patrolMovementSpeedMultiplier`))))

(fn `GetStartingAIState`
  (returns (_startingAIState :type "/Game/Blueprints/Game/AI/States/EN_AIStates Enum"))
  (return (`self._startingAIState`)))

(fn `GetStrafeMovementSpeed`
  (returns (ReturnValue :type "Float (double-precision)"))
  (return (* (`self._startingMovementSpeed`) (`self._strafeMovementSpeedMultiplier`))))

(fn `GetStrafeRadius`
  (returns (radius :type "Float (double-precision)"))
  (return (`self._strafeRadius`)))

(fn `GetTargetsHitThisAttack`
  (returns (_targetsHitThisAttack :type "Array of Actor Object Reference"))
  (return (`self._targetsHitThisAttack`)))

(fn `IncrementAttackCooldownTimerCheck`
  (params (Value :type "Float (single-precision)"))
  (if (and (`self.GetIsAlive`) (not (`self.GetIsStunned`)) (not (`self.GetIsStaggered`)) (not (`self._isAttacking`)))
    (set `self._attackCooldownTimer` (+ (`self._attackCooldownTimer`) Value))))

(fn `IsAttackOffCooldown`
  (returns (IsAttackOffCooldown :type Boolean))
  (return (>= (`self._attackCooldownTimer`) (`self._attackCooldown`))))

(fn `OnAIStateChanged`
  (params (State :type "/Game/Blueprints/Game/AI/States/EN_AIStates Enum" :default "NewEnumerator0"))
  (`self.StopLookAroundAnimMontage`))

(fn `OnAttack`
  (`KismetSystemLibrary.PrintString` (`KismetStringLibrary.Concat_StrStr` (`KismetSystemLibrary.GetDisplayName` self) " " ": OnAttack() needs to be override and defined in it's BP for what OnAttack() Does")))

(fn `OnAttackCallback`
  (params (attackTarget :type "/Game/Blueprints/Game/Characters/BP_BaseCharacter Object Reference") (attackResult :type "/Game/Blueprints/Game/AttackResult/EAttackResult Enum" :default "NewEnumerator0") (attackIndex :type Integer))
  ;[1 1 1] You can override this for each character to do unique callbacks to specific attacks
  ;
  ; Look at "BP_SandGolemCharacter" 'OnAttackCallback' override as an example
)

(fn `OnAttackTargetContact`
  (params (Actor :type "Actor Object Reference (by ref)"))
  (bind _returnvalue (`KismetMathLibrary.Conv_IntToDouble` (`self.GetAttackDamage`)))
  (bind _targetcantrybehitthisattack (`self.CanHitTargetThisAttack` Actor))
  (if _targetcantrybehitthisattack
    (`self.AddTargetHitThisAttackToList` Actor)
    (bind _asbp_base_character (cast `/Game/Blueprints/Game/Characters/BP_BaseCharacter` Actor)
      (:`then`
        (bind _attackresult (`self.TryOnHit` _asbp_base_character self _returnvalue))
        (`self.OnAttackCallback` _asbp_base_character _attackresult (`self._attackIndex`)))
      (:`CastFailed`
        (`GameplayStatics.ApplyDamage` Actor _returnvalue null self)))))

(fn `OnSetAttackIndex`
  (locals (_nextAttackIndex :type Integer :default 0))
  (bind __attackmontage (`self._attackMontage`))
  (bind _returnvalue (+ (`self.GetAttackIndex`) 1))
  (if (`self._IsRandomAttackAnimMontage`)
    (set `local._nextAttackIndex` (`.OutIndex` (`KismetArrayLibrary.Array_Random` __attackmontage)))
    (elif (>= _returnvalue (`KismetArrayLibrary.Array_Length` __attackmontage))
      (set `local._nextAttackIndex` 0)
      (else
        (set `local._nextAttackIndex` _returnvalue))))
  (`self.SetAttackIndex` (`local._nextAttackIndex`)))

(fn `OnTryReportDamageEventForAIStateChange`
  (params (Object :type "Object Object Reference"))
  ;[1 1 1] This does not deal damage, but the AI listens for this event to break out of idle/investage/patrol to chase the damage causer (Instigator)
  (bind _asbp_base_character (cast `/Game/Blueprints/Game/Characters/BP_BaseCharacter` Object))
  (bind _returnvalue (`self.K2_GetActorLocation` _asbp_base_character))
  (`AISense_Damage.ReportDamageEvent` self _asbp_base_character 0.0 _returnvalue _returnvalue) ; The damage amount does not\nmater in this case.
  (`self.StopLookAroundAnimMontage`))

(fn `SetAttackIndex`
  (params (_attackCount :type Integer))
  (returns (Output_Get :type Integer))
  (bind _output_get (set `self._attackIndex` _attackCount))
  (return _output_get))

(fn `SetCollisionDamageObject`
  (params (Condition :type Boolean) (CollisionObject :type "PrimitiveComponent Object Reference"))
  (if Condition
    (`PrimitiveComponent.SetCollisionEnabled` CollisionObject "QueryAndProbe")
    (`PrimitiveComponent.SetCollisionResponseToChannel` CollisionObject "ECC_Pawn" "ECR_Overlap")
    (else
      (`PrimitiveComponent.SetCollisionEnabled` CollisionObject "NoCollision"))))

(fn `SetStartingVariables`
  ;[1 1 1] Cache movement speed to later apply to different movement types and their respective speeds.
  (set `self._startingMovementSpeed` (`CharacterMovementComponent.MaxWalkSpeed` (`self.CharacterMovement`))))

(fn `StopLookAroundAnimMontage`
  (bind __lookaroundanimmontage (`self._lookAroundAnimMontage`))
  (`/Engine/EditorBlueprintResources/StandardMacros.IsValid` __lookaroundanimmontage
    (:`Is Valid`
      (`self.StopAnimMontage` __lookaroundanimmontage))))

(fn `ToggleMeleeDamageCollision`
  (params (IsEnabled :type Boolean) (CollisionIndex :type Integer))
  ;[1 1 1] blueprint class must override what happens in 'ToggleMeleeDamageCollision' without taking the base class. Make sure to toggle on/off the correct collision to enable damage. Refer to 'BP_Anubis' and check out the override there.
)

(fn `UserConstructionScript`
  (bind __startingpatrolpath (`self._startingPatrolPath`))
  (`parent.UserConstructionScript`)
  (`/Engine/EditorBlueprintResources/StandardMacros.IsValid` __startingpatrolpath
    (:`Is Valid`
      (set `self._startingAIState` "NewEnumerator2")
      (`self.SetPatrolPath` __startingpatrolpath))
    (:`Is Not Valid`
      (set `self._startingAIState` "NewEnumerator0")))
  (`self.SetStartingVariables`))