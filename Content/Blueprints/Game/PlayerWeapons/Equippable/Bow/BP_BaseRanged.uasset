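; Base bow weapon for the player that fires arrow projectiles and animates the bowstring.
; Attacks sphere-trace along the camera when aiming, otherwise from the arrow socket toward the lock-on target or character forward.
; The arrow spawns at the socket facing the first qualifying hit, or the trace end if nothing is hit.
; Draw, sheathe, shot, aim and lock-on events drive idle, pull, aim and shoot animations, chained with delays.
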(event `OnWeaponDrawnEvent_Event` :!signature `self.OnWeaponDrawnEvent`
  (params (Player :type "/Game/Blueprints/Game/Characters/Player/BP_BasePlayerCharacter Object Reference"))
  ;[1 1 1] Listen for when we want to play the correct animations for the bow string
  (`self.PlayBowIdleAnimation`)
  (add `/Game/Blueprints/Game/Characters/Player/BP_BasePlayerCharacter.OnToggleIsAimingEvent` Player (delegate `OnToggleIsAimingEvent_Event`))
  (add `/Game/Blueprints/Game/TargetSystem/BPC_TargetSystem.OnLockonToggleEvent` (`/Game/Blueprints/Game/AI/Controllers/Player/BP_BasePlayerController.TargetingSystem` (`/Game/Blueprints/Game/Characters/Player/BP_BasePlayerCharacter.GetPlayerController` Player)) (delegate `OnLockonToggleEvent_Event`)))

(event `OnLockonToggleEvent_Event`
  (params (target :type "Actor Object Reference"))
  ;[1 1 1] Listen for when we want to play the correct animations for the bow string
  (if (or (`/Game/Blueprints/Game/Characters/Player/BP_BasePlayerCharacter.GetIsAiming` (stale `OnWeaponDrawnEvent_Event` Player)) (`/Game/Blueprints/Game/Characters/Player/BP_BasePlayerCharacter.GetIsLockedOnTarget` (stale `OnWeaponDrawnEvent_Event` Player)))
    (`self.PlayBowPulledAnimation` :!label _label)
    (else
      (`self.PlayBowIdleAnimation` :!label _label_2))))

(event `OnToggleIsAimingEvent_Event`
  (params (isAiming :type Boolean))
  ;[1 1 1] Listen for when we want to play the correct animations for the bow string
  (if (or isAiming (`/Game/Blueprints/Game/Characters/Player/BP_BasePlayerCharacter.GetIsLockedOnTarget` (stale `OnWeaponDrawnEvent_Event` Player)))
    (goto _label)
    (else
      (goto _label_2))))

(event `self.ReceiveBeginPlay`
  (`parent.ReceiveBeginPlay`)
  (add `self.OnProjectileShotEvent` (delegate `OnProjectileShotEvent_Event`))
  (add `self.OnWeaponDrawnEvent` (delegate `OnWeaponDrawnEvent_Event`))
  (add `self.OnWeaponSheathedEvent` (delegate `OnWeaponSheathedEvent_Event`))
  (`self.AttachArrowMesh`))

(event `OnProjectileShotEvent_Event` :!signature `self.OnProjectileShotEvent`
  (params (Projectile :type "/Game/Blueprints/Game/Projectiles/Arrows/BP_BaseArrow Object Reference"))
  (`self.PlayBowShootAnimation`))

(event `OnWeaponSheathedEvent_Event` :!signature `self.OnWeaponSheathedEvent`
  (params (Player :type "/Game/Blueprints/Game/Characters/Player/BP_BasePlayerCharacter Object Reference"))
  (`self.PlayBowIdleAnimation`))

(event `PlayBowShootAnimation`
  (bind __shootanim (`self._shootAnim`))
  (bind __equippedtoplayer (`self._equippedToPlayer`))
  ;[1 1 1] Bow string animations
  (`SkeletalMeshComponent.PlayAnimation` (`self.Weapon`) __shootanim false)
  (`KismetSystemLibrary.Delay` (/ (`AnimationAsset.GetPlayLength` __shootanim) 3.0))
  (if (or (`/Game/Blueprints/Game/Characters/Player/BP_BasePlayerCharacter.GetIsAiming` __equippedtoplayer) (`/Game/Blueprints/Game/Characters/Player/BP_BasePlayerCharacter.GetIsLockedOnTarget` __equippedtoplayer))
    (`self.PlayBowPulledAnimation`)
    (else
      (`self.PlayBowIdleAnimation`))))

(event `PlayBowPulledAnimation`
  (bind __equippedtoplayer (`self._equippedToPlayer`))
  (bind __pullanim (`self._pullAnim`))
  ;[1 1 1] Bow string animations
  (`SkeletalMeshComponent.PlayAnimation` (`self.Weapon`) __pullanim false)
  (`KismetSystemLibrary.Delay` (/ (`AnimationAsset.GetPlayLength` __pullanim) 3.0))
  (if (or (`/Game/Blueprints/Game/Characters/Player/BP_BasePlayerCharacter.GetIsAiming` __equippedtoplayer) (`/Game/Blueprints/Game/Characters/Player/BP_BasePlayerCharacter.GetIsLockedOnTarget` __equippedtoplayer))
    (`self.PlayBowAimAnimation`)
    (else
      (`self.PlayBowIdleAnimation`))))

(event `PlayBowAimAnimation`
  ;[1 1 1] Bow string animations
  (`SkeletalMeshComponent.PlayAnimation` (`self.Weapon`) (`self._aimAnim`) false))

(event `PlayBowIdleAnimation`
  ;[1 1 1] Bow string animations
  (`SkeletalMeshComponent.PlayAnimation` (`self.Weapon`) (`self._idleAnim`) false))

(fn `AttachArrowMesh`
  (bind _returnvalue (`AddComponent|NODE_AddSkeletalMeshComponent-0`))
  (`SceneComponent.K2_AttachToComponent` _returnvalue (`self.Weapon`) "String" "SnapToTarget" "SnapToTarget" "KeepRelative" true))

(fn `GetEndTrace`
  (returns (_endTrace :type "Vector Structure"))
  (bind __equippedtoplayer (`self._equippedToPlayer`))
  (bind __equippedtoplayer_2 (`self._equippedToPlayer`))
  (bind _camera (`/Game/Blueprints/Game/Characters/Player/BP_BasePlayerCharacter.Camera` __equippedtoplayer))
  (bind _actor_to_target (`/Game/Blueprints/Game/TargetSystem/BPC_TargetSystem.Actor To Target` (`/Game/Blueprints/Game/AI/Controllers/Player/BP_BasePlayerController.TargetingSystem` (`/Game/Blueprints/Game/Characters/Player/BP_BasePlayerCharacter.GetPlayerController` __equippedtoplayer_2))))
  (if (`/Game/Blueprints/Game/Characters/Player/BP_BasePlayerCharacter.GetIsAiming` __equippedtoplayer)
    ;[1 1 1] Aiming
    (set `self._endTrace` (+ (`SceneComponent.K2_GetComponentLocation` _camera) (* (`SceneComponent.GetForwardVector` _camera) (`self.GetAttackRange`))))
    (elif (`/Game/Blueprints/Game/Characters/Player/BP_BasePlayerCharacter.GetIsLockedOnTarget` __equippedtoplayer)
      ;[1 1 1] Locked on target.
      (`/Engine/EditorBlueprintResources/StandardMacros.IsValid` _actor_to_target
        (:`Is Valid`
          (set `self._endTrace` (+ (+ (* (`KismetMathLibrary.GetForwardVector` (`KismetMathLibrary.FindLookAtRotation` (`self.K2_GetActorLocation` __equippedtoplayer_2) (`self.K2_GetActorLocation` _actor_to_target))) (`self.GetAttackRange`)) (`self.K2_GetActorLocation` (`self._equippedToPlayer`))) (`KismetMathLibrary.MakeVector` 0.0 0.0 (`self.ZShootOffset`)))))
        (:`Is Not Valid`
          ;[1 1 1] Free aiming (No aim, no target lock)
          (set `self._endTrace` (+ (+ (`self.K2_GetActorLocation` __equippedtoplayer) (* (`SceneComponent.GetForwardVector` (`Character.CapsuleComponent` __equippedtoplayer)) (`self.GetAttackRange`))) (`KismetMathLibrary.MakeVector` 0.0 0.0 (`self.ZShootOffset`))) :!label _label)))
      (else
        (goto _label))))
  (return (`self._endTrace`)))

(fn `GetStartTrace`
  (returns (startTrace :type "Vector Structure"))
  (locals (_startTrace :type "Vector Structure" :default (0.0 0.0 0.0)))
  (bind __equippedtoplayer (`self._equippedToPlayer`))
  (bind __equippedtoplayer_2 (`self._equippedToPlayer`))
  (bind _camera (`/Game/Blueprints/Game/Characters/Player/BP_BasePlayerCharacter.Camera` __equippedtoplayer))
  (if (`/Game/Blueprints/Game/Characters/Player/BP_BasePlayerCharacter.GetIsAiming` __equippedtoplayer_2)
    (set `local._startTrace` (+ (`SceneComponent.K2_GetComponentLocation` _camera) (* (`SceneComponent.GetForwardVector` _camera) (`SpringArmComponent.TargetArmLength` (`/Game/Blueprints/Game/Characters/Player/BP_BasePlayerCharacter.SpringArm` __equippedtoplayer)))))
    (else
      (set `local._startTrace` (`SceneComponent.GetSocketLocation` (`Character.Mesh` __equippedtoplayer_2) (`self.ArrowSpawnPointAttachmentName`)))))
  (return (`local._startTrace`)))

(fn `OnPickup`
  (params (PlayerCharacter :type "/Game/Blueprints/Game/Characters/Player/BP_BasePlayerCharacter Object Reference"))
  (`parent.OnPickup` PlayerCharacter)
  ;[1 1 1] Add the player to ignore list when raycasting what to hit on shoot
  (`KismetArrayLibrary.Array_AddUnique` (`self.IgnoredActors`) (`self._equippedToPlayer`)))

(fn `OnStartAttack`
  (returns (isWeaponNull :type Boolean))
  (locals (_shootHitLocationTrace :type "Vector Structure" :default (0.0 0.0 0.0)) (_objectLineTrace :type "Array of EObjectTypeQuery Enum"))
  (bind __endtrace (`self.GetEndTrace`))
  (bind __equippedtoplayer (`self._equippedToPlayer`))
  (`/Engine/EditorBlueprintResources/StandardMacros.IsValid` __equippedtoplayer
    (:`Is Valid`
      (bind (_outhits _returnvalue) (`KismetSystemLibrary.SphereTraceMulti` (`self.GetStartTrace`) __endtrace 2.5 "TraceTypeQuery1" false (`self.IgnoredActors`)))
      (if _returnvalue
        (for _array_element _outhits
          (bind (_bblockinghit _binitialoverlap _time _distance _location _impactpoint _normal _impactnormal _physmat _hitactor _hitcomponent) (`GameplayStatics.BreakHitResult` _array_element))
          (bind _returnvalue_2 (`PrimitiveComponent.GetCollisionResponseToChannel` _hitcomponent "ECC_GameTraceChannel1"))
          (if (or (`|EnumEquality` _returnvalue_2 "ECR_Overlap") (`|EnumEquality` _returnvalue_2 "ECR_Block"))
            (set `local._shootHitLocationTrace` _impactpoint)
            (break)))
        (else
          (set `local._shootHitLocationTrace` __endtrace)))
      (`self.ShootProjectile` (`SceneComponent.GetSocketLocation` (`Character.Mesh` __equippedtoplayer) (`self.ArrowSpawnPointAttachmentName`)) (`local._shootHitLocationTrace`) (`self.WeaponOutputDamage`))
      (return false))
    (:`Is Not Valid`
      (return true))))

(fn `ShootProjectile`
  (params (SpawnLocation :type "Vector Structure") (HitPoint :type "Vector Structure") (Damage :type "Float (double-precision)"))
  (bind __equippedtoplayer (`self._equippedToPlayer`))
  (bind _returnvalue (`|SpawnActorFromClass` (`self.ArrowClassToSpawn`) (`KismetMathLibrary.MakeTransform` SpawnLocation (`KismetMathLibrary.FindLookAtRotation` SpawnLocation HitPoint)) "Undefined" "SelectDefaultAtRuntime" __equippedtoplayer Damage __equippedtoplayer (`self.ArrowSpeed`) __equippedtoplayer))
  (`self.OnProjectileShotEvent` _returnvalue))

(fn `UserConstructionScript`
  (`parent.UserConstructionScript`))