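; Base Blueprint for equippable one-hand-and-shield player weapons, extending the parent weapon's behavior to a separate Shield component.
; Attach and sheathe overrides call the parent, then snap the Shield to left-side sockets on the player character's mesh.
; Dropping detaches the Shield and places it at the drop location with a fixed rotation.
; On player death, the Shield detaches and enables collision and physics simulation.
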(fn `DropWeapon`
  (params (Location :type "Vector Structure"))
  (bind _shield (`self.Shield`))
  (`parent.DropWeapon` Location)
  (`SceneComponent.K2_DetachFromComponent` _shield "KeepWorld" "KeepWorld" "KeepWorld" true)
  (`SceneComponent.K2_SetWorldLocationAndRotation` _shield Location (struct :`Pitch` -90.0 :`Yaw` 135.0 :`Roll` -45.0) false false))

(fn `OnAttachWeapon`
  (params (PlayerCharacter :type "/Game/Blueprints/Game/Characters/Player/BP_BasePlayerCharacter Object Reference"))
  (`parent.OnAttachWeapon` PlayerCharacter)
  (`SceneComponent.K2_AttachToComponent` (`self.Shield`) (`Character.Mesh` PlayerCharacter) (`self.LeftShieldSocketAttachmentName`) "SnapToTarget" "SnapToTarget" "KeepWorld" true))

(fn `OnPlayerDied`
  (bind _shield (`self.Shield`))
  (`parent.OnPlayerDied`)
  (`SceneComponent.K2_DetachFromComponent` _shield "KeepWorld" "KeepWorld" "KeepWorld" true)
  (`PrimitiveComponent.SetCollisionEnabled` _shield "QueryAndPhysics")
  (`PrimitiveComponent.SetSimulatePhysics` _shield true))

(fn `OnSheatheWeapon`
  (params (PlayerCharacter :type "/Game/Blueprints/Game/Characters/Player/BP_BasePlayerCharacter Object Reference"))
  (`parent.OnSheatheWeapon` PlayerCharacter)
  (`SceneComponent.K2_AttachToComponent` (`self.Shield`) (`Character.Mesh` PlayerCharacter) (`self.LeftShieldSheathSocketName`) "SnapToTarget" "SnapToTarget" "KeepWorld" true))

(fn `UserConstructionScript`
  (`parent.UserConstructionScript`))