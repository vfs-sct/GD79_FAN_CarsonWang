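; Base pickup actor that hovers in place, flies to the player on sphere overlap, then notifies the player and destroys itself.
; Chest-spawned pickups disable collision and rise briefly for display before homing to the player, with timelines driving all motion.
; Collection is saved under the actor GUID unless chest-spawned or flagged to respawn on death, and BeginPlay destroys pickups already saved as collected.
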(event `self.ReceiveBeginPlay`
  (bind __currentposition (`self._currentPosition`))
  (bind _value (`self.GetSavedValue`))
  (switch `int` _value
    (:`Default`
      (`|ExecutionSequence`
        (:`then_0`
          ;[1 1 1] If opened from chest, give a chance to display the item before moving towards player
          (if (`self._isSpawnedFromChest`)
            (`PrimitiveComponent.SetCollisionEnabled` (`self.Sphere`) "NoCollision")
            (`TimelineComponent.Stop` (`self.HoverTimeline`))
            (`TimelineComponent.Stop` (`self.MoveTimeline`))
            (set `self._currentPosition` (`self.K2_GetActorLocation`))
            (bind (_direction _alpha) (`Timeline|DisplayTimeline`)
              (:`Update`
                (`self.K2_SetActorLocation` (`KismetMathLibrary.VLerp` __currentposition (`KismetMathLibrary.MakeVector` (.x __currentposition) (.y __currentposition) (+ (.z __currentposition) 200.0)) _alpha)))
              (:`Finished`
                (bind _asbp_base_player_character (cast `/Game/Blueprints/Game/Characters/Player/BP_BasePlayerCharacter` (`GameplayStatics.GetPlayerCharacter` 0)))
                (set `self._interactedPlayer` _asbp_base_player_character)
                (`self.ToPlayer`)))))
        (:`then_1`
          (bind (_direction_2 _zoffset _alpha_2) (`Timeline|HoverTimeline`)
            (:`Update`
              (`SceneComponent.K2_SetRelativeLocation` (`self.hoverRoot`) (`KismetMathLibrary.VLerp` (0.0 0.0 0.0) (`KismetMathLibrary.MakeVector` 0.0 0.0 _zoffset) _alpha_2) false false))))))
    (:`1`
      (`self.K2_DestroyActor`) ; Already picked up, destroy
    )))

(event `ToPlayer`
  (`/Engine/EditorBlueprintResources/StandardMacros.DoOnce` false :!label _label
    (:`Completed`
      (`TimelineComponent.Stop` (`self.HoverTimeline`))
      (set `self._startLocation` (`self.K2_GetActorLocation`))
      (bind (_direction _alpha _zoffset) (`Timeline|MoveTimeline`)
        (:`Update`
          (`self.K2_SetActorLocation` (`KismetMathLibrary.VLerp` (`self._startLocation`) (+ (`self.K2_GetActorLocation` (stale `self.Sphere.OnComponentBeginOverlap` _output_get)) (`KismetMathLibrary.MakeVector` 0.0 0.0 _zoffset)) _alpha)))
        (:`Finished`
          (`self.PickupComplete`))))))

(event `self.Sphere.OnComponentBeginOverlap`
  (params (OverlappedComponent :type "PrimitiveComponent Object Reference") (OtherActor :type "Actor Object Reference") (OtherComp :type "PrimitiveComponent Object Reference") (OtherBodyIndex :type Integer) (bFromSweep :type Boolean) (SweepResult :type "HitResult Structure (by ref)"))
  (if (not (`self._isSpawnedFromChest`))
    (bind _asbp_base_player_character (cast `/Game/Blueprints/Game/Characters/Player/BP_BasePlayerCharacter` OtherActor))
    (bind _output_get (set `self._interactedPlayer` _asbp_base_player_character))
    (goto _label)))

(event `/Game/Blueprints/Core/Save/BPI_Saveable.SetSavedValue`
  (params (Value :type Integer))
  (if (not (`self._isSpawnedFromChest`))
    (bind _key (`self.GetSavedKey`))
    (`/Game/Blueprints/Game/Utility/BP_FunctionLibrary.SetSaveKeyData` _key Value)))

(fn `GetSavedKey`
  (returns (Key :type String))
  (return (`KismetGuidLibrary.Conv_GuidToString` (`self.ActorGuid`))))

(fn `GetSavedValue`
  (returns (Value :type Integer))
  (return (`/Game/Blueprints/Game/Utility/BP_FunctionLibrary.GetSaveKeyData` (`KismetGuidLibrary.Conv_GuidToString` (`self.ActorGuid`)))))

(fn `PickupComplete`
  (`/Game/Blueprints/Game/Characters/Player/BP_BasePlayerCharacter.OnItemPickedUp` (`self._interactedPlayer`) self)
  (if (not (`self._isRespawnOnDeathIfAlreadyPickedUp`))
    (`self.SetSavedValue` (`self._pickedUpSavedKey`)))
  (`self.OnPickupComplete` self)
  (`self.K2_DestroyActor`))

(fn `UserConstructionScript`)