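; Game instance that holds session-wide state: checkpoint ID, equipped weapon classes, a key-value map, first boot-up flag and music playback.
; Init restores the checkpoint and loads or creates the settings save, applying saved volumes through a sound mix.
; Checkpoint IDs only advance unless backtracking is allowed, notify on change and are cleared on packaged-build shutdown.
; PlayMusic reuses one 2D audio source, fading out before switching tracks.
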(event `self.ReceiveInit`
  (`self.InitializeCheckpointData`)
  (`self.LoadGameStateSettings`))

(event `self.ReceiveShutdown`
  ;[1 1 1] Clearing checkpoint data when quitting within a real build.
  (if (`KismetSystemLibrary.IsPackagedForDistribution`)
    (`/Game/Blueprints/Game/Utility/BP_FunctionLibrary.SetCurrentCheckpointID` 0)))

(event `PlayMusic`
  (params (Music :type "SoundBase Object Reference") (FadeOutCurrentMusicDuration :type "Float (single-precision)") (FadeInNewMusicDuration :type "Float (single-precision)"))
  (bind __musicaudiosource (`self._musicAudioSource`))
  ;[1 1 1] Play Music
  (`/Engine/EditorBlueprintResources/StandardMacros.IsValid` (`self._musicAudioSource`)
    (:`Is Valid`
      (if (not (== Music (`AudioComponent.Sound` __musicaudiosource)))
        (if (`AudioComponent.IsPlaying` __musicaudiosource) :!label _label
          (`AudioComponent.FadeOut` __musicaudiosource FadeOutCurrentMusicDuration 0.0 "Linear")
          (`KismetSystemLibrary.Delay` FadeOutCurrentMusicDuration))
        (`AudioComponent.SetSound` __musicaudiosource Music)
        (`AudioComponent.Play` __musicaudiosource 0.0)
        (`AudioComponent.FadeIn` __musicaudiosource FadeInNewMusicDuration 1.0 0.0 "Linear")))
    (:`Is Not Valid`
      (bind _returnvalue (`GameplayStatics.CreateSound2D` Music 1.0 1.0 0.0 null true false))
      (set `self._musicAudioSource` _returnvalue)
      (goto _label))))

(fn `GetCheckpointID`
  (returns (id :type Integer))
  (return (`self._currentCheckpointID`)))

(fn `GetEquippedOneHandAndShieldWeaponClass`
  (returns (_equippedOneHandAndShieldWeaponClass :type "/Game/Blueprints/Game/PlayerWeapons/Equippable/1HandAndShield/BP_BaseOneHandAndShield Class Reference"))
  (return (`self._equippedOneHandAndShieldWeaponClass`)))

(fn `GetEquippedRangedWeaponClass`
  (returns (_equippedRangedWeaponClass :type "/Game/Blueprints/Game/PlayerWeapons/Equippable/Bow/BP_BaseRanged Class Reference"))
  (return (`self._equippedRangedWeaponClass`)))

(fn `GetEquippedTwoHandedWeaponClass`
  (returns (_equippedTwoHandWeaponClass :type "/Game/Blueprints/Game/PlayerWeapons/Equippable/2HandMelee/BP_BaseTwoHandMelee Class Reference"))
  (return (`self._equippedTwoHandWeaponClass`)))

(fn `GetGameStateSettings`
  (returns (_baseSaveGameState :type "/Game/Blueprints/Core/Save/SV_BaseGameState Object Reference"))
  (return (`self._baseSaveGameState`)))

(fn `GetIsOutOfMenuFirstTimeBootUp`
  (returns (_isOutOfMenuFirstTimeBootup :type Boolean))
  (return (`self._isOutOfMenuFirstTimeBootup`)))

(fn `GetSaveKey`
  (params (Key :type "String (by ref)") (DebugFailedResult :type Boolean))
  (returns (Value :type Integer))
  (bind (_value _returnvalue) (`BlueprintMapLibrary.Map_Find` (`self._keyMapping`) Key))
  (if _returnvalue
    (return _value)
    (else
      (if DebugFailedResult
        (`KismetSystemLibrary.PrintString` (`KismetStringLibrary.Concat_StrStr` "'" Key "'" "Not found in key mapping. Return 0.")))
      (return 0))))

(fn `InitializeCheckpointData`
  (`self.SetCheckpointID` (`/Game/Blueprints/Game/Checkpoint/Tools/BP_CheckpointData.GetCurrentID` (`self._currentCheckpointData`))))

(fn `LoadGameStateSettings`
  (bind __saveslotname (`self._saveSlotName`))
  (bind _returnvalue (`GameplayStatics.DoesSaveGameExist` __saveslotname))
  (if _returnvalue
    (bind _returnvalue_2 (`GameplayStatics.LoadGameFromSlot` __saveslotname))
    (bind _assv_base_game_state (cast `/Game/Blueprints/Core/Save/SV_BaseGameState` _returnvalue_2))
    (bind _output_get (set `self._baseSaveGameState` _assv_base_game_state))
    (`|ExecutionSequence`
      (:`then_0`
        (bind (__mastervolume __musicvolume __sfxvolume) (`/Game/Blueprints/Core/Save/SV_BaseGameState.GetVolumes` _output_get))
        (`GameplayStatics.SetSoundMixClassOverride` "/Game/Blueprints/Core/Audio/AudioMixer.AudioMixer" "/Game/Blueprints/Core/Audio/Channels/CustomMaster.CustomMaster" __mastervolume 1.0 0.0)
        (`GameplayStatics.SetSoundMixClassOverride` "/Game/Blueprints/Core/Audio/AudioMixer.AudioMixer" "/Game/Blueprints/Core/Audio/Channels/CustomMusic.CustomMusic" __musicvolume 1.0 0.0)
        (`GameplayStatics.SetSoundMixClassOverride` "/Game/Blueprints/Core/Audio/AudioMixer.AudioMixer" "/Game/Blueprints/Core/Audio/Channels/CustomSFX.CustomSFX" __sfxvolume 1.0 0.0)
        (`GameplayStatics.PushSoundMixModifier` "/Game/Blueprints/Core/Audio/AudioMixer.AudioMixer")))
    (else
      (bind _returnvalue_3 (`GameplayStatics.CreateSaveGameObject` "/Game/Blueprints/Core/Save/SV_BaseGameState.SV_BaseGameState_C"))
      (set `self._baseSaveGameState` _returnvalue_3))))

(fn `SaveGameStateSettings`
  (params (MasterVolume :type "Float (double-precision)") (MusicVolume :type "Float (double-precision)") (SfxVolume :type "Float (double-precision)") (_brightnessLevel :type "Float (double-precision)"))
  (bind __basesavegamestate (`self._baseSaveGameState`))
  (`/Engine/EditorBlueprintResources/StandardMacros.IsValid` __basesavegamestate
    (:`Is Valid`
      (`/Game/Blueprints/Core/Save/SV_BaseGameState.SetData` __basesavegamestate MasterVolume MusicVolume SfxVolume _brightnessLevel)
      (`GameplayStatics.SaveGameToSlot` (`self._baseSaveGameState`) (`self._saveSlotName`)))
    (:`Is Not Valid`
      (`KismetSystemLibrary.PrintString` "'_baseSaveGameState' IS NULL!"))))

(fn `SetCheckpointID`
  (params (newId :type Integer) (isAllowingBacktrackingId :type Boolean))
  (if isAllowingBacktrackingId
    (if (!= (`self._currentCheckpointID`) newId)
      (bind _output_get (set `self._currentCheckpointID` newId :!label _label))
      (`self.OnCheckpointSet` _output_get))
    (elif (> newId (`self._currentCheckpointID`))
      (goto _label))))

(fn `SetEquippedOneHandAndShieldWeaponClass`
  (params (_equippedOneHandAndShieldWeaponClass :type "/Game/Blueprints/Game/PlayerWeapons/Equippable/1HandAndShield/BP_BaseOneHandAndShield Class Reference"))
  (set `self._equippedOneHandAndShieldWeaponClass` _equippedOneHandAndShieldWeaponClass))

(fn `SetEquippedRangedWeaponClass`
  (params (_equippedRangedWeaponClass :type "/Game/Blueprints/Game/PlayerWeapons/Equippable/Bow/BP_BaseRanged Class Reference"))
  (set `self._equippedRangedWeaponClass` _equippedRangedWeaponClass))

(fn `SetEquippedTwoHandedWeaponClass`
  (params (_equippedTwoHandWeaponClass :type "/Game/Blueprints/Game/PlayerWeapons/Equippable/2HandMelee/BP_BaseTwoHandMelee Class Reference"))
  (set `self._equippedTwoHandWeaponClass` _equippedTwoHandWeaponClass))

(fn `SetIsOutOfMenuFirstTimeBootUp`
  (set `self._isOutOfMenuFirstTimeBootup` true))

(fn `SetSaveKey`
  (params (Key :type "String (by ref)") (Value :type "Integer (by ref)"))
  (`BlueprintMapLibrary.Map_Add` (`self._keyMapping`) Key Value))