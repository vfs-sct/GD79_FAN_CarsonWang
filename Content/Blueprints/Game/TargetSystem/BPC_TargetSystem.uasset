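; Lock-on targeting component that keeps the owning character's controller facing a chosen enemy.
; LockOn toggles targeting, sphere-tracing for the nearest targetable enemy that is also in the externally maintained TargetableActors array.
; CycleTargets uses a camera right-vector dot product to pick the closest neighbor left or right, also used when the current target leaves the array.
; Tick updates facing, and a bound death event triggers a forced re-search around the owner.
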(event `Initialize Variables`
  (params (`Owning Character` :type "/Game/Blueprints/Game/Characters/Player/BP_BasePlayerCharacter Object Reference"))
  ;[0 0 0] Initialize Variables
  (set `self.Owning Actor` `Owning Character`)
  (add `self.OnLockonToggleEvent` (delegate `OnLockonToggleEvent_Event`)))

(event `OnLockonToggleEvent_Event` :!signature `self.OnLockonToggleEvent`
  (params (target :type "Actor Object Reference"))
  (bind _lastenemytarget (`self.LastEnemyTarget`))
  ;[0 0 0] Initialize Variables
  ;[1 1 1] Listen for current target to die. If we are still targetting them, it will change ctargets.
  (bind _asbp_base_enemy_character (cast `/Game/Blueprints/Game/Characters/AI/Enemies/BP_BaseEnemyCharacter` target))
  (add `/Game/Blueprints/Game/Characters/BP_BaseCharacter.OnDeathComplete` _asbp_base_enemy_character (delegate `OnDeathComplete_Event`))
  ;[1 1 1] Unbind listening for previous target death on changing targets
  (`/Engine/EditorBlueprintResources/StandardMacros.IsValid` _lastenemytarget
    (:`Is Valid`
      (remove `/Game/Blueprints/Game/Characters/BP_BaseCharacter.OnDeathComplete` _lastenemytarget (delegate `OnDeathComplete_Event`))
      (set `self.LastEnemyTarget` _asbp_base_enemy_character))))

(event `OnDeathComplete_Event`
  ;[1 1 1] Listen for current target to die. If we are still targetting them, it will change ctargets.
  (`self.LockOn` (`Actor.K2_GetActorLocation` (`self.Owning Actor`)) (`Actor.K2_GetActorLocation` (`self.Owning Actor`)) 5000.0 true))

(event `self.ReceiveTick`
  (params (DeltaSeconds :type "Float (single-precision)"))
  ;[0 0 0] Event Tick
  (`self.SetCameraFocus`))

(event `Disable Lock On`
  ;[0 0 0] Turn off Lock on
  (set `self.IsLockedOn` false)
  (`self.OnLockonToggleEvent` null)
  (`self.SetTarget` null) ; Pass in null
)

(fn `AddTargetToArray`
  (params (Actor :type "Actor Object Reference (by ref)"))
  (bind _targetableactors (`self.TargetableActors`))
  (if (not (`KismetArrayLibrary.Array_Contains` _targetableactors Actor))
    (`KismetArrayLibrary.Array_Add` _targetableactors Actor)))

(fn `CycleTargets`
  (params (isRight :type Boolean))
  (returns (Target :type "Actor Object Reference"))
  (locals (_targetsTowardsDirection :type "Array of Actor Object Reference") (_nearestTarget :type "Actor Object Reference"))
  (bind _actor_to_target (`self.Actor To Target`))
  (bind _actor_to_target_2 (`self.Actor To Target`))
  (bind _output (`|GetArrayItem` (`local._targetsTowardsDirection`)))
  (`/Engine/EditorBlueprintResources/StandardMacros.IsValid` (`self.Actor To Target`)
    (:`Is Valid`
      (set `local._nearestTarget` null) ; Set Null
      (`KismetArrayLibrary.Array_Clear` (`local._targetsTowardsDirection`))
      (for _array_element (`self.TargetableActors`)
        (if (!= _array_element _actor_to_target)
          (bind _asbp_base_enemy_character (cast `/Game/Blueprints/Game/Characters/AI/Enemies/BP_BaseEnemyCharacter` _array_element))
          (bind _istargetable (`/Game/Blueprints/Core/Targetable/BPI_Targetable.IsTargetable` _asbp_base_enemy_character))
          (if _istargetable
            (if isRight
              (bind _returnvalue (> (`KismetMathLibrary.Dot_VectorVector` (`SceneComponent.GetRightVector` (`/Game/Blueprints/Game/Characters/Player/BP_BasePlayerCharacter.Camera` (`self.Owning Actor`))) (`KismetMathLibrary.Normal` (- (`Actor.K2_GetActorLocation` _actor_to_target) (`Actor.K2_GetActorLocation` _array_element)))) 0.0))
              (if (not _returnvalue)
                (`KismetArrayLibrary.Array_Add` (`local._targetsTowardsDirection`) _array_element :!label _label))
              (elif _returnvalue
                (goto _label))))))
      ;[1 1 1] Closest to Locked On Target
      (`/Engine/EditorBlueprintResources/StandardMacros.IsValid` _output
        (:`Is Valid`
          (set `local._nearestTarget` _output)
          (for _array_element_2 (`local._targetsTowardsDirection`)
            (if (!= _array_element_2 _actor_to_target_2)
              (if (< (`Actor.GetDistanceTo` _array_element_2 _actor_to_target_2) (`Actor.GetDistanceTo` (`local._nearestTarget`) _actor_to_target_2))
                (set `local._nearestTarget` _array_element_2))))
          (`self.OnTargetChanged` (`local._nearestTarget`)))
        (:`Is Not Valid`
          _))
      (return (`local._nearestTarget`)))))

(fn `LockOn`
  (params (Start :type "Vector Structure") (End :type "Vector Structure") (Radius :type "Float (single-precision)") (isForceSearchTarget :type Boolean))
  (returns (ChosenTarget :type "Actor Object Reference"))
  (locals (_nearestTarget :type "Actor Object Reference") (_objectTypes :type "Array of EObjectTypeQuery Enum") (_distance :type "Float (double-precision)" :default 99999.0))
  (bind __nearesttarget (`local._nearestTarget`))
  (if isForceSearchTarget
    _
    (elif (`self.IsLockedOn`)
      (`self.Disable Lock On`)
      (return null)
      (else
        _)))
  (bind (_outhits _returnvalue) (`KismetSystemLibrary.SphereTraceMultiForObjects` Start End Radius (`local._objectTypes`)))
  (if _returnvalue
    (for _array_element _outhits
      (bind _asbp_base_enemy_character (cast `/Game/Blueprints/Game/Characters/AI/Enemies/BP_BaseEnemyCharacter` (`.HitActor` (`GameplayStatics.BreakHitResult` _array_element))))
      (`/Engine/EditorBlueprintResources/StandardMacros.IsValid` _asbp_base_enemy_character
        (:`Is Valid`
          (if (`KismetArrayLibrary.Array_Contains` (`self.TargetableActors`) _asbp_base_enemy_character)
            (bind _istargetable (`/Game/Blueprints/Core/Targetable/BPI_Targetable.IsTargetable` _asbp_base_enemy_character))
            (if _istargetable
              (bind _returnvalue_2 (`Actor.GetDistanceTo` (`self.Owning Actor`) _asbp_base_enemy_character))
              (if (< _returnvalue_2 (`local._distance`))
                (set `local._distance` _returnvalue_2)
                (set `local._nearestTarget` _asbp_base_enemy_character)))))))
    (`/Engine/EditorBlueprintResources/StandardMacros.IsValid` __nearesttarget
      (:`Is Valid`
        (`self.OnTargetChanged` __nearesttarget)
        (return __nearesttarget))
      (:`Is Not Valid`
        (`self.Disable Lock On`)))))

(fn `OnTargetChanged`
  (params (Actor :type "Actor Object Reference"))
  (`self.SetTarget` Actor)
  (set `self.IsLockedOn` (`KismetSystemLibrary.IsValid` Actor))
  (`self.OnLockonToggleEvent` Actor))

(fn `RemoveTargetFromArray`
  (params (Actor :type "Actor Object Reference"))
  (bind _targetableactors (`self.TargetableActors`))
  (if (`KismetArrayLibrary.Array_Contains` _targetableactors Actor)
    (`KismetArrayLibrary.Array_RemoveItem` _targetableactors Actor)
    (if (== (`self.Actor To Target`) Actor)
      (bind _target (`self.CycleTargets` true))
      (`/Engine/EditorBlueprintResources/StandardMacros.IsValid` _target ; If nothing on right,  check left
        (:`Is Not Valid`
          (bind _target_2 (`self.CycleTargets` false))
          (`/Engine/EditorBlueprintResources/StandardMacros.IsValid` _target_2 ; No enemies around, disable
            (:`Is Not Valid`
              (`self.Disable Lock On`))))))))

(fn `SetCameraFocus`
  (bind _owning_actor (`self.Owning Actor`))
  (if (`self.IsLockedOn`)
    (`/Engine/EditorBlueprintResources/StandardMacros.IsValid` _owning_actor
      (:`Is Valid`
        (bind _actor_to_target (`self.Actor To Target`)
          (:`then`
            (if (`KismetArrayLibrary.Array_Contains` (`self.TargetableActors`) _actor_to_target)
              (`/Game/Blueprints/Game/Characters/Player/BP_BasePlayerCharacter.OnSetControllerFacing` _owning_actor (`Actor.K2_GetActorLocation` _actor_to_target) (`self.CameraInterpolationSpeed`))))
          (:`else`))))))

(fn `SetTarget`
  (params (Actor :type "Actor Object Reference"))
  (set `self.Actor To Target` Actor))