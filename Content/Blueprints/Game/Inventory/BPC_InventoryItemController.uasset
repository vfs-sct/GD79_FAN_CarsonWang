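; Inventory item controller component that tracks the count of an item and persists it under a save key.
; On BeginPlay it loads the saved count, and add or remove calls step it up or down by one.
; All changes go through SetCount, which saves the value, updates Count and fires a value-changed event, including on the initial load.
; Getters expose the count and whether any are available.
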(event `self.ReceiveBeginPlay`
  (`self.LoadCount`))

(fn `GetCount`
  (returns (_count :type Integer))
  (return (`self._count`)))

(fn `HasAvailable`
  (returns (hasAvailable :type Boolean))
  (return (> (`self._count`) 0)))

(fn `LoadCount`
  (`self.SetCount` (`/Game/Blueprints/Game/Utility/BP_FunctionLibrary.GetSaveKeyData` (`self._countSavedKey`))))

(fn `OnAdded`
  (bind _result (`/Engine/EditorBlueprintResources/StandardMacros.IncrementInt` (`self._count`))
    (:`  `
      (`self.SetCount` _result))))

(fn `OnRemoved`
  (bind _result (`/Engine/EditorBlueprintResources/StandardMacros.DecrementInt` (`self._count`))
    (:`  `
      (`self.SetCount` _result))))

(fn `SaveCount`
  (params (InputPin :type Integer))
  (`/Game/Blueprints/Game/Utility/BP_FunctionLibrary.SetSaveKeyData` (`self._countSavedKey`) InputPin))

(fn `SetCount`
  (params (Value :type Integer))
  (`self.SaveCount` Value)
  (bind _output_get (set `self._count` Value))
  (`self.OnValueChangedCompleted` _output_get))