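; Barricade actor with selectable visual variants, some of which have spikes that hurt the player on contact.
; The construction script uses BarricadeType to pick the mesh, flag whether it has a damage area, and fit the DamageCollision box to the spikes.
; When a BP_BasePlayerCharacter begins overlapping that box, it receives OnHit with SpikeContactDamage if the flag is set and damage is positive.
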(event `self.DamageCollision.OnComponentBeginOverlap`
  (params (OverlappedComponent :type "PrimitiveComponent Object Reference") (OtherActor :type "Actor Object Reference") (OtherComp :type "PrimitiveComponent Object Reference") (OtherBodyIndex :type Integer) (bFromSweep :type Boolean) (SweepResult :type "HitResult Structure (by ref)"))
  (if (`self._hasDamageArea`)
    (bind _asbp_base_player_character (cast `/Game/Blueprints/Game/Characters/Player/BP_BasePlayerCharacter` OtherActor))
    (if (> (`self._spikeContactDamage`) 0)
      (`/Game/Blueprints/Game/Characters/BP_BaseCharacter.OnHit` _asbp_base_player_character (`self._spikeContactDamage`)))))

(fn `SetDamageAreaPlacement`
  (params (InBoxExtent :type "Vector Structure") (RelativeLocation :type "Vector Structure") (RelativeRotation :type "Rotator Structure"))
  (bind _damagecollision (`self.DamageCollision`))
  (`BoxComponent.SetBoxExtent` _damagecollision InBoxExtent true)
  (`SceneComponent.K2_SetRelativeLocationAndRotation` _damagecollision RelativeLocation RelativeRotation false false))

(fn `UserConstructionScript`
  (bind _staticmesh (`self.StaticMesh`))
  ;[1 1 1] Set visuals based on type
  (switch `/Game/Blueprints/Game/Barricade/EN_Barricade` (`self._barricadeType`)
    (:`NewEnumerator0`
      (`StaticMeshComponent.SetStaticMesh` _staticmesh "/Game/Assets/Props/Barricades_Pack/Meshes/Barricade_High_1.Barricade_High_1")
      ;[1 1 1] Set offset collision area, size, and rotation if barricade has spikes
      (`self.SetDamageAreaPlacement` (119.143598 22.454118 36.418985) (-13.333333 -6.666667 393.333333))
      ;[1 1 1] Depending on visual, some have spikes and others dont. Touching the spikes will hurt the player
      (bind _output_get (set `self._hasDamageArea` true :!label _label))
      (`SceneComponent.SetVisibility` (`self.DamageCollision`) _output_get false))
    (:`NewEnumerator1`
      (`StaticMeshComponent.SetStaticMesh` _staticmesh "/Game/Assets/Props/Barricades_Pack/Meshes/Barricade_High_2.Barricade_High_2")
      (`self.SetDamageAreaPlacement` (132.864914 22.454118 73.329528) (6.666667 -6.666667 353.333333) (struct :`Pitch` -30.0))
      (goto _label))
    (:`NewEnumerator2`
      (`StaticMeshComponent.SetStaticMesh` _staticmesh "/Game/Assets/Props/Barricades_Pack/Meshes/Barricade_High_3.Barricade_High_3")
      (`self.SetDamageAreaPlacement` (120.136616 22.454118 73.329528) (0.0 -6.666667 386.666666))
      (goto _label))
    (:`NewEnumerator3`
      (`StaticMeshComponent.SetStaticMesh` _staticmesh "/Game/Assets/Props/Barricades_Pack/Meshes/Barricade_High_4.Barricade_High_4")
      (`self.SetDamageAreaPlacement` (132.705564 57.786516 106.780553) (13.333334 106.86923 257.68469) :!label _label_2)
      (goto _label))
    (:`NewEnumerator4`
      (`StaticMeshComponent.SetStaticMesh` _staticmesh "/Game/Assets/Props/Barricades_Pack/Meshes/Barricade_High_5.Barricade_High_5")
      (`self.SetDamageAreaPlacement` (132.705564 24.563874 44.830854) (6.666668 102.369589 337.291023))
      (goto _label))
    (:`NewEnumerator5`
      (`StaticMeshComponent.SetStaticMesh` _staticmesh "/Game/Assets/Props/Barricades_Pack/Meshes/Barricade_High_6.Barricade_High_6")
      (goto _label_2))
    (:`NewEnumerator6`
      (`StaticMeshComponent.SetStaticMesh` _staticmesh "/Game/Assets/Props/Barricades_Pack/Meshes/Barricade_High_7.Barricade_High_7")
      (bind _output_get_2 (set `self._hasDamageArea` false :!label _label_3))
      (`SceneComponent.SetVisibility` (`self.DamageCollision`) _output_get_2 false))
    (:`NewEnumerator7`
      (`StaticMeshComponent.SetStaticMesh` _staticmesh "/Game/Assets/Props/Barricades_Pack/Meshes/Barricade_High_8.Barricade_High_8")
      (goto _label_3))
    (:`NewEnumerator8`
      (`StaticMeshComponent.SetStaticMesh` _staticmesh "/Game/Assets/Props/Barricades_Pack/Meshes/Barricade_High_9.Barricade_High_9")
      (goto _label_3))
    (:`NewEnumerator9`
      (`StaticMeshComponent.SetStaticMesh` _staticmesh "/Game/Assets/Props/Barricades_Pack/Meshes/Barricade_Low_1.Barricade_Low_1")
      (`self.SetDamageAreaPlacement` (98.985467 71.133768 26.506209) (6.666668 2.369589 137.291023))
      (goto _label))
    (:`NewEnumerator10`
      (`StaticMeshComponent.SetStaticMesh` _staticmesh "/Game/Assets/Props/Barricades_Pack/Meshes/Barricade_Low_2.Barricade_Low_2")
      (`self.SetDamageAreaPlacement` (131.845732 78.575934 24.204195) (0.0 2.369589 137.291023))
      (goto _label))
    (:`NewEnumerator11`
      (`StaticMeshComponent.SetStaticMesh` _staticmesh "/Game/Assets/Props/Barricades_Pack/Meshes/Barricade_Medium_1.Barricade_Medium_1")
      (goto _label_3))
    (:`NewEnumerator12`
      (`StaticMeshComponent.SetStaticMesh` _staticmesh "/Game/Assets/Props/Barricades_Pack/Meshes/Barricade_Medium_2.Barricade_Medium_2")
      (goto _label_3))
    (:`NewEnumerator13`
      (`StaticMeshComponent.SetStaticMesh` _staticmesh "/Game/Assets/Props/Barricades_Pack/Meshes/Barricade_Medium_3.Barricade_Medium_3")
      (goto _label_3))
    (:`NewEnumerator14`
      (`StaticMeshComponent.SetStaticMesh` _staticmesh "/Game/Assets/Props/Barricades_Pack/Meshes/Barricade_Small_1.Barricade_Small_1")
      (`self.SetDamageAreaPlacement` (51.453917 42.578305 17.0) (0.0 9.036256 133.333333) (struct :`Yaw` -30.0))
      (goto _label))
    (:`NewEnumerator15`
      (`StaticMeshComponent.SetStaticMesh` _staticmesh "/Game/Assets/Props/Barricades_Pack/Meshes/Barricade_Small_2.Barricade_Small_2")
      (`self.SetDamageAreaPlacement` (51.453917 42.578305 28.964814) (0.0 -4.297077 150.624356) (struct :`Yaw` -30.0))
      (goto _label))))