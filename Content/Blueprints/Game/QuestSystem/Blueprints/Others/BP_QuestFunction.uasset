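; BP_QuestFunction is a set of helper functions for the quest system, serving quest data lookups and category colors.
; GetCategoryColor maps each quest category to a semi-transparent color.
; GetQuestFromDataTable reads a row by the handle's row name, always from DT_Quests regardless of the handle's table.
; GetQuestFromGuid linearly scans DT_Quests rows for a matching QuestID, stopping at the first hit.
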(fn `GetCategoryColor`
  (params (Index :type "/Game/Blueprints/Game/QuestSystem/Logics/Enums/E_QuestCategory Enum" :default "NewEnumerator3"))
  (returns (Color :type "LinearColor Structure"))
  (return (select `/Game/Blueprints/Game/QuestSystem/Logics/Enums/E_QuestCategory` Index :`NewEnumerator3` (struct :`R` 1.0 :`G` 1.0 :`B` 1.0 :`A` 0.75) :`NewEnumerator0` (struct :`R` 0.101961 :`G` 0.32549 :`B` 1.0 :`A` 0.75) :`NewEnumerator1` (struct :`R` 0.356863 :`G` 1.0 :`B` 0.411765 :`A` 0.74902) :`NewEnumerator14` (struct :`R` 1.0 :`G` 0.905882 :`B` 0.368627 :`A` 0.74902) :`NewEnumerator5` (struct :`R` 1.0 :`G` 0.321569 :`B` 0.070588 :`A` 0.74902) :`NewEnumerator15` (struct :`R` 0.627098 :`G` 1.0 :`B` 0.034841 :`A` 0.75) :`NewEnumerator4` (struct :`R` 1.0 :`A` 0.74902) :!type "LinearColor Structure")))

(fn `GetQuestFromDataTable`
  (params (DataTable :type "DataTableRowHandle Structure"))
  (returns (`Sucess?` :type Boolean) (QuestData :type "/Game/Blueprints/Game/QuestSystem/Logics/Structures/S_QuestData Structure"))
  (bind _returnvalue (`|GetDataTableRow` "/Game/Blueprints/Game/QuestSystem/Logics/DT_Quests.DT_Quests" (`.RowName` (break `DataTableRowHandle` DataTable)))
    (:`then`
      (return true _returnvalue))
    (:`RowNotFound`
      (return false))))

(fn `GetQuestFromGuid`
  (params (QuestGuid :type "Guid Structure"))
  (returns (`Found?` :type Boolean) (QuestData :type "/Game/Blueprints/Game/QuestSystem/Logics/Structures/S_QuestData Structure"))
  (locals (`Local_Found?` :type Boolean) (Local_QuestData :type "/Game/Blueprints/Game/QuestSystem/Logics/Structures/S_QuestData Structure"))
  (bind _outrownames (`DataTableFunctionLibrary.GetDataTableRowNames` "/Game/Blueprints/Game/QuestSystem/Logics/DT_Quests.DT_Quests"))
  (for _array_element _outrownames
    (bind _returnvalue (`|GetDataTableRow` "/Game/Blueprints/Game/QuestSystem/Logics/DT_Quests.DT_Quests" _array_element)
      (:`then`
        (if (== (`local.QuestGuid`) (`.QuestID_49_6980E81A4EA48C0674BD0AB490768D3B` (break `/Game/Blueprints/Game/QuestSystem/Logics/Structures/S_QuestData` _returnvalue)))
          (set `local.Local_Found?` true)
          (set `local.Local_QuestData` _returnvalue)
          (break)))))
  (return (`local.Local_Found?`) (`local.Local_QuestData`)))