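; Quest child actor for talk interactions, exposing quest data and an interaction prompt widget.
; On BeginPlay it caches the user widget from its widget component and hides it through the quest visibility message.
; Later visibility and distance messages are forwarded straight to that widget.
; The interact interface function returns the objective to complete, whether the quest can finish, and the quest to give, leaving quest logic to the caller.
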(event `self.ReceiveBeginPlay`
  ;[1 1 1] Constructeur
  (`parent.ReceiveBeginPlay`)
  (set `self.WidgetRef` (`WidgetComponent.GetUserWidgetObject` (`self.Widget`)))
  (`/Game/Blueprints/Game/QuestSystem/Blueprints/Others/BPI_QuestObjectiveInterface.MSG_QuestSetInteractVisibility` false))

(event `/Game/Blueprints/Game/QuestSystem/Blueprints/Others/BPI_QuestObjectiveInterface.MSG_QuestSetInteractVisibility`
  (params (`IsVisible?` :type Boolean) (Distance :type Integer))
  ;[1 1 1] Set interaction widget visibility
  (message `/Game/Blueprints/Game/QuestSystem/Blueprints/Others/BPI_QuestObjectiveInterface.MSG_QuestSetInteractVisibility` (`self.WidgetRef`) `IsVisible?` Distance))

(fn `MSG_QuestOnInteract`
  (returns (ObjectiveToComplete :type "Array of /Game/Blueprints/Game/QuestSystem/Logics/Structures/S_ActorQuestObjective Structure") (QuestCanFinish :type "Array of DataTableRowHandle Structure") (QuestToGive :type "Array of DataTableRowHandle Structure"))
  (return (`self.ObjectiveToComplete`) (`self.QuestCanFinish`) (`self.QuestToGive`)))

(fn `UserConstructionScript`
  (`parent.UserConstructionScript`))