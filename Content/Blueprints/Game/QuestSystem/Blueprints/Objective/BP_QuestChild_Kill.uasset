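; BP_QuestChild_Kill is a quest objective actor that simulates a kill target using a demo shape chosen by DemoType in the construction script.
; When a locally controlled character overlaps its collision sphere, OnKilled passes ObjectiveToComplete to that character's BPC_Quest component.
; The shape then hides for a short delay before reappearing, with a DoOnce blocking repeat triggers until it returns.
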(event `self.CollisionSphere.OnComponentBeginOverlap`
  (params (OverlappedComponent :type "PrimitiveComponent Object Reference") (OtherActor :type "Actor Object Reference") (OtherComp :type "PrimitiveComponent Object Reference") (OtherBodyIndex :type Integer) (bFromSweep :type Boolean) (SweepResult :type "HitResult Structure (by ref)"))
  (bind _actualmeshref (`self.ActualMeshRef`))
  ;[1 1 1] On overlap
  (bind _ascharacter (cast `Character` OtherActor))
  (if (`Pawn.IsLocallyControlled` _ascharacter)
    (`/Engine/EditorBlueprintResources/StandardMacros.DoOnce` false :!label _label
      (:`Completed`
        (`self.OnKilled` _ascharacter)
        (`SceneComponent.SetVisibility` _actualmeshref false false)
        (`KismetSystemLibrary.Delay` 3.0)
        (`SceneComponent.SetVisibility` _actualmeshref true false)
        (goto _label :!via `Reset`)))))

(event `OnKilled`
  (params (KillerRef :type "Actor Object Reference"))
  (bind _returnvalue (`self.GetComponentByClass` KillerRef "/Game/Blueprints/Game/QuestSystem/Blueprints/BPC_Quest.BPC_Quest_C"))
  ;[1 1 1] Kill model
  (`/Engine/EditorBlueprintResources/StandardMacros.IsValid` _returnvalue
    (:`Is Valid`
      (`/Game/Blueprints/Game/QuestSystem/Blueprints/BPC_Quest.ByActorDoObjectives` _returnvalue (`self.ObjectiveToComplete`)))))

(fn `UserConstructionScript`
  (`parent.UserConstructionScript`)
  (bind _output_get (set `self.ActualMeshRef` (select `/Game/Blueprints/Game/QuestSystem/Demo/E_DemoMonsterType` (`self.DemoType`) :`NewEnumerator1` (`self.Sphere`) :`NewEnumerator0` (`self.Cube`) :`NewEnumerator2` (`self.Cylinder`) :`NewEnumerator3` (`self.Cone`) :!type "SceneComponent Object Reference")))
  (`SceneComponent.SetVisibility` _output_get true false))