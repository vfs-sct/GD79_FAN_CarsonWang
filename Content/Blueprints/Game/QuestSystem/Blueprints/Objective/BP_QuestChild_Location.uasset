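; BP_QuestChild_Location is a location objective actor for the quest system that completes objectives when the player enters its box.
; A locally controlled Character overlapping the box passes ObjectiveToComplete to its BPC_Quest component through ByActorDoObjectives.
; A DoOnce that resets after a three-second delay throttles repeat triggers.
; The construction script applies InteractionTransform to the box, so the trigger area is adjustable per instance.
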(event `self.Box.OnComponentBeginOverlap`
  (params (OverlappedComponent :type "PrimitiveComponent Object Reference") (OtherActor :type "Actor Object Reference") (OtherComp :type "PrimitiveComponent Object Reference") (OtherBodyIndex :type Integer) (bFromSweep :type Boolean) (SweepResult :type "HitResult Structure (by ref)"))
  ;[1 1 1] On overlap
  (bind _ascharacter (cast `Character` OtherActor))
  (if (`Pawn.IsLocallyControlled` _ascharacter)
    (`/Engine/EditorBlueprintResources/StandardMacros.DoOnce` false :!label _label
      (:`Completed`
        (bind _returnvalue (`self.GetComponentByClass` _ascharacter "/Game/Blueprints/Game/QuestSystem/Blueprints/BPC_Quest.BPC_Quest_C"))
        (`/Engine/EditorBlueprintResources/StandardMacros.IsValid` _returnvalue
          (:`Is Valid`
            (`/Game/Blueprints/Game/QuestSystem/Blueprints/BPC_Quest.ByActorDoObjectives` _returnvalue (`self.ObjectiveToComplete`))
            (`KismetSystemLibrary.Delay` 3.0)
            (goto _label :!via `Reset`)))))))

(fn `UserConstructionScript`
  (`parent.UserConstructionScript`)
  (`SceneComponent.K2_SetRelativeTransform` (`self.Box`) (`self.InteractionTransform`) false false))