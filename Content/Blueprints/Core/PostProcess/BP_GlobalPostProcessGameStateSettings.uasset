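; Global post-process Blueprint that applies the player's brightness setting as exposure compensation.
; On BeginPlay it loads the saved brightness from the custom game instance's game state settings and binds to the HUD's brightness-changed event.
; Both the initial load and later changes go through SetBrightness, which replaces the post-process component's whole settings struct with one built from that value.
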(event `self.ReceiveBeginPlay`
  (`self.LoadBrightness`)
  (add `/Game/Blueprints/Game/UI/Hud/HUD_BaseCustom.OnBrightnessValueChanged` (`/Game/Blueprints/Game/Utility/BP_FunctionLibrary.GetBaseCustomHUD`) (delegate `OnBrightnessValueChanged_Event`)))

(event `OnBrightnessValueChanged_Event`
  (params (value :type "Float (double-precision)"))
  (`self.SetBrightness` value))

(fn `LoadBrightness`
  (`self.SetBrightness` (`/Game/Blueprints/Core/Save/SV_BaseGameState.GetBrightness` (`/Game/Blueprints/Game/GameInstance/BP_CustomGameInstance.GetGameStateSettings` (`/Game/Blueprints/Game/Utility/BP_FunctionLibrary.GetCustomGameInstance`)))))

(fn `SetBrightness`
  (params (`Exposure Compensation` :type "Float (single-precision)"))
  (set `PostProcessComponent.Settings` (make `PostProcessSettings` :`AutoExposureBias` `Exposure Compensation`) (`self.PostProcess`)))

(fn `UserConstructionScript`)