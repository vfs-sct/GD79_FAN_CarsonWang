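; BP_FollowSpline is a spline utility that moves a given actor along its path, optionally starting on BeginPlay.
; A timeline, rate-scaled by duration, sets the actor's location and rotation (plus an offset) at constant velocity, teleporting without sweep.
; Spline type controls looping: Linear clears the actor and signals completion, Ping Pong alternates direction with a callback, and looping types repeat.
; It extends a parent spline class and supports backward play and stopping.
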(event `self.ReceiveBeginPlay`
  ;[1 1 1] Start playing on instantiation check
  (if (and (`self._isStartPlaying`) (`KismetSystemLibrary.IsValid` (`self._actorToMove`)))
    (`self.Play` (`self._actorToMove`) (`self._duration`) "Forward" (`self._isStartPlayingRotationOffset`))))

(event `Play`
  (params (ActorToMove :type "Actor Object Reference") (Duration :type "Float (double-precision)") (TimelineDirection :type "ETimelineDirection Enum" :default "Forward") (OffsetRotation :type "Rotator Structure"))
  (bind __actortomove (`self._actorToMove`))
  (bind _spline (`self.Spline`))
  (bind _splinetimeline (`self.SplineTimeline`))
  ;[1 1 1] Play
  (`/Engine/EditorBlueprintResources/StandardMacros.IsValid` ActorToMove
    (:`Is Valid`
      (`self.SetActorToMove` ActorToMove)
      (`self.SetDuration` Duration)
      (switch `ETimelineDirection` TimelineDirection
        (:`Forward`
          (bind (_direction _alpha) (`Timeline|SplineTimeline` :!label _label)
            (:`Update`
              (`self.K2_SetActorLocation` __actortomove (`SplineComponent.GetLocationAtTime` _spline _alpha "World" true) false true)
              (`self.K2_SetActorRotation` __actortomove (`KismetMathLibrary.ComposeRotators` (`SplineComponent.GetRotationAtTime` _spline _alpha "World" true) OffsetRotation) true))
            (:`Finished`
              (switch `/Game/Blueprints/Core/Utility/Spline/EN_SplineMovementType` "NewEnumerator0" ; LinearLoop and Loop never reach\n'Finished' as the spline & timeline is on a loop
                (:`NewEnumerator1`
                  (`self.SetActorToMove` null) ; Clear the '_actorToMove' by passing\nin a null value in the 'Actor to Move'\nvariable
                  (`self.OnLinearMoveComplete`))
                (:`NewEnumerator2`
                  (bind _isa (`/Engine/EditorBlueprintResources/StandardMacros.FlipFlop`)
                    (:`A`
                      (`TimelineComponent.Reverse` _splinetimeline))
                    (:`B`
                      (`TimelineComponent.Play` _splinetimeline)))
                  (`self.OnPingPongReachedComplete` _isa))))))
        (:`Backward`
          (goto _label :!via `Reverse`))))
    (:`Is Not Valid`
      (`KismetSystemLibrary.PrintString` "\"ERROR: YOUR SPLINE IS TRYING TO MOVE/PLAY A NULL 'ACTOR TO MOVE' REFERENCE! MAKE SURE TO GIVE A REFERENCE TO \nAN OBJECT IF YOU WANT IT TO MOVE ON THE SPLINE!\"" true true (struct :`R` 1.0 :`B` 0.113821 :`A` 1.0) 20.0))))

(event `Stop`
  ;[1 1 1] Stop
  (`TimelineComponent.Stop` (`self.SplineTimeline`)))

(fn `SetActorToMove`
  (params (_actorToMove :type "Actor Object Reference"))
  (set `self._actorToMove` _actorToMove))

(fn `SetDuration`
  (params (Duration :type "Float (double-precision)"))
  (`TimelineComponent.SetPlayRate` (`self.SplineTimeline`) (/ 1.0 Duration)))

(fn `SetSplineType`
  (params (splineType :type "/Game/Blueprints/Core/Utility/Spline/EN_SplineMovementType Enum" :default "NewEnumerator0"))
  (`parent.SetSplineType` splineType)
  (`TimelineComponent.SetLooping` (`self.SplineTimeline`) (select `/Game/Blueprints/Core/Utility/Spline/EN_SplineMovementType` splineType :`NewEnumerator0` true :`NewEnumerator3` true)))

(fn `UserConstructionScript`
  (`parent.UserConstructionScript`))