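; BP_Zombie_OldRd is a stylized zombie enemy NPC assembled from modular body, armor, clothing and weapon mesh components.
; On BeginPlay it sets the main SkeletalMeshComponent as leader pose for all those parts, so they animate together from one skeleton.
; The graph holds no AI, combat or other gameplay logic, and the construction script is empty.
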(event `self.ReceiveBeginPlay`
  (`SkinnedMeshComponent.SetLeaderPoseComponent` (`self.ArmBracer`) (`self.SkeletalMeshComponent`) false false)
  (`SkinnedMeshComponent.SetLeaderPoseComponent` (`self.Weapon_L`) (`self.SkeletalMeshComponent`) false false)
  (`SkinnedMeshComponent.SetLeaderPoseComponent` (`self.BootsPads`) (`self.SkeletalMeshComponent`) false false)
  (`SkinnedMeshComponent.SetLeaderPoseComponent` (`self.ArmPads`) (`self.SkeletalMeshComponent`) false false)
  (`SkinnedMeshComponent.SetLeaderPoseComponent` (`self.Belt`) (`self.SkeletalMeshComponent`) false false)
  (`SkinnedMeshComponent.SetLeaderPoseComponent` (`self.Tabard`) (`self.SkeletalMeshComponent`) false false)
  (`SkinnedMeshComponent.SetLeaderPoseComponent` (`self.Shoulder_R`) (`self.SkeletalMeshComponent`) false false)
  (`SkinnedMeshComponent.SetLeaderPoseComponent` (`self.BodyStuff`) (`self.SkeletalMeshComponent`) false false)
  (`SkinnedMeshComponent.SetLeaderPoseComponent` (`self.Shoulder_L`) (`self.SkeletalMeshComponent`) false false)
  (`SkinnedMeshComponent.SetLeaderPoseComponent` (`self.Helm`) (`self.SkeletalMeshComponent`) false false)
  (`SkinnedMeshComponent.SetLeaderPoseComponent` (`self.Boots`) (`self.SkeletalMeshComponent`) false false)
  (`SkinnedMeshComponent.SetLeaderPoseComponent` (`self.Weapon_R`) (`self.SkeletalMeshComponent`) false false)
  (`SkinnedMeshComponent.SetLeaderPoseComponent` (`self.Bracers`) (`self.SkeletalMeshComponent`) false false)
  (`SkinnedMeshComponent.SetLeaderPoseComponent` (`self.Buckle`) (`self.SkeletalMeshComponent`) false false)
  (`SkinnedMeshComponent.SetLeaderPoseComponent` (`self.Pants`) (`self.SkeletalMeshComponent`) false false))

(fn `UserConstructionScript`)