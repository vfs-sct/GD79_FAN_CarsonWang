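; Placeable horror decal actor that shows a chosen material from a library of skulls, text, symbols, smears, stains and circular designs.
; The Construction Script switches on DecalType to a per-category function, which maps DecalNumber to a material instance on the Decal component.
; It also rescales the decal from the actor's scale, swapping Y and Z, negating and halving, as a scaling fix.
; No runtime logic runs.
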(fn `Circular Decals Switch`
  (bind _decal (`self.Decal`))
  (switch `int` (`self.DecalNumber`)
    (:`0`
      (`DecalComponent.SetDecalMaterial` _decal "/Game/Assets/Decals/HorrorDecals/Materials/HorrorDecals/Circular/MI_HorrorDecals_Circular_A.MI_HorrorDecals_Circular_A"))
    (:`1`
      (`DecalComponent.SetDecalMaterial` _decal "/Game/Assets/Decals/HorrorDecals/Materials/HorrorDecals/Circular/MI_HorrorDecals_Circular_B.MI_HorrorDecals_Circular_B"))
    (:`2`
      (`DecalComponent.SetDecalMaterial` _decal "/Game/Assets/Decals/HorrorDecals/Materials/HorrorDecals/Circular/MI_HorrorDecals_Circular_C.MI_HorrorDecals_Circular_C"))
    (:`3`
      (`DecalComponent.SetDecalMaterial` _decal "/Game/Assets/Decals/HorrorDecals/Materials/HorrorDecals/Circular/MI_HorrorDecals_Circular_D.MI_HorrorDecals_Circular_D"))
    (:`4`
      (`DecalComponent.SetDecalMaterial` _decal "/Game/Assets/Decals/HorrorDecals/Materials/HorrorDecals/Circular/MI_HorrorDecals_Circular_E.MI_HorrorDecals_Circular_E"))
    (:`5`
      (`DecalComponent.SetDecalMaterial` _decal "/Game/Assets/Decals/HorrorDecals/Materials/HorrorDecals/Circular/MI_HorrorDecals_Circular_F.MI_HorrorDecals_Circular_F"))
    (:`6`
      (`DecalComponent.SetDecalMaterial` _decal "/Game/Assets/Decals/HorrorDecals/Materials/HorrorDecals/Circular/MI_HorrorDecals_Circular_G.MI_HorrorDecals_Circular_G"))
    (:`7`
      (`DecalComponent.SetDecalMaterial` _decal "/Game/Assets/Decals/HorrorDecals/Materials/HorrorDecals/Circular/MI_HorrorDecals_Circular_H.MI_HorrorDecals_Circular_H"))
    (:`8`
      (`DecalComponent.SetDecalMaterial` _decal "/Game/Assets/Decals/HorrorDecals/Materials/HorrorDecals/Circular/MI_HorrorDecals_Circular_I.MI_HorrorDecals_Circular_I"))
    (:`9`
      (`DecalComponent.SetDecalMaterial` _decal "/Game/Assets/Decals/HorrorDecals/Materials/HorrorDecals/Circular/MI_HorrorDecals_Circular_J.MI_HorrorDecals_Circular_J"))
    (:`10`
      (`DecalComponent.SetDecalMaterial` _decal "/Game/Assets/Decals/HorrorDecals/Materials/HorrorDecals/Circular/MI_HorrorDecals_Circular_K.MI_HorrorDecals_Circular_K"))
    (:`11`
      (`DecalComponent.SetDecalMaterial` _decal "/Game/Assets/Decals/HorrorDecals/Materials/HorrorDecals/Circular/MI_HorrorDecals_Circular_L.MI_HorrorDecals_Circular_L"))
    (:`12`
      (`DecalComponent.SetDecalMaterial` _decal "/Game/Assets/Decals/HorrorDecals/Materials/HorrorDecals/Circular/MI_HorrorDecals_Circular_M.MI_HorrorDecals_Circular_M"))
    (:`13`
      (`DecalComponent.SetDecalMaterial` _decal "/Game/Assets/Decals/HorrorDecals/Materials/HorrorDecals/Circular/MI_HorrorDecals_Circular_N.MI_HorrorDecals_Circular_N"))
    (:`14`
      (`DecalComponent.SetDecalMaterial` _decal "/Game/Assets/Decals/HorrorDecals/Materials/HorrorDecals/Circular/MI_HorrorDecals_Circular_O.MI_HorrorDecals_Circular_O"))
    (:`15`
      (`DecalComponent.SetDecalMaterial` _decal "/Game/Assets/Decals/HorrorDecals/Materials/HorrorDecals/Circular/MI_HorrorDecals_Circular_P.MI_HorrorDecals_Circular_P"))))

(fn `Large Alien Text Switch`
  (bind _decal (`self.Decal`))
  (switch `int` (`self.DecalNumber`)
    (:`0`
      (`DecalComponent.SetDecalMaterial` _decal "/Game/Assets/Decals/HorrorDecals/Materials/HorrorDecals/LargeAlienText/MI_HorrorDecals_LargeAlienTexMI_A.MI_HorrorDecals_LargeAlienTexMI_A"))
    (:`1`
      (`DecalComponent.SetDecalMaterial` _decal "/Game/Assets/Decals/HorrorDecals/Materials/HorrorDecals/LargeAlienText/MI_HorrorDecals_LargeAlienTexMI_B.MI_HorrorDecals_LargeAlienTexMI_B"))
    (:`2`
      (`DecalComponent.SetDecalMaterial` _decal "/Game/Assets/Decals/HorrorDecals/Materials/HorrorDecals/LargeAlienText/MI_HorrorDecals_LargeAlienTexMI_C.MI_HorrorDecals_LargeAlienTexMI_C"))
    (:`3`
      (`DecalComponent.SetDecalMaterial` _decal "/Game/Assets/Decals/HorrorDecals/Materials/HorrorDecals/LargeAlienText/MI_HorrorDecals_LargeAlienTexMI_D.MI_HorrorDecals_LargeAlienTexMI_D"))
    (:`4`
      (`DecalComponent.SetDecalMaterial` _decal "/Game/Assets/Decals/HorrorDecals/Materials/HorrorDecals/LargeAlienText/MI_HorrorDecals_LargeAlienTexMI_E.MI_HorrorDecals_LargeAlienTexMI_E"))
    (:`5`
      (`DecalComponent.SetDecalMaterial` _decal "/Game/Assets/Decals/HorrorDecals/Materials/HorrorDecals/LargeAlienText/MI_HorrorDecals_LargeAlienTexMI_F.MI_HorrorDecals_LargeAlienTexMI_F"))
    (:`6`
      (`DecalComponent.SetDecalMaterial` _decal "/Game/Assets/Decals/HorrorDecals/Materials/HorrorDecals/LargeAlienText/MI_HorrorDecals_LargeAlienTexMI_G.MI_HorrorDecals_LargeAlienTexMI_G"))
    (:`7`
      (`DecalComponent.SetDecalMaterial` _decal "/Game/Assets/Decals/HorrorDecals/Materials/HorrorDecals/LargeAlienText/MI_HorrorDecals_LargeAlienTexMI_H.MI_HorrorDecals_LargeAlienTexMI_H"))
    (:`8`
      (`DecalComponent.SetDecalMaterial` _decal "/Game/Assets/Decals/HorrorDecals/Materials/HorrorDecals/LargeAlienText/MI_HorrorDecals_LargeAlienTexMI_I.MI_HorrorDecals_LargeAlienTexMI_I"))
    (:`9`
      (`DecalComponent.SetDecalMaterial` _decal "/Game/Assets/Decals/HorrorDecals/Materials/HorrorDecals/LargeAlienText/MI_HorrorDecals_LargeAlienTexMI_J.MI_HorrorDecals_LargeAlienTexMI_J"))
    (:`10`
      (`DecalComponent.SetDecalMaterial` _decal "/Game/Assets/Decals/HorrorDecals/Materials/HorrorDecals/LargeAlienText/MI_HorrorDecals_LargeAlienTexMI_K.MI_HorrorDecals_LargeAlienTexMI_K"))
    (:`11`
      (`DecalComponent.SetDecalMaterial` _decal "/Game/Assets/Decals/HorrorDecals/Materials/HorrorDecals/LargeAlienText/MI_HorrorDecals_LargeAlienTexMI_L.MI_HorrorDecals_LargeAlienTexMI_L"))
    (:`12`
      (`DecalComponent.SetDecalMaterial` _decal "/Game/Assets/Decals/HorrorDecals/Materials/HorrorDecals/LargeAlienText/MI_HorrorDecals_LargeAlienTexMI_M.MI_HorrorDecals_LargeAlienTexMI_M"))
    (:`13`
      (`DecalComponent.SetDecalMaterial` _decal "/Game/Assets/Decals/HorrorDecals/Materials/HorrorDecals/LargeAlienText/MI_HorrorDecals_LargeAlienTexMI_N.MI_HorrorDecals_LargeAlienTexMI_N"))))

(fn `Large English Text Switch`
  (bind _decal (`self.Decal`))
  (switch `int` (`self.DecalNumber`)
    (:`0`
      (`DecalComponent.SetDecalMaterial` _decal "/Game/Assets/Decals/HorrorDecals/Materials/HorrorDecals/LargeEnglishText/MI_HorrorDecals_LargeEnglishText_A.MI_HorrorDecals_LargeEnglishText_A"))
    (:`1`
      (`DecalComponent.SetDecalMaterial` _decal "/Game/Assets/Decals/HorrorDecals/Materials/HorrorDecals/LargeEnglishText/MI_HorrorDecals_LargeEnglishText_B.MI_HorrorDecals_LargeEnglishText_B"))
    (:`2`
      (`DecalComponent.SetDecalMaterial` _decal "/Game/Assets/Decals/HorrorDecals/Materials/HorrorDecals/LargeEnglishText/MI_HorrorDecals_LargeEnglishText_C.MI_HorrorDecals_LargeEnglishText_C"))
    (:`3`
      (`DecalComponent.SetDecalMaterial` _decal "/Game/Assets/Decals/HorrorDecals/Materials/HorrorDecals/LargeEnglishText/MI_HorrorDecals_LargeEnglishText_D.MI_HorrorDecals_LargeEnglishText_D"))
    (:`4`
      (`DecalComponent.SetDecalMaterial` _decal "/Game/Assets/Decals/HorrorDecals/Materials/HorrorDecals/LargeEnglishText/MI_HorrorDecals_LargeEnglishText_E.MI_HorrorDecals_LargeEnglishText_E"))
    (:`5`
      (`DecalComponent.SetDecalMaterial` _decal "/Game/Assets/Decals/HorrorDecals/Materials/HorrorDecals/LargeEnglishText/MI_HorrorDecals_LargeEnglishText_F.MI_HorrorDecals_LargeEnglishText_F"))
    (:`6`
      (`DecalComponent.SetDecalMaterial` _decal "/Game/Assets/Decals/HorrorDecals/Materials/HorrorDecals/LargeEnglishText/MI_HorrorDecals_LargeEnglishText_G.MI_HorrorDecals_LargeEnglishText_G"))
    (:`7`
      (`DecalComponent.SetDecalMaterial` _decal "/Game/Assets/Decals/HorrorDecals/Materials/HorrorDecals/LargeEnglishText/MI_HorrorDecals_LargeEnglishText_H.MI_HorrorDecals_LargeEnglishText_H"))
    (:`8`
      (`DecalComponent.SetDecalMaterial` _decal "/Game/Assets/Decals/HorrorDecals/Materials/HorrorDecals/LargeEnglishText/MI_HorrorDecals_LargeEnglishText_I.MI_HorrorDecals_LargeEnglishText_I"))
    (:`9`
      (`DecalComponent.SetDecalMaterial` _decal "/Game/Assets/Decals/HorrorDecals/Materials/HorrorDecals/LargeEnglishText/MI_HorrorDecals_LargeEnglishText_J.MI_HorrorDecals_LargeEnglishText_J"))
    (:`10`
      (`DecalComponent.SetDecalMaterial` _decal "/Game/Assets/Decals/HorrorDecals/Materials/HorrorDecals/LargeEnglishText/MI_HorrorDecals_LargeEnglishText_K.MI_HorrorDecals_LargeEnglishText_K"))
    (:`11`
      (`DecalComponent.SetDecalMaterial` _decal "/Game/Assets/Decals/HorrorDecals/Materials/HorrorDecals/LargeEnglishText/MI_HorrorDecals_LargeEnglishText_L.MI_HorrorDecals_LargeEnglishText_L"))
    (:`12`
      (`DecalComponent.SetDecalMaterial` _decal "/Game/Assets/Decals/HorrorDecals/Materials/HorrorDecals/LargeEnglishText/MI_HorrorDecals_LargeEnglishText_M.MI_HorrorDecals_LargeEnglishText_M"))
    (:`13`
      (`DecalComponent.SetDecalMaterial` _decal "/Game/Assets/Decals/HorrorDecals/Materials/HorrorDecals/LargeEnglishText/MI_HorrorDecals_LargeEnglishText_N.MI_HorrorDecals_LargeEnglishText_N"))
    (:`14`
      (`DecalComponent.SetDecalMaterial` _decal "/Game/Assets/Decals/HorrorDecals/Materials/HorrorDecals/LargeEnglishText/MI_HorrorDecals_LargeEnglishText_O.MI_HorrorDecals_LargeEnglishText_O"))
    (:`15`
      (`DecalComponent.SetDecalMaterial` _decal "/Game/Assets/Decals/HorrorDecals/Materials/HorrorDecals/LargeEnglishText/MI_HorrorDecals_LargeEnglishText_P.MI_HorrorDecals_LargeEnglishText_P"))
    (:`16`
      (`DecalComponent.SetDecalMaterial` _decal "/Game/Assets/Decals/HorrorDecals/Materials/HorrorDecals/LargeEnglishText/MI_HorrorDecals_LargeEnglishText_Q.MI_HorrorDecals_LargeEnglishText_Q"))
    (:`17`
      (`DecalComponent.SetDecalMaterial` _decal "/Game/Assets/Decals/HorrorDecals/Materials/HorrorDecals/LargeEnglishText/MI_HorrorDecals_LargeEnglishText_R.MI_HorrorDecals_LargeEnglishText_R"))))

(fn `Skulls Switch`
  (bind _decal (`self.Decal`))
  (switch `int` (`self.DecalNumber`)
    (:`0`
      (`DecalComponent.SetDecalMaterial` _decal "/Game/Assets/Decals/HorrorDecals/Materials/HorrorDecals/Skulls/MI_HorrorDecals_Skull_A.MI_HorrorDecals_Skull_A"))
    (:`1`
      (`DecalComponent.SetDecalMaterial` _decal "/Game/Assets/Decals/HorrorDecals/Materials/HorrorDecals/Skulls/MI_HorrorDecals_Skull_B.MI_HorrorDecals_Skull_B"))
    (:`2`
      (`DecalComponent.SetDecalMaterial` _decal "/Game/Assets/Decals/HorrorDecals/Materials/HorrorDecals/Skulls/MI_HorrorDecals_Skull_C.MI_HorrorDecals_Skull_C"))
    (:`3`
      (`DecalComponent.SetDecalMaterial` _decal "/Game/Assets/Decals/HorrorDecals/Materials/HorrorDecals/Skulls/MI_HorrorDecals_Skull_D.MI_HorrorDecals_Skull_D"))
    (:`4`
      (`DecalComponent.SetDecalMaterial` _decal "/Game/Assets/Decals/HorrorDecals/Materials/HorrorDecals/Skulls/MI_HorrorDecals_Skull_E.MI_HorrorDecals_Skull_E"))
    (:`5`
      (`DecalComponent.SetDecalMaterial` _decal "/Game/Assets/Decals/HorrorDecals/Materials/HorrorDecals/Skulls/MI_HorrorDecals_Skull_F.MI_HorrorDecals_Skull_F"))
    (:`6`
      (`DecalComponent.SetDecalMaterial` _decal "/Game/Assets/Decals/HorrorDecals/Materials/HorrorDecals/Skulls/MI_HorrorDecals_Skull_G.MI_HorrorDecals_Skull_G"))
    (:`7`
      (`DecalComponent.SetDecalMaterial` _decal "/Game/Assets/Decals/HorrorDecals/Materials/HorrorDecals/Skulls/MI_HorrorDecals_Skull_H.MI_HorrorDecals_Skull_H"))
    (:`8`
      (`DecalComponent.SetDecalMaterial` _decal "/Game/Assets/Decals/HorrorDecals/Materials/HorrorDecals/Skulls/MI_HorrorDecals_Skull_I.MI_HorrorDecals_Skull_I"))
    (:`9`
      (`DecalComponent.SetDecalMaterial` _decal "/Game/Assets/Decals/HorrorDecals/Materials/HorrorDecals/Skulls/MI_HorrorDecals_Skull_J.MI_HorrorDecals_Skull_J"))
    (:`10`
      (`DecalComponent.SetDecalMaterial` _decal "/Game/Assets/Decals/HorrorDecals/Materials/HorrorDecals/Skulls/MI_HorrorDecals_Skull_K.MI_HorrorDecals_Skull_K"))
    (:`11`
      (`DecalComponent.SetDecalMaterial` _decal "/Game/Assets/Decals/HorrorDecals/Materials/HorrorDecals/Skulls/MI_HorrorDecals_Skull_L.MI_HorrorDecals_Skull_L"))))

(fn `Small Text Switch`
  (bind _decal (`self.Decal`))
  (switch `int` (`self.DecalNumber`)
    (:`0`
      (`DecalComponent.SetDecalMaterial` _decal "/Game/Assets/Decals/HorrorDecals/Materials/HorrorDecals/SmallText/MI_HorrorDecals_SmallText_A.MI_HorrorDecals_SmallText_A"))
    (:`1`
      (`DecalComponent.SetDecalMaterial` _decal "/Game/Assets/Decals/HorrorDecals/Materials/HorrorDecals/SmallText/MI_HorrorDecals_SmallText_B.MI_HorrorDecals_SmallText_B"))
    (:`2`
      (`DecalComponent.SetDecalMaterial` _decal "/Game/Assets/Decals/HorrorDecals/Materials/HorrorDecals/SmallText/MI_HorrorDecals_SmallText_C.MI_HorrorDecals_SmallText_C"))
    (:`3`
      (`DecalComponent.SetDecalMaterial` _decal "/Game/Assets/Decals/HorrorDecals/Materials/HorrorDecals/SmallText/MI_HorrorDecals_SmallText_D.MI_HorrorDecals_SmallText_D"))
    (:`4`
      (`DecalComponent.SetDecalMaterial` _decal "/Game/Assets/Decals/HorrorDecals/Materials/HorrorDecals/SmallText/MI_HorrorDecals_SmallText_E.MI_HorrorDecals_SmallText_E"))
    (:`5`
      (`DecalComponent.SetDecalMaterial` _decal "/Game/Assets/Decals/HorrorDecals/Materials/HorrorDecals/SmallText/MI_HorrorDecals_SmallText_F.MI_HorrorDecals_SmallText_F"))
    (:`6`
      (`DecalComponent.SetDecalMaterial` _decal "/Game/Assets/Decals/HorrorDecals/Materials/HorrorDecals/SmallText/MI_HorrorDecals_SmallText_G.MI_HorrorDecals_SmallText_G"))))

(fn `Smears Switch`
  (bind _decal (`self.Decal`))
  (switch `int` (`self.DecalNumber`)
    (:`0`
      (`DecalComponent.SetDecalMaterial` _decal "/Game/Assets/Decals/HorrorDecals/Materials/HorrorDecals/Smears/MI_HorrorDecals_Smears_A.MI_HorrorDecals_Smears_A"))
    (:`1`
      (`DecalComponent.SetDecalMaterial` _decal "/Game/Assets/Decals/HorrorDecals/Materials/HorrorDecals/Smears/MI_HorrorDecals_Smears_B.MI_HorrorDecals_Smears_B"))
    (:`2`
      (`DecalComponent.SetDecalMaterial` _decal "/Game/Assets/Decals/HorrorDecals/Materials/HorrorDecals/Smears/MI_HorrorDecals_Smears_C.MI_HorrorDecals_Smears_C"))
    (:`3`
      (`DecalComponent.SetDecalMaterial` _decal "/Game/Assets/Decals/HorrorDecals/Materials/HorrorDecals/Smears/MI_HorrorDecals_Smears_D.MI_HorrorDecals_Smears_D"))
    (:`4`
      (`DecalComponent.SetDecalMaterial` _decal "/Game/Assets/Decals/HorrorDecals/Materials/HorrorDecals/Smears/MI_HorrorDecals_Smears_E.MI_HorrorDecals_Smears_E"))
    (:`5`
      (`DecalComponent.SetDecalMaterial` _decal "/Game/Assets/Decals/HorrorDecals/Materials/HorrorDecals/Smears/MI_HorrorDecals_Smears_F.MI_HorrorDecals_Smears_F"))
    (:`6`
      (`DecalComponent.SetDecalMaterial` _decal "/Game/Assets/Decals/HorrorDecals/Materials/HorrorDecals/Smears/MI_HorrorDecals_Smears_G.MI_HorrorDecals_Smears_G"))
    (:`7`
      (`DecalComponent.SetDecalMaterial` _decal "/Game/Assets/Decals/HorrorDecals/Materials/HorrorDecals/Smears/MI_HorrorDecals_Smears_H.MI_HorrorDecals_Smears_H"))
    (:`8`
      (`DecalComponent.SetDecalMaterial` _decal "/Game/Assets/Decals/HorrorDecals/Materials/HorrorDecals/Smears/MI_HorrorDecals_Smears_I.MI_HorrorDecals_Smears_I"))
    (:`9`
      (`DecalComponent.SetDecalMaterial` _decal "/Game/Assets/Decals/HorrorDecals/Materials/HorrorDecals/Smears/MI_HorrorDecals_Smears_J.MI_HorrorDecals_Smears_J"))
    (:`10`
      (`DecalComponent.SetDecalMaterial` _decal "/Game/Assets/Decals/HorrorDecals/Materials/HorrorDecals/Smears/MI_HorrorDecals_Smears_K.MI_HorrorDecals_Smears_K"))
    (:`11`
      (`DecalComponent.SetDecalMaterial` _decal "/Game/Assets/Decals/HorrorDecals/Materials/HorrorDecals/Smears/MI_HorrorDecals_Smears_L.MI_HorrorDecals_Smears_L"))
    (:`12`
      (`DecalComponent.SetDecalMaterial` _decal "/Game/Assets/Decals/HorrorDecals/Materials/HorrorDecals/Smears/MI_HorrorDecals_Smears_M.MI_HorrorDecals_Smears_M"))
    (:`13`
      (`DecalComponent.SetDecalMaterial` _decal "/Game/Assets/Decals/HorrorDecals/Materials/HorrorDecals/Smears/MI_HorrorDecals_Smears_N.MI_HorrorDecals_Smears_N"))
    (:`14`
      (`DecalComponent.SetDecalMaterial` _decal "/Game/Assets/Decals/HorrorDecals/Materials/HorrorDecals/Smears/MI_HorrorDecals_Smears_O.MI_HorrorDecals_Smears_O"))
    (:`15`
      (`DecalComponent.SetDecalMaterial` _decal "/Game/Assets/Decals/HorrorDecals/Materials/HorrorDecals/Smears/MI_HorrorDecals_Smears_P.MI_HorrorDecals_Smears_P"))))

(fn `Symbols Switch`
  (bind _decal (`self.Decal`))
  (switch `int` (`self.DecalNumber`)
    (:`0`
      (`DecalComponent.SetDecalMaterial` _decal "/Game/Assets/Decals/HorrorDecals/Materials/HorrorDecals/Symbols/MI_HorrorDecals_Symbol_A.MI_HorrorDecals_Symbol_A"))
    (:`1`
      (`DecalComponent.SetDecalMaterial` _decal "/Game/Assets/Decals/HorrorDecals/Materials/HorrorDecals/Symbols/MI_HorrorDecals_Symbol_B.MI_HorrorDecals_Symbol_B"))
    (:`2`
      (`DecalComponent.SetDecalMaterial` _decal "/Game/Assets/Decals/HorrorDecals/Materials/HorrorDecals/Symbols/MI_HorrorDecals_Symbol_C.MI_HorrorDecals_Symbol_C"))
    (:`3`
      (`DecalComponent.SetDecalMaterial` _decal "/Game/Assets/Decals/HorrorDecals/Materials/HorrorDecals/Symbols/MI_HorrorDecals_Symbol_D.MI_HorrorDecals_Symbol_D"))
    (:`4`
      (`DecalComponent.SetDecalMaterial` _decal "/Game/Assets/Decals/HorrorDecals/Materials/HorrorDecals/Symbols/MI_HorrorDecals_Symbol_E.MI_HorrorDecals_Symbol_E"))
    (:`5`
      (`DecalComponent.SetDecalMaterial` _decal "/Game/Assets/Decals/HorrorDecals/Materials/HorrorDecals/Symbols/MI_HorrorDecals_Symbol_F.MI_HorrorDecals_Symbol_F"))
    (:`6`
      (`DecalComponent.SetDecalMaterial` _decal "/Game/Assets/Decals/HorrorDecals/Materials/HorrorDecals/Symbols/MI_HorrorDecals_Symbol_G.MI_HorrorDecals_Symbol_G"))
    (:`7`
      (`DecalComponent.SetDecalMaterial` _decal "/Game/Assets/Decals/HorrorDecals/Materials/HorrorDecals/Symbols/MI_HorrorDecals_Symbol_H.MI_HorrorDecals_Symbol_H"))
    (:`8`
      (`DecalComponent.SetDecalMaterial` _decal "/Game/Assets/Decals/HorrorDecals/Materials/HorrorDecals/Symbols/MI_HorrorDecals_Symbol_I.MI_HorrorDecals_Symbol_I"))
    (:`9`
      (`DecalComponent.SetDecalMaterial` _decal "/Game/Assets/Decals/HorrorDecals/Materials/HorrorDecals/Symbols/MI_HorrorDecals_Symbol_J.MI_HorrorDecals_Symbol_J"))
    (:`10`
      (`DecalComponent.SetDecalMaterial` _decal "/Game/Assets/Decals/HorrorDecals/Materials/HorrorDecals/Symbols/MI_HorrorDecals_Symbol_K.MI_HorrorDecals_Symbol_K"))
    (:`11`
      (`DecalComponent.SetDecalMaterial` _decal "/Game/Assets/Decals/HorrorDecals/Materials/HorrorDecals/Symbols/MI_HorrorDecals_Symbol_L.MI_HorrorDecals_Symbol_L"))
    (:`12`
      (`DecalComponent.SetDecalMaterial` _decal "/Game/Assets/Decals/HorrorDecals/Materials/HorrorDecals/Symbols/MI_HorrorDecals_Symbol_M.MI_HorrorDecals_Symbol_M"))
    (:`13`
      (`DecalComponent.SetDecalMaterial` _decal "/Game/Assets/Decals/HorrorDecals/Materials/HorrorDecals/Symbols/MI_HorrorDecals_Symbol_N.MI_HorrorDecals_Symbol_N"))
    (:`14`
      (`DecalComponent.SetDecalMaterial` _decal "/Game/Assets/Decals/HorrorDecals/Materials/HorrorDecals/Symbols/MI_HorrorDecals_Symbol_O.MI_HorrorDecals_Symbol_O"))
    (:`15`
      (`DecalComponent.SetDecalMaterial` _decal "/Game/Assets/Decals/HorrorDecals/Materials/HorrorDecals/Symbols/MI_HorrorDecals_Symbol_P.MI_HorrorDecals_Symbol_P"))
    (:`16`
      (`DecalComponent.SetDecalMaterial` _decal "/Game/Assets/Decals/HorrorDecals/Materials/HorrorDecals/Symbols/MI_HorrorDecals_Symbol_Q.MI_HorrorDecals_Symbol_Q"))
    (:`17`
      (`DecalComponent.SetDecalMaterial` _decal "/Game/Assets/Decals/HorrorDecals/Materials/HorrorDecals/Symbols/MI_HorrorDecals_Symbol_R.MI_HorrorDecals_Symbol_R"))
    (:`18`
      (`DecalComponent.SetDecalMaterial` _decal "/Game/Assets/Decals/HorrorDecals/Materials/HorrorDecals/Symbols/MI_HorrorDecals_Symbol_S.MI_HorrorDecals_Symbol_S"))
    (:`19`
      (`DecalComponent.SetDecalMaterial` _decal "/Game/Assets/Decals/HorrorDecals/Materials/HorrorDecals/Symbols/MI_HorrorDecals_Symbol_T.MI_HorrorDecals_Symbol_T"))
    (:`20`
      (`DecalComponent.SetDecalMaterial` _decal "/Game/Assets/Decals/HorrorDecals/Materials/HorrorDecals/Symbols/MI_HorrorDecals_Symbol_U.MI_HorrorDecals_Symbol_U"))
    (:`21`
      (`DecalComponent.SetDecalMaterial` _decal "/Game/Assets/Decals/HorrorDecals/Materials/HorrorDecals/Symbols/MI_HorrorDecals_Symbol_V.MI_HorrorDecals_Symbol_V"))
    (:`22`
      (`DecalComponent.SetDecalMaterial` _decal "/Game/Assets/Decals/HorrorDecals/Materials/HorrorDecals/Symbols/MI_HorrorDecals_Symbol_W.MI_HorrorDecals_Symbol_W"))
    (:`23`
      (`DecalComponent.SetDecalMaterial` _decal "/Game/Assets/Decals/HorrorDecals/Materials/HorrorDecals/Symbols/MI_HorrorDecals_Symbol_X.MI_HorrorDecals_Symbol_X"))
    (:`24`
      (`DecalComponent.SetDecalMaterial` _decal "/Game/Assets/Decals/HorrorDecals/Materials/HorrorDecals/Symbols/MI_HorrorDecals_Symbol_Y.MI_HorrorDecals_Symbol_Y"))
    (:`25`
      (`DecalComponent.SetDecalMaterial` _decal "/Game/Assets/Decals/HorrorDecals/Materials/HorrorDecals/Symbols/MI_HorrorDecals_Symbol_Z.MI_HorrorDecals_Symbol_Z"))))

(fn `UserConstructionScript`
  ;[1 1 1] Fix Scaling issue
  (`SceneComponent.SetWorldScale3D` (`self.Decal`) (* (`KismetMathLibrary.MakeVector` (* (.x (`self.GetActorScale3D`)) -1.0) (.z (`self.GetActorScale3D`)) (* (.y (`self.GetActorScale3D`)) -1.0)) 0.5))
  (switch `/Game/Assets/Decals/HorrorDecals/Enums/Enum_HorrorDecalTypes` (`self.Decal Type`)
    (:`NewEnumerator0`
      (`self.Circular Decals Switch`))
    (:`NewEnumerator1`
      (`self.Large Alien Text Switch`))
    (:`NewEnumerator2`
      (`self.Large English Text Switch`))
    (:`NewEnumerator4`
      (`self.Skulls Switch`))
    (:`NewEnumerator5`
      (`self.Small Text Switch`))
    (:`NewEnumerator6`
      (`self.Smears Switch`))
    (:`NewEnumerator7`
      (`self.Symbols Switch`))
    (:`NewEnumerator8`
      (`self.Wallstain Switch`))))

(fn `Wallstain Switch`
  (bind _decal (`self.Decal`))
  (switch `int` (`self.DecalNumber`)
    (:`0`
      (`DecalComponent.SetDecalMaterial` _decal "/Game/Assets/Decals/HorrorDecals/Materials/HorrorDecals/WallStains/MI_HorrorDecals_WallStain_A.MI_HorrorDecals_WallStain_A"))
    (:`1`
      (`DecalComponent.SetDecalMaterial` _decal "/Game/Assets/Decals/HorrorDecals/Materials/HorrorDecals/WallStains/MI_HorrorDecals_WallStain_B.MI_HorrorDecals_WallStain_B"))
    (:`2`
      (`DecalComponent.SetDecalMaterial` _decal "/Game/Assets/Decals/HorrorDecals/Materials/HorrorDecals/WallStains/MI_HorrorDecals_WallStain_C.MI_HorrorDecals_WallStain_C"))
    (:`3`
      (`DecalComponent.SetDecalMaterial` _decal "/Game/Assets/Decals/HorrorDecals/Materials/HorrorDecals/WallStains/MI_HorrorDecals_WallStain_D.MI_HorrorDecals_WallStain_D"))
    (:`4`
      (`DecalComponent.SetDecalMaterial` _decal "/Game/Assets/Decals/HorrorDecals/Materials/HorrorDecals/WallStains/MI_HorrorDecals_WallStain_E.MI_HorrorDecals_WallStain_E"))
    (:`5`
      (`DecalComponent.SetDecalMaterial` _decal "/Game/Assets/Decals/HorrorDecals/Materials/HorrorDecals/WallStains/MI_HorrorDecals_WallStain_F.MI_HorrorDecals_WallStain_F"))
    (:`6`
      (`DecalComponent.SetDecalMaterial` _decal "/Game/Assets/Decals/HorrorDecals/Materials/HorrorDecals/WallStains/MI_HorrorDecals_WallStain_G.MI_HorrorDecals_WallStain_G"))
    (:`7`
      (`DecalComponent.SetDecalMaterial` _decal "/Game/Assets/Decals/HorrorDecals/Materials/HorrorDecals/WallStains/MI_HorrorDecals_WallStain_H.MI_HorrorDecals_WallStain_H"))
    (:`8`
      (`DecalComponent.SetDecalMaterial` _decal "/Game/Assets/Decals/HorrorDecals/Materials/HorrorDecals/WallStains/MI_HorrorDecals_WallStain_I.MI_HorrorDecals_WallStain_I"))
    (:`9`
      (`DecalComponent.SetDecalMaterial` _decal "/Game/Assets/Decals/HorrorDecals/Materials/HorrorDecals/WallStains/MI_HorrorDecals_WallStain_J.MI_HorrorDecals_WallStain_J"))
    (:`10`
      (`DecalComponent.SetDecalMaterial` _decal "/Game/Assets/Decals/HorrorDecals/Materials/HorrorDecals/WallStains/MI_HorrorDecals_WallStain_K.MI_HorrorDecals_WallStain_K"))
    (:`11`
      (`DecalComponent.SetDecalMaterial` _decal "/Game/Assets/Decals/HorrorDecals/Materials/HorrorDecals/WallStains/MI_HorrorDecals_WallStain_L.MI_HorrorDecals_WallStain_L"))
    (:`12`
      (`DecalComponent.SetDecalMaterial` _decal "/Game/Assets/Decals/HorrorDecals/Materials/HorrorDecals/WallStains/MI_HorrorDecals_WallStain_M.MI_HorrorDecals_WallStain_M"))))