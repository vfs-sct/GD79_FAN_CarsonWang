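; BP_Laser is a laser VFX actor that fires a Niagara beam along its forward vector.
; Each Tick line-traces on the Camera channel to set the beam end, place and orient the hit effect, toggle its spawn probability and scale all three Niagara effects.
; Beam length snaps to the offset hit point when blocked and grows rapidly each frame toward a range cap, so the beam visibly extends.
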(event `self.ReceiveTick`
  (params (DeltaSeconds :type "Float (single-precision)"))
  (bind _returnvalue (`self.K2_GetActorLocation`))
  (bind _distance (`self.Distance`))
  (bind _returnvalue_2 (+ _returnvalue (* (`self.GetActorForwardVector`) (`self.Distance`))))
  (`|ExecutionSequence`
    (:`then_0`
      (set `self.TraceEnd` _returnvalue_2)
      (bind _outhit (`KismetSystemLibrary.LineTraceSingle` _returnvalue _returnvalue_2 "TraceTypeQuery2"))
      (bind (_bblockinghit _binitialoverlap _time _distance_2 _location _impactpoint _normal _impactnormal) (`GameplayStatics.BreakHitResult` _outhit))
      (set `self.LaserHit` _bblockinghit)
      (set `self.HitLocation` (+ _location (* _impactnormal (`self.Hit offset`))))
      (if (`self.Use zero rotation`)
        (set `self.Rotation` (struct))
        (elif (`self.Use self rotation`)
          (set `self.Rotation` (`self.K2_GetActorRotation`))
          (else
            (set `self.Rotation` (`KismetMathLibrary.MakeRotFromX` _impactnormal)))))
      (`FXSystemComponent.SetVectorParameter` (`self.NiagaraLaser`) "LaserEnd" (select `bool` (`self.LaserHit`) :`false` (`self.TraceEnd`) :`true` _location))
      (if (`self.LaserHit`)
        (set `self.HitEffectLocation` (`self.HitLocation`))
        (set `self.BeamSpawnProb` 1.0)
        (else
          (set `self.HitEffectLocation` (`self.TraceEnd`))
          (set `self.BeamSpawnProb` 0.0)))
      (`NiagaraComponent.SetVariableFloat` (`self.NiagaraLaserHit`) "BeamSpawnProb" (`self.BeamSpawnProb`))
      (`NiagaraComponent.SetVariableFloat` (`self.LaserFlash`) "Scale" (`self.Scale`))
      (`NiagaraComponent.SetVariableFloat` (`self.NiagaraLaserHit`) "Scale" (`self.Scale`))
      (`NiagaraComponent.SetVariableFloat` (`self.NiagaraLaser`) "Scale" (`self.Scale`))
      (`SceneComponent.K2_SetWorldLocation` (`self.NiagaraLaserHit`) (`self.HitEffectLocation`) false false)
      (`SceneComponent.K2_SetWorldRotation` (`self.NiagaraLaserHit`) (`self.Rotation`) false false)
      (if (`self.LaserHit`)
        (set `self.Distance` (`KismetMathLibrary.VSize` (- (`self.HitLocation`) (`self.K2_GetActorLocation`))))))
    (:`then_1`
      (if (< _distance 5000.0)
        (set `self.Distance` (+ _distance (* DeltaSeconds 30000.0)))))))

(fn `UserConstructionScript`)