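; BP_spline_root is an Underworld environment actor that builds a tapering mesh along an editable spline, apparently for roots.
; The construction script adds a spline mesh for each segment between spline points, matching local positions and tangents with collision enabled.
; Segment end scales interpolate linearly from ScaleStart to ScaleEnd by distance along the spline, so thickness stays continuous across joins.
; The event graph has no active logic.
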(fn `UserConstructionScript`
  (bind _spline (`self.Spline`))
  (bind _spline_2 (`self.Spline`))
  (bind _spline_3 (`self.Spline`))
  (bind _scale_end (`self.Scale_End`))
  (bind _returnvalue (`SplineComponent.GetSplineLength` _spline_2))
  (bind _returnvalue_2 (/ (- _scale_end (`self.Scale_Start`)) _returnvalue))
  (for _index (range (+ (- (`SplineComponent.GetNumberOfSplinePoints` (`self.Spline`)) 2) 1))
    (bind _returnvalue_3 (`AddComponent|NODE_AddSplineMeshComponent-0`))
    (`SplineMeshComponent.SetForwardAxis` _returnvalue_3 "X" true)
    (bind _returnvalue_4 (+ _index 1))
    (`SplineMeshComponent.SetStartAndEnd` _returnvalue_3 (`SplineComponent.GetLocationAtSplinePoint` _spline_2 _index "Local") (`SplineComponent.GetTangentAtSplinePoint` _spline_2 _index "Local") (`SplineComponent.GetLocationAtSplinePoint` _spline_3 _returnvalue_4 "Local") (`SplineComponent.GetTangentAtSplinePoint` _spline_3 _returnvalue_4 "Local") true)
    (bind _returnvalue_5 (- _scale_end (* _returnvalue_2 (- _returnvalue (`SplineComponent.GetDistanceAlongSplineAtSplinePoint` _spline (+ _index 1))))))
    (`SplineMeshComponent.SetEndScale` _returnvalue_3 (`KismetMathLibrary.MakeVector2D` _returnvalue_5 _returnvalue_5) true)
    (bind _returnvalue_6 (- _scale_end (* _returnvalue_2 (- _returnvalue (`SplineComponent.GetDistanceAlongSplineAtSplinePoint` _spline _index)))))
    (`SplineMeshComponent.SetStartScale` _returnvalue_3 (`KismetMathLibrary.MakeVector2D` _returnvalue_6 _returnvalue_6) true)
    (`PrimitiveComponent.SetCollisionEnabled` _returnvalue_3 "QueryAndPhysics")))